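; BP_ds_easter_egg is a Death Stranding-themed easter egg actor that plays a scripted cinematic sequence on BeginPlay.
; Four timelines chain through Finished pins and delays, offsetting flowers, BTs, dead fish and a chiral crystal while driving post-process weight and decal scale.
; Between stages it reveals a storm, plays a palm animation and hides spent elements, ending with crystal particle activation.
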(event EventBeginPlay
  (bind (_direction _postprocess _flowers) (Timeline|Timeline_1 Play)
    (:Update
      (Variables|/Script/Engine.PostProcessComponent|SetBlendWeight (Variables|Default|GetPostProcess) _postprocess)
      (Transformation|AddWorldOffset (Variables|Default|Getflowers) _flowers true false))
    (:Finished
      (Utilities|FlowControl|Delay 2.0)
      (Rendering|SetVisibility (Variables|Default|GetBP_Storm) true false)
      (Utilities|FlowControl|Delay 1.0)
      (Components|Animation|PlayAnimation (Variables|Default|Getds_palm) "/Game/users/andrej/ds/ds_palm_Anim.ds_palm_Anim" false)
      (Utilities|FlowControl|Delay 1.0)
      (bind (_direction_2 _newtrack_0 _bts) (Timeline|Timeline_0 PlayFromStart)
        (:Update
          (Transformation|SetWorldScale3D (Variables|Default|GetDecal) (* (Math|Conversions|ToVector(Float) _newtrack_0) "0.800000,2.300000,2.300000"))
          (Transformation|AddWorldOffset (Variables|Default|GetBts) (* (Math|Conversions|ToVector(Float) _bts) "0.000000,0.000000,4.000000") true false))
        (:Finished
          (Rendering|SetVisibility (Variables|Default|Getflowers) false true)
          (Utilities|FlowControl|Delay 2.0)
          (bind (_direction_3 _postprocess_2 _fish _decal1) (Timeline|fish_appear PlayFromStart)
            (:Update
              (Transformation|AddWorldOffset (Variables|Default|Getdead_fish) _fish false false)
              (Variables|/Script/Engine.PostProcessComponent|SetBlendWeight (Variables|Default|GetPostProcess) _postprocess_2)
              (Transformation|SetWorldScale3D (Variables|Default|GetDecal) _decal1)
              (Rendering|SetVisibility (Variables|Default|GetPlane) false false))
            (:Finished
              (Rendering|SetVisibility (Variables|Default|GetBts) false true)
              (bind _newtrack_0_2 (Timeline|chrystal PlayFromStart)
                (:Update
                  (Transformation|AddWorldOffset (Variables|Default|Getchiral_crystal) _newtrack_0_2 true false))
                (:Finished
                  (Components|Activation|Activate (Variables|Default|Getchyral_crystal_particles) false))))))))))

(event Collision|EventActorBeginOverlap
  (params (OtherActor :type Actor%20Object%20Reference)))

(event EventTick
  (params (DeltaSeconds :type Float%20%28single-precision%29)))

(fn ConstructionScript)