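; BP_door_toilet is a toilet door that swings open when a FirstPersonCharacter enters the Open_door1 trigger and closes when they leave.
; Overlap begin and end play one timeline forward from the start or in reverse from the end, driving Door1's relative yaw.
; Both events disable the door's collision during the swing, and the timeline's Finished output restores query and physics collision.
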(event OnComponentBeginOverlap(open_door1)
  (params (OverlappedComponent :type Primitive%20Component%20Object%20Reference) (OtherActor :type Actor%20Object%20Reference) (OtherComp :type Primitive%20Component%20Object%20Reference) (OtherBodyIndex :type Integer) (bFromSweep :type Boolean) (SweepResult :type Hit%20Result%20Structure%20%28by%20ref%29))
  (Utilities|Casting|CastToFirstPersonCharacter OtherActor)
  (Collision|SetCollisionEnabled (Variables|Default|Getdoor1) "NoCollision")
  (bind _newtrack_0 (Timeline|Timeline_1 PlayFromStart)
    (:Update
      (Transformation|SetRelativeRotation (Variables|Default|Getdoor1) (Math|Rotator|MakeRotator 0.0 0.0 _newtrack_0) false false))
    (:Finished
      (Collision|SetCollisionEnabled (Variables|Default|Getdoor1) "QueryAndPhysics"))))

(event OnComponentEndOverlap(open_door1)
  (params (OverlappedComponent :type Primitive%20Component%20Object%20Reference) (OtherActor :type Actor%20Object%20Reference) (OtherComp :type Primitive%20Component%20Object%20Reference) (OtherBodyIndex :type Integer))
  (Utilities|Casting|CastToFirstPersonCharacter OtherActor)
  (Collision|SetCollisionEnabled (Variables|Default|Getdoor1) "NoCollision")
  (bind _newtrack_0 (Timeline|Timeline_1 ReverseFromEnd)
    (:Update
      (Transformation|SetRelativeRotation (Variables|Default|Getdoor1) (Math|Rotator|MakeRotator 0.0 0.0 _newtrack_0) false false))
    (:Finished
      (Collision|SetCollisionEnabled (Variables|Default|Getdoor1) "QueryAndPhysics"))))

(fn ConstructionScript)