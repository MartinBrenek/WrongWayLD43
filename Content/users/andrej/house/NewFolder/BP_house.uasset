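; House actor that swaps streamed interior levels and shell meshes as something moves through its trigger volumes.
; Enter and Exit set EnteredHouse, toggle the Backside mesh and swap the house_hide and house_hallway levels.
; While EnteredHouse is set, hall and room triggers toggle HouseTest and unload or load house_room.
; Two timelines yaw the doors open on overlap and reverse on exit; only Door requires EnteredHouse to open.
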(event OnComponentBeginOverlap(enter)
  (params (OverlappedComponent :type Primitive%20Component%20Object%20Reference) (OtherActor :type Actor%20Object%20Reference) (OtherComp :type Primitive%20Component%20Object%20Reference) (OtherBodyIndex :type Integer) (bFromSweep :type Boolean) (SweepResult :type Hit%20Result%20Structure%20%28by%20ref%29))
  (bind _backside (Variables|Default|Getbackside))
  (Variables|Default|Setentered_house true)
  (Collision|SetCollisionEnabled _backside "NoCollision")
  (Rendering|SetVisibility _backside false false)
  (Game|UnloadStreamLevel(byName) "house_hide" false)
  (Game|LoadStreamLevel(byName) "house_hallway" true))

(event OnComponentBeginOverlap(exit)
  (params (OverlappedComponent :type Primitive%20Component%20Object%20Reference) (OtherActor :type Actor%20Object%20Reference) (OtherComp :type Primitive%20Component%20Object%20Reference) (OtherBodyIndex :type Integer) (bFromSweep :type Boolean) (SweepResult :type Hit%20Result%20Structure%20%28by%20ref%29))
  (bind _backside (Variables|Default|Getbackside))
  (Variables|Default|Setentered_house false)
  (Collision|SetCollisionEnabled _backside "QueryOnly")
  (Rendering|SetVisibility _backside true false)
  (Game|LoadStreamLevel(byName) "house_hide" true)
  (Game|UnloadStreamLevel(byName) "house_hallway" false))

(event OnComponentBeginOverlap(enter_hall)
  (params (OverlappedComponent :type Primitive%20Component%20Object%20Reference) (OtherActor :type Actor%20Object%20Reference) (OtherComp :type Primitive%20Component%20Object%20Reference) (OtherBodyIndex :type Integer) (bFromSweep :type Boolean) (SweepResult :type Hit%20Result%20Structure%20%28by%20ref%29))
  (bind _house_test (Variables|Default|Gethouse_test))
  (if (Variables|Default|Getentered_house)
    (Collision|SetCollisionEnabled _house_test "QueryOnly")
    (Rendering|SetVisibility _house_test true false)
    (Game|UnloadStreamLevel(byName) "house_room" false)))

(event OnComponentBeginOverlap(enter_room)
  (params (OverlappedComponent :type Primitive%20Component%20Object%20Reference) (OtherActor :type Actor%20Object%20Reference) (OtherComp :type Primitive%20Component%20Object%20Reference) (OtherBodyIndex :type Integer) (bFromSweep :type Boolean) (SweepResult :type Hit%20Result%20Structure%20%28by%20ref%29))
  (bind _house_test (Variables|Default|Gethouse_test))
  (if (Variables|Default|Getentered_house)
    (Collision|SetCollisionEnabled _house_test "NoCollision")
    (Rendering|SetVisibility _house_test false false)
    (Game|LoadStreamLevel(byName) "house_room" true)))

(event OnComponentBeginOverlap(open_door)
  (params (OverlappedComponent :type Primitive%20Component%20Object%20Reference) (OtherActor :type Actor%20Object%20Reference) (OtherComp :type Primitive%20Component%20Object%20Reference) (OtherBodyIndex :type Integer) (bFromSweep :type Boolean) (SweepResult :type Hit%20Result%20Structure%20%28by%20ref%29))
  (if (Variables|Default|Getentered_house)
    (bind _newtrack_0 (Timeline|Timeline_0 PlayFromStart)
      (:Update
        (Transformation|SetRelativeRotation (Variables|Default|Getdoor) (Math|Rotator|MakeRotator 0.0 0.0 _newtrack_0) false false)))))

(event OnComponentEndOverlap(open_door)
  (params (OverlappedComponent :type Primitive%20Component%20Object%20Reference) (OtherActor :type Actor%20Object%20Reference) (OtherComp :type Primitive%20Component%20Object%20Reference) (OtherBodyIndex :type Integer))
  (bind _newtrack_0 (Timeline|Timeline_0 ReverseFromEnd)
    (:Update
      (Transformation|SetRelativeRotation (Variables|Default|Getdoor) (Math|Rotator|MakeRotator 0.0 0.0 _newtrack_0) false false))))

(event OnComponentBeginOverlap(open_door1)
  (params (OverlappedComponent :type Primitive%20Component%20Object%20Reference) (OtherActor :type Actor%20Object%20Reference) (OtherComp :type Primitive%20Component%20Object%20Reference) (OtherBodyIndex :type Integer) (bFromSweep :type Boolean) (SweepResult :type Hit%20Result%20Structure%20%28by%20ref%29))
  (bind _newtrack_0 (Timeline|Timeline_1 PlayFromStart)
    (:Update
      (Transformation|SetRelativeRotation (Variables|Default|Getdoor1) (Math|Rotator|MakeRotator 0.0 0.0 _newtrack_0) false false))))

(event OnComponentEndOverlap(open_door1)
  (params (OverlappedComponent :type Primitive%20Component%20Object%20Reference) (OtherActor :type Actor%20Object%20Reference) (OtherComp :type Primitive%20Component%20Object%20Reference) (OtherBodyIndex :type Integer))
  (bind _newtrack_0 (Timeline|Timeline_1 ReverseFromEnd)
    (:Update
      (Transformation|SetRelativeRotation (Variables|Default|Getdoor1) (Math|Rotator|MakeRotator 0.0 0.0 _newtrack_0) false false))))

(event EventBeginPlay)

(event Collision|EventActorBeginOverlap
  (params (OtherActor :type Actor%20Object%20Reference)))

(event EventTick
  (params (DeltaSeconds :type Float%20%28single-precision%29)))

(fn ConstructionScript)