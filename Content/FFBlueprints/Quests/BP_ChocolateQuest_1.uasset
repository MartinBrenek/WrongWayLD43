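; Chocolate quest Blueprint that extends a parent quest class with a bottle cap spawn and an NPC end-of-quest call.
; On BeginPlay it spawns a BP_BottleCap at the SpawnPointBottleCap component's transform.
; Its CanFinalizeQuest override runs the parent check, calls EndQuest regardless of the result, then returns that result.
; EndQuest casts the spawned NPC to CrowdCharacter and calls CallToEndQuest on it.
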(event EventBeginPlay
  (|CallParentFunction)
  (Game|SpawnActorfromClass "/Game/FFBlueprints/FastFoodOutDoor/BP_BottleCap.BP_BottleCap_C" (Transformation|GetWorldTransform (Variables|Default|GetSpawnPointBottleCap)) "Undefined" 0 0))

(event Collision|EventActorBeginOverlap
  (params (OtherActor :type Actor%20Object%20Reference))
  (|CallParentFunction OtherActor) ; This node is disabled and will not be called.\nDrag off pins to build functionality.
)

(event EventTick
  (params (DeltaSeconds :type Float%20%28single-precision%29))
  (|CallParentFunction DeltaSeconds) ; This node is disabled and will not be called.\nDrag off pins to build functionality.
)

(event EventEndQuest
  (bind _ascrowd_character (Utilities|Casting|CastToCrowdCharacter (Variables|Default|GetSpawnedNPC)))
  (Default|CalltoEndQuest _ascrowd_character))

(fn ConstructionScript
  (|CallParentFunction))

(fn CanFinalizeQuest
  (params (Ingredients :type Ingredients%20Enum :default "NewEnumerator9"))
  (bind _success (|CallParentFunction Ingredients))
  (CallFunction|EndQuest)
  (return _success))