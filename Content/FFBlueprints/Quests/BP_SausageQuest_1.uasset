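; Quest Blueprint for the first sausage quest, which hands the "BaldGuy" NPC a quest role when it starts.
; On StartQuest it runs the parent logic, then looks up the NPC by name through the FastFoodGameState's QuestManager.
; It sets the NPC's current quest type, queries its state component for the next state and changes its role to it.
; Failed lookups are written to the debug log.
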(event EventBeginPlay
  (|CallParentFunction) ; This node is disabled and will not be called.\nDrag off pins to build functionality.
)

(event Collision|EventActorBeginOverlap
  (params (OtherActor :type Actor%20Object%20Reference))
  (|CallParentFunction OtherActor) ; This node is disabled and will not be called.\nDrag off pins to build functionality.
)

(event EventTick
  (params (DeltaSeconds :type Float%20%28single-precision%29))
  (|CallParentFunction DeltaSeconds) ; This node is disabled and will not be called.\nDrag off pins to build functionality.
)

(event EventStartQuest
  (|CallParentFunction)
  (bind _asfast_food_game_state (Utilities|Casting|CastToFastFoodGameState (Game|GetGameState)))
  (bind _output_get (Variables|Default|SetQuestManager (Variables|/Game/FFBlueprints/GameMode/FastFoodGameState.FastFoodGameState_C|GetQuestManager _asfast_food_game_state)))
  (bind (_value _found) (Default|GetActorReference _output_get "BaldGuy"))
  (if _found
    (bind (_parent _statecomp _valid) (CallFunction|GetNPCState _value))
    (if _valid
      (bind (_nextstatefound _newstate) (Default|NextState _statecomp "NewEnumerator3"))
      (Variables|/Game/FFBlueprints/Crowd/CrowdCharacter.CrowdCharacter_C|SetCurrentQuestType _parent "NewEnumerator5")
      (if _nextstatefound
        (Default|ChangeRole _parent _newstate)
        (else
          (CallFunction|DebugLog (Utilities|String|Append "Next state not found:" (Utilities|GetDisplayName _value)) "NewEnumerator2")))
      (else
        (CallFunction|DebugLog (Utilities|String|Append "Missing NPCState:" (Utilities|GetDisplayName _value)) "NewEnumerator2")))
    (else
      (CallFunction|DebugLog (Utilities|String|Append "Missing Reference:" "BaldGuy") "NewEnumerator2"))))

(fn ConstructionScript
  (|CallParentFunction))