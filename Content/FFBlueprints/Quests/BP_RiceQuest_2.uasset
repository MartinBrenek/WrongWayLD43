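; BP_RiceQuest_2 is a quest Blueprint whose only custom logic decides whether the quest can be finalized for a given set of ingredients.
; CanFinalizeQuest reads the HookStolen key from the spawned BP_Builder NPC's blackboard.
; While the key is false it queues the ingredients in PendingQuestEnd and refuses; once true, it finalizes only queued ingredients, removing them from that list.
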(event EventBeginPlay
  (|CallParentFunction) ; This node is disabled and will not be called.\nDrag off pins to build functionality.
)

(event Collision|EventActorBeginOverlap
  (params (OtherActor :type Actor%20Object%20Reference))
  (|CallParentFunction OtherActor) ; This node is disabled and will not be called.\nDrag off pins to build functionality.
)

(event EventTick
  (params (DeltaSeconds :type Float%20%28single-precision%29))
  (|CallParentFunction DeltaSeconds) ; This node is disabled and will not be called.\nDrag off pins to build functionality.
)

(fn ConstructionScript
  (|CallParentFunction))

(fn CanFinalizeQuest
  (params (Ingredients :type Ingredients%20Enum :default "NewEnumerator9"))
  (bind _asbp_builder (Utilities|Casting|CastToBP_Builder (Variables|Default|GetSpawnedNPC)))
  (if (ScalableFloat|GetValueasBool (AI|GetBlackboard _asbp_builder) (Variables|Default|GetHookStolenKey))
    (if (Utilities|Array|ContainsItem (Variables|Default|GetPendingQuestEnd) Ingredients)
      (Utilities|Array|RemoveItem (Variables|Default|GetPendingQuestEnd) Ingredients)
      (return true)
      (else
        _))
    (else
      (Utilities|Array|AddUnique (Variables|Default|GetPendingQuestEnd) Ingredients)))
  (return false))