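; Quest Blueprint for the first vegetable quest, which delegates its start and end to the green grocer character.
; StartQuest gets the QuestManager from the FastFoodGameState, looks up the "GreenGrocer" actor reference, caches it as Babuska and passes itself to the grocer's start call.
; EndQuest forwards to that cached grocer, so the quest itself holds no objective logic.
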(event EventBeginPlay
  (|CallParentFunction) ; This node is disabled and will not be called.\nDrag off pins to build functionality.
)

(event Collision|EventActorBeginOverlap
  (params (OtherActor :type Actor%20Object%20Reference))
  (|CallParentFunction OtherActor) ; This node is disabled and will not be called.\nDrag off pins to build functionality.
)

(event EventTick
  (params (DeltaSeconds :type Float%20%28single-precision%29))
  (|CallParentFunction DeltaSeconds) ; This node is disabled and will not be called.\nDrag off pins to build functionality.
)

(event EventStartQuest
  (bind _asfast_food_game_state (Utilities|Casting|CastToFastFoodGameState (Game|GetGameState)))
  (bind _output_get (Variables|Default|SetQuestManager (Variables|/Game/FFBlueprints/GameMode/FastFoodGameState.FastFoodGameState_C|GetQuestManager _asfast_food_game_state)))
  (bind _value (Default|GetActorReference _output_get "GreenGrocer"))
  (bind _asbp_green_grocer (Utilities|Casting|CastToBP_GreenGrocer _value))
  (bind _output_get_2 (Variables|Default|SetBabuska _asbp_green_grocer))
  (Default|CAlltoStartQuest _output_get_2 self))

(event EventEndQuest
  (Default|CalltoEndQuest (Variables|Default|GetBabuska)))

(fn ConstructionScript
  (|CallParentFunction))