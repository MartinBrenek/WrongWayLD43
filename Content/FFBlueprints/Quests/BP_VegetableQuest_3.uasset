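; BP_VegetableQuest_3 is a quest Blueprint, by name the third vegetable quest, built around the Bald King NPC.
; Its debug setup runs the parent logic, then casts the spawned NPC to BP_BaldKing and sets a preset state on its Bald King state component.
; Ending the quest delegates to BaldGuy through CallToEndQuest, while spawning and other quest logic are not defined here.
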(event EventBeginPlay
  (|CallParentFunction) ; This node is disabled and will not be called.\nDrag off pins to build functionality.
)

(event Collision|EventActorBeginOverlap
  (params (OtherActor :type Actor%20Object%20Reference))
  (|CallParentFunction OtherActor) ; This node is disabled and will not be called.\nDrag off pins to build functionality.
)

(event EventTick
  (params (DeltaSeconds :type Float%20%28single-precision%29))
  (|CallParentFunction DeltaSeconds) ; This node is disabled and will not be called.\nDrag off pins to build functionality.
)

(event EventEndQuest
  (Default|CalltoEndQuest (Variables|Default|GetBaldGuy)))

(event EventRunDebugSetup
  (|CallParentFunction)
  (bind _asbp_bald_king (Utilities|Casting|CastToBP_BaldKing (Variables|Default|GetSpawnedNPC)))
  (Default|SetStateBaldKing (Variables|/Game/FFBlueprints/NPC/BaldKing/BP_BaldKing.BP_BaldKing_C|GetBP_BaldkingState _asbp_bald_king) "NewEnumerator2"))

(fn ConstructionScript
  (|CallParentFunction))