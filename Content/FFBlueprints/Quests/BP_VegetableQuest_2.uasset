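; BP_VegetableQuest_2 is a quest Blueprint that hands the start of a vegetable quest to the BaldGuy NPC.
; StartQuest waits half a second, looks up "BaldGuy" through the game state's QuestManager, caches it as a BP_BaldKing and calls CAllToStartQuest on it with itself.
; EndQuest is empty, and the default BeginPlay, overlap and Tick events are disabled.
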(event EventBeginPlay
  (|CallParentFunction) ; This node is disabled and will not be called.\nDrag off pins to build functionality.
)

(event Collision|EventActorBeginOverlap
  (params (OtherActor :type Actor%20Object%20Reference))
  (|CallParentFunction OtherActor) ; This node is disabled and will not be called.\nDrag off pins to build functionality.
)

(event EventTick
  (params (DeltaSeconds :type Float%20%28single-precision%29))
  (|CallParentFunction DeltaSeconds) ; This node is disabled and will not be called.\nDrag off pins to build functionality.
)

(event EventStartQuest
  (bind _asfast_food_game_state (Utilities|Casting|CastToFastFoodGameState (Game|GetGameState)))
  (Utilities|FlowControl|Delay 0.5)
  (bind _output_get (Variables|Default|SetQuestManager (Variables|/Game/FFBlueprints/GameMode/FastFoodGameState.FastFoodGameState_C|GetQuestManager _asfast_food_game_state)))
  (bind (_value _found) (Default|GetActorReference _output_get "BaldGuy"))
  (if _found
    (bind _asbp_bald_king (Utilities|Casting|CastToBP_BaldKing _value))
    (bind _output_get_2 (Variables|Default|SetBaldGuy _asbp_bald_king))
    (Default|CAlltoStartQuest _output_get_2 self)))

(event EventEndQuest)

(fn ConstructionScript
  (|CallParentFunction))