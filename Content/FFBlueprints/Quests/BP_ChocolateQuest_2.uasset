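; Second stage of the Chocolate quest, which puts the quest dog into its first phase and has Babuska call to end the quest.
; On start it looks up the Dog actor in the QuestManager, falling back to debug setup if it is missing.
; Debug setup spawns the dog at the Kennel with the Greengrocer as owner, opens the dog toy and assigns it to the dog, logging failed lookups.
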(event EventBeginPlay
  (|CallParentFunction) ; This node is disabled and will not be called.\nDrag off pins to build functionality.
)

(event Collision|EventActorBeginOverlap
  (params (OtherActor :type Actor%20Object%20Reference))
  (|CallParentFunction OtherActor) ; This node is disabled and will not be called.\nDrag off pins to build functionality.
)

(event EventTick
  (params (DeltaSeconds :type Float%20%28single-precision%29))
  (|CallParentFunction DeltaSeconds) ; This node is disabled and will not be called.\nDrag off pins to build functionality.
)

(event EventEndQuest
  (Default|CalltoEndQuest (Variables|Default|GetBabuska)))

(event EventStartQuest
  (bind _asfast_food_game_state (Utilities|Casting|CastToFastFoodGameState (Game|GetGameState)))
  (bind _output_get (Variables|Default|SetQuestManager (Variables|/Game/FFBlueprints/GameMode/FastFoodGameState.FastFoodGameState_C|GetQuestManager _asfast_food_game_state)))
  (bind (_value _found) (Default|GetActorReference _output_get "Dog"))
  (if _found
    (bind _asbp_dog (Utilities|Casting|CastToBP_Dog _value))
    (Variables|Default|SetDogActor _asbp_dog)
    (else
      (CallFunction|RunDebugSetup)))
  (Variables|/Game/FFBlueprints/NPC/Animals/Dog/BP_Dog.BP_Dog_C|SetPhase (Variables|Default|GetDogActor) 1))

(event EventRunDebugSetup
  (|CallParentFunction)
  (CallFunction|SpawnandSetupDog))

(fn ConstructionScript
  (|CallParentFunction))

(fn SpawnandSetupDog
  (bind _dogtoytoyname (Variables|Default|GetDogToyToyName))
  (bind _greengrocer (Variables|Default|GetGreengrocer))
  (bind _kennel (Variables|Default|GetKennel))
  (Utilities|FlowControl|Sequence
    (:then_0
      (bind _value (Default|GetActorReference (Variables|Default|GetQuestManager) (Utilities|String|StringToName _greengrocer)))
      (bind _ascrowd_character (Utilities|Casting|CastToCrowdCharacter _value)
        (:then
          (LocalVariables|SetDogOwner _ascrowd_character))
        (:CastFailed
          (Utilities|WrongReference _greengrocer))))
    (:then_1
      (bind _poi (Default|GetBasePOI (CallFunction|GetNPCManager) _kennel))
      (bind _asbp_kennel (Utilities|Casting|CastToBP_Kennel _poi)
        (:then
          (bind _instance (Default|SpawnAnimal _asbp_kennel "/Game/FFBlueprints/NPC/Animals/Dog/BP_Dog.BP_Dog_C" (LocalVariables|GetDogOwner)))
          (bind _asbp_dog (Utilities|Casting|CastToBP_Dog _instance))
          (Variables|Default|SetDogActor _asbp_dog))
        (:CastFailed
          (Utilities|WrongReference _kennel))))
    (:then_2
      (bind _poi_2 (Default|GetBasePOI (CallFunction|GetNPCManager) _dogtoytoyname))
      (bind _asbt_dog_toy_toy (Utilities|Casting|CastToBT_DogToyToy _poi_2)
        (:then
          (Default|Open _asbt_dog_toy_toy)
          (Default|SetActualObject (Variables|Default|GetDogActor) _asbt_dog_toy_toy))
        (:CastFailed
          (Utilities|WrongReference _dogtoytoyname))))))