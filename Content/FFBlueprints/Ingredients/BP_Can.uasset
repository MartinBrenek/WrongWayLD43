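; BP_Can is a can ingredient that turns into a sausage when combined with a BP_Condom item.
; On a match, CombineWithItem disables its mesh physics and collision, spawns a Sausage at its transform, and returns success with flags allowing destruction and release.
; Any other item fails with flags that block both.
; IsReadyToUse always returns true, and the event graph holds only disabled stubs.
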(event EventBeginPlay
  (|CallParentFunction) ; This node is disabled and will not be called.\nDrag off pins to build functionality.
)

(event Collision|EventActorBeginOverlap
  (params (OtherActor :type Actor%20Object%20Reference))
  (|CallParentFunction OtherActor) ; This node is disabled and will not be called.\nDrag off pins to build functionality.
)

(event EventTick
  (params (DeltaSeconds :type Float%20%28single-precision%29))
  (|CallParentFunction DeltaSeconds) ; This node is disabled and will not be called.\nDrag off pins to build functionality.
)

(fn ConstructionScript
  (|CallParentFunction))

(fn CombinewithItem
  (params (ItemToCombine :type Actor%20Object%20Reference))
  (bind _self self)
  (Utilities|Casting|CastToBP_Condom ItemToCombine
    (:then
      (Physics|SetSimulatePhysics (Variables|Default|GetStaticMesh _self) false)
      (Collision|SetCollisionEnabled (Variables|Default|GetStaticMesh _self) "NoCollision")
      (Game|SpawnActorfromClass "/Game/FFBlueprints/Ingredients/Sausage.Sausage_C" (Transformation|GetActorTransform _self) "Undefined" 0 0)
      (return true false false true))
    (:CastFailed
      (return false true true false))))

(fn IsReadytoUse
  (return true))