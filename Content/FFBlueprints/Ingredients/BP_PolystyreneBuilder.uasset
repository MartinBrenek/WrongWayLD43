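; BP_PolystyreneBuilder is an ingredient Blueprint that reports readiness and can fade itself out of the world.
; Its IsReadyToUse override returns true only while the LiftComponent has not started lifting.
; Disappear waits briefly, then creates a dynamic material on the Cube mesh and drives its "Hide" parameter with the FadeOut timeline, destroying the actor when the fade finishes.
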(event Custom|Disappear
  (bind _cube (Variables|Default|GetCube))
  (Utilities|FlowControl|Delay 1.0)
  (bind _returnvalue (Rendering|Material|CreateDynamicMaterialInstance _cube 0 (Utilities|Array|Get(acopy) (Rendering|Material|GetMaterials _cube)) "None" :!class /Script/Engine.PrimitiveComponent))
  (bind _newtrack_0 (Timeline|FadeOut Play)
    (:Update
      (Rendering|Material|SetScalarParameterValue _returnvalue "Hide" _newtrack_0 :!class /Script/Engine.MaterialInstanceDynamic))
    (:Finished
      (Actor|DestroyActor))))

(event EventBeginPlay
  (|CallParentFunction))

(event Collision|EventActorBeginOverlap
  (params (OtherActor :type Actor%20Object%20Reference))
  (|CallParentFunction OtherActor) ; This node is disabled and will not be called.\nDrag off pins to build functionality.
)

(event EventTick
  (params (DeltaSeconds :type Float%20%28single-precision%29))
  (|CallParentFunction DeltaSeconds) ; This node is disabled and will not be called.\nDrag off pins to build functionality.
)

(fn ConstructionScript
  (|CallParentFunction))

(fn IsReadytoUse
  (|CallParentFunction)
  (return (not (Variables|/Game/FFBlueprints/LiftComponent.LiftComponent_C|GetLiftStarted (Variables|Default|GetLiftComponent)))))