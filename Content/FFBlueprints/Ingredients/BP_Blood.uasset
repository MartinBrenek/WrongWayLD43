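; BP_Blood is a blood ingredient that works as a source for the player's injection item.
; IsReadyToUse is true only while the first-person character's PickedActor is a BP_Injection.
; CombineWithItem calls FeedUp on an injection and reports success, flagging it neither to be destroyed nor released.
; Any other item fails the combine, and the event graph holds no logic.
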(event EventBeginPlay)

(event Collision|EventActorBeginOverlap
  (params (OtherActor :type Actor%20Object%20Reference)))

(event EventTick
  (params (DeltaSeconds :type Float%20%28single-precision%29)))

(fn ConstructionScript)

(fn CombinewithItem
  (params (ItemToCombine :type Actor%20Object%20Reference))
  (bind _asbp_injection (Utilities|Casting|CastToBP_Injection ItemToCombine)
    (:then
      (Default|FeedUp _asbp_injection)
      (return true true true))
    (:CastFailed
      (return false true false))))

(fn IsReadytoUse
  (bind _asfirst_person_character (Utilities|Casting|CastToFirstPersonCharacter (Game|Player|GetPlayerPawn 0))
    (:then
      (Utilities|Casting|CastToBP_Injection (Variables|/Game/FirstPersonBP/Blueprints/FirstPersonCharacter.FirstPersonCharacter_C|GetPickedActor _asfirst_person_character)
        (:then
          (return true))
        (:CastFailed
          _)))
    (:CastFailed
      _))
  (return false))