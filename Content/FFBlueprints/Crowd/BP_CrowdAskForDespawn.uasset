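; Behavior tree task that sends an AI-controlled crowd character off to be despawned.
; It asks the NPC manager for an available despawner, registers the character with it for destruction, and writes the returned vector to the target blackboard key.
; It succeeds after registering and fails when no valid despawner exists, but never finishes if either controller or character cast fails.
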(event EventReceiveExecute
  (params (OwnerActor :type Actor%20Object%20Reference))
  (bind _ascrowd_aicontroller (Utilities|Casting|CastToCrowdAIController OwnerActor))
  (bind _ascrowd_character (Utilities|Casting|CastToCrowdCharacter (Pawn|GetControlledPawn _ascrowd_aicontroller)))
  (Variables|Default|SetCrowd _ascrowd_character)
  (bind _despawner (Default|GetAviableDespawner (CallFunction|GetNPCManager)))
  (Utilities|IsValid _despawner
    (:Is%20Valid
      (bind _destroypoint (Default|RegisterCrowdtoDestroy _despawner (Variables|Default|GetCrowd)))
      (AI|BehaviorTree|SetBlackboardValueasVector (Variables|Default|GetTargetKey) _destroypoint)
      (AI|BehaviorTree|FinishExecute true))
    (:Is%20Not%20Valid
      (AI|BehaviorTree|FinishExecute false))))