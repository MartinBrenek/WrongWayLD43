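; Behavior tree task that finds and occupies a free point of interest for a crowd NPC.
; With a valid cycle config, it asks the NPC manager for the next POI type and clears the config on a work-in-progress leave-cycle result; without one, it searches using the current type.
; A found node updates the cycle config and blackboard object and location keys; the task succeeds only when one is found.
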(event EventReceiveExecute
  (params (OwnerActor :type Actor%20Object%20Reference))
  (bind _npcpoimanager (CallFunction|GetNPCManager))
  (bind _ascrowd_aicontroller (Utilities|Casting|CastToCrowdAIController OwnerActor))
  (bind _ascrowd_character (Utilities|Casting|CastToCrowdCharacter (Pawn|GetControlledPawn _ascrowd_aicontroller)))
  (Utilities|IsValid (Variables|/Game/FFBlueprints/Crowd/CrowdCharacter.CrowdCharacter_C|GetCurrentConfig _ascrowd_character)
    (:Is%20Valid
      (bind _nextstate (Default|GetNextPOI _npcpoimanager (Variables|/Game/FFBlueprints/Crowd/CrowdCharacter.CrowdCharacter_C|GetCurrentPOI _ascrowd_character) (Variables|/Game/FFBlueprints/Crowd/CrowdCharacter.CrowdCharacter_C|GetCurrentConfig _ascrowd_character)))
      ;[1 1 1] WIP - Leave Cycle
      (if (Utilities|Enum|Equal(Enum) _nextstate "NewEnumerator4")
        (Variables|/Game/FFBlueprints/Crowd/CrowdCharacter.CrowdCharacter_C|SetCurrentConfig _ascrowd_character 0)
        (AI|BehaviorTree|FinishExecute false)
        (else
          (Variables|/Game/FFBlueprints/Crowd/CrowdCharacter.CrowdCharacter_C|SetCurrentPOI _ascrowd_character _nextstate)
          (bind (_outputnode _cycledefinition _found) (Default|FindandOccupyPOI _npcpoimanager false (Variables|/Game/FFBlueprints/Crowd/CrowdCharacter.CrowdCharacter_C|GetCurrentPOI _ascrowd_character) :!label _label))
          (if _found
            (Class|BTFunctionLibrary|SetBlackboardValueasObject (Variables|Default|GetActualObject) _outputnode)
            (Variables|/Game/FFBlueprints/Crowd/CrowdCharacter.CrowdCharacter_C|SetCurrentConfig _ascrowd_character _cycledefinition)
            (AI|BehaviorTree|SetBlackboardValueasVector (Variables|Default|GetFleeToLocation) (Transformation|GetActorLocation _outputnode)))
          (AI|BehaviorTree|FinishExecute _found))))
    (:Is%20Not%20Valid
      (goto _label))))