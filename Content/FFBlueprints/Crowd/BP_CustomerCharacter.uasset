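; Crowd customer character for the fast food game that waits in a queue and takes its food order.
; At queue index 0, WantOrder gets an order from FastFoodManager or a DebugManager override.
; CatchOrder overlap checks food class, attaches a match to the Finger, clears the queue front and saves a checkpoint; the food is destroyed with the customer.
; Debug aids include player-facing queue index text and drawn capsule hit points.
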(event OnComponentBeginOverlap(CatchOrder)
  (params (OverlappedComponent :type Primitive%20Component%20Object%20Reference) (OtherActor :type Actor%20Object%20Reference) (OtherComp :type Primitive%20Component%20Object%20Reference) (OtherBodyIndex :type Integer) (bFromSweep :type Boolean) (SweepResult :type Hit%20Result%20Structure%20%28by%20ref%29))
  (if (Variables|Default|GetIsWaitingForOrder)
    (bind _ascomplete_food (Utilities|Casting|CastToCompleteFood OtherActor))
    (if (== (Utilities|GetClass _ascomplete_food) (Variables|Default|GetOrdered))
      (Collision|SetCollisionEnabled (Variables|/Game/FFBlueprints/PickableItem.PickableItem_C|GetCube _ascomplete_food) "NoCollision")
      (Physics|SetSimulatePhysics (Variables|/Game/FFBlueprints/PickableItem.PickableItem_C|GetCube _ascomplete_food) false)
      (Transformation|AttachComponentToComponent _ascomplete_food (Variables|Default|GetFinger) "" "SnapToTarget" "SnapToTarget" "KeepRelative" true)
      (Variables|Default|SetItemInHand _ascomplete_food)
      (Variables|Default|SetOrderCompleted true)
      (Variables|Default|SetIsWaitingForOrder false)
      (Default|ClearFirst (Variables|Default|GetActualQueue))
      (Default|SaveCheckPoint (CallFunction|GetFastFoodGameState))
      (else
        (CallFunction|DebugLog "Using wrong complete food ( kurva co jsi podelal?)" "NewEnumerator2")))))

(event OnComponentHit(CapsuleComponent)
  (params (HitComponent :type Primitive%20Component%20Object%20Reference) (OtherActor :type Actor%20Object%20Reference) (OtherComp :type Primitive%20Component%20Object%20Reference) (NormalImpulse :type Vector :default "0, 0, 0") (Hit :type Hit%20Result%20Structure%20%28by%20ref%29))
  (Rendering|Debug|DrawDebugPoint (.ImpactPoint (Collision|BreakHitResult Hit)) 2.0 "(R=1.000000,G=0.000000,B=0.705616,A=1.000000)" 3e+01))

(event Custom|WantOrder
  (bind _fastfoodgamestate (CallFunction|GetFastFoodGameState))
  (bind _debugmanager (Variables|/Game/FFBlueprints/GameMode/FastFoodGameState.FastFoodGameState_C|GetDebugManager _fastfoodgamestate))
  (if (and (== (Variables|Default|GetActualNodeIndex) 0) (not (Variables|Default|GetIsWaitingForOrder)))
    (Variables|Default|SetIsWaitingForOrder true)
    (if (Default|GetUseInstantNewOrder _debugmanager)
      (Variables|Default|SetOrdered (Variables|/Game/FFBlueprints/Debug/BP_DebugFastFoodManager.BP_DebugFastFoodManager_C|GetOrdered _debugmanager))
      (else
        (bind _finalproduct (Default|CreateNewOrder (CallFunction|GetFastFoodManager)))
        (Variables|Default|SetOrdered _finalproduct)))))

(event EventBeginPlay
  (|CallParentFunction) ; This node is disabled and will not be called.\nDrag off pins to build functionality.
)

(event Collision|EventActorBeginOverlap
  (params (OtherActor :type Actor%20Object%20Reference))
  (|CallParentFunction OtherActor) ; This node is disabled and will not be called.\nDrag off pins to build functionality.
)

(event EventTick
  (params (DeltaSeconds :type Float%20%28single-precision%29))
  (|CallParentFunction DeltaSeconds)
  (CallFunction|UpdateDebugInfo))

(event EventDestroyed
  (|CallParentFunction)
  (Utilities|IsValid (Variables|Default|GetItemInHand)
    (:Is%20Valid
      (Actor|DestroyActor (Variables|Default|GetItemInHand)))))

(fn ConstructionScript
  (|CallParentFunction))

(fn UpdateDebugInfo
  (if (Variables|Default|GetShowDebugInfo)
    (Utilities|FlowControl|Sequence
      (:then_0
        (|Show))
      (:then_1
        (|LookOnPlayerText))
      (:then_2
        (Rendering|Components|TextRender|SetText (Variables|Default|GetDebugInfo) (Utilities|Text|ToText(String) (Utilities|String|Append "Actual index: " (Utilities|String|ToString(Integer) (Variables|Default|GetActualNodeIndex)))))))
    (else
      (|Hide))))