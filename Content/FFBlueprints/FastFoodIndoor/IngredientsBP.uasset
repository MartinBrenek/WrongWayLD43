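; IngredientsBP is a pick-up fast-food ingredient that can be placed on the workbench.
; It lazily caches the FastFoodManager from the game state and is ready only while its Type is among the manager's current ingredients and it is unused.
; TryAddToWorkBench hands it to the manager and stores the result as Used.
; It always refuses item combining, and saves its class and transform, teleporting back on load.
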(event Custom|UseItem_1
  (Default|CallItemPicked))

(event Custom|LoadedData_1
  (params (Data :type Save%20Object%20Data%20Structure))
  (Transformation|SetActorTransform (.TransforMain (Utilities|Struct|BreakSaveObjectData Data)) false true))

(event EventBeginPlay)

(event Collision|EventActorBeginOverlap
  (params (OtherActor :type Actor%20Object%20Reference)))

(event EventTick
  (params (DeltaSeconds :type Float%20%28single-precision%29)))

(event EventUseItem
  (CallFunction|PickUpInternal)
  (Default|CallItemPicked))

(fn ConstructionScript)

(fn GetFastFoodManager
  (Utilities|IsValid (Variables|Default|GetFastFoodManager)
    (:Is%20Valid
      _)
    (:Is%20Not%20Valid
      (bind _asfast_food_game_state (Utilities|Casting|CastToFastFoodGameState (Game|GetGameState)))
      (Variables|Default|SetFastFoodManager (Variables|/Game/FFBlueprints/GameMode/FastFoodGameState.FastFoodGameState_C|GetFastFoodManger _asfast_food_game_state))))
  (return (Variables|Default|GetFastFoodManager)))

(fn IsReadytoUse
  (return (and (Default|IsinActualIngrediets (CallFunction|GetFastFoodManager) (Variables|Default|GetType)) (not (Variables|Default|GetUsed)))))

(fn CombinewithItem
  (params (ItemToCombine :type Actor%20Object%20Reference))
  (return false false false false))

(fn GetSaveData
  (return (Utilities|Struct|MakeSaveObjectData (Utilities|GetClass self) (Transformation|GetActorTransform self))))

(fn TryAddtoWorkBench
  (bind _correct (Default|AddIngredient (CallFunction|GetFastFoodManager) self))
  (bind _output_get (Variables|Default|SetUsed _correct))
  (return _output_get))