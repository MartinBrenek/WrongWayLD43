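; BP_HotDogEatable is a hot dog item in the indoor fast food scene that starts the fast food phase when used.
; It cannot be picked up or combined, and is usable only once a prerequisite tutorial has been shown.
; On use it starts the phase through the game state, shows the one-time customer tutorial through the fast food manager and destroys itself.
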(event EventBeginPlay)

(event Collision|EventActorBeginOverlap
  (params (OtherActor :type Actor%20Object%20Reference)))

(event EventTick
  (params (DeltaSeconds :type Float%20%28single-precision%29)))

(event EventUseItem
  (Default|StartFastFoodPhase (CallFunction|GetFastFoodGameState))
  (Default|ShowTutorial (CallFunction|GetFastFoodManager) "Tut_Customer" true)
  (Actor|DestroyActor))

(fn ConstructionScript)

(fn CombinewithItem
  (params (ItemToCombine :type Actor%20Object%20Reference))
  (return false false false false))

(fn IsReadytoPickUp
  (return false))

(fn IsReadytoUse
  (return (Default|WasShowedTutorial (CallFunction|GetFastFoodManager) (Variables|Default|GetDependendentTutName))))