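; BP_car is a car that loops along a spline while CarMoving is set, with a random body material picked in the construction script.
; Tick advances Distance by Speed, and SetCarAtDistance wraps it at the spline's end and aligns MeshPivot to the location and tangent.
; Construction also places the car at its Distance.
; ActivateBlood reveals the Blood component and BloodObj actor; an older Timeline movement loop is left disconnected.
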(event EventBeginPlay)

(event Collision|EventActorBeginOverlap
  (params (OtherActor :type Actor%20Object%20Reference)))

(event EventTick
  (params (DeltaSeconds :type Float%20%28single-precision%29))
  (if (Variables|Default|GetCarMoving)
    (Variables|Default|SetDistance (+ (Variables|Default|GetDistance) (* DeltaSeconds (Variables|Default|GetSpeed))))
    (CallFunction|SetCaratDistance)))

(fn ConstructionScript
  (Rendering|Material|SetMaterial (Variables|Default|Getcar_test3) 0 (Utilities|Array|Get(acopy) (Variables|Default|GetCarMaterials) (Math|Random|RandomIntegerinRange 0 5)))
  (CallFunction|SetCaratDistance))

(fn SetCaratDistance
  (bind _spline (Variables|Default|GetSpline))
  (if (> (Variables|Default|GetDistance) (Spline|GetSplineLength (Variables|Default|GetSpline)))
    (Variables|Default|SetDistance 0.0))
  (Transformation|SetWorldTransform (Variables|Default|GetMeshPivot) (Math|Transform|MakeTransform (Spline|GetLocationatDistanceAlongSpline _spline (Variables|Default|GetDistance) "World") (Math|Rotator|MakeRotfromX (Spline|GetTangentatDistanceAlongSpline _spline (Variables|Default|GetDistance) "World"))) false false))

(fn ActivateBlood
  (Rendering|SetVisibility (Variables|Default|GetBlood) true false)
  (Rendering|SetActorHiddenInGame (Variables|Default|GetBloodObj) false))