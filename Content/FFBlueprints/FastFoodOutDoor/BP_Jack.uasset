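; BP_Jack is a usable car jack item that drops the vehicle it is linked to.
; UseItem only acts while the player's FirstPersonCharacter has SlowTime active, in which case it calls BulletTimePressed.
; If a Vehicle is valid, it shifts the jack and its Cube along negative Y and calls DropCar on the vehicle.
; The parent UseItem then runs, still only under the SlowTime condition.
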(event EventBeginPlay
  (|CallParentFunction) ; This node is disabled and will not be called.\nDrag off pins to build functionality.
)

(event Collision|EventActorBeginOverlap
  (params (OtherActor :type Actor%20Object%20Reference))
  (|CallParentFunction OtherActor) ; This node is disabled and will not be called.\nDrag off pins to build functionality.
)

(event EventTick
  (params (DeltaSeconds :type Float%20%28single-precision%29))
  (|CallParentFunction DeltaSeconds) ; This node is disabled and will not be called.\nDrag off pins to build functionality.
)

(event EventUseItem
  (bind _returnvalue (Transformation|GetActorLocation))
  (bind _vehicle (Variables|Default|GetVehicle))
  (bind _returnvalue_2 (- _returnvalue "0,40.000000, 0"))
  (bind _asfirst_person_character (Utilities|Casting|CastToFirstPersonCharacter (Game|GetPlayerCharacter 0)))
  (if (Variables|/Game/FirstPersonBP/Blueprints/FirstPersonCharacter.FirstPersonCharacter_C|GetSlowTime _asfirst_person_character)
    (Default|BulletTimePressed _asfirst_person_character)
    (Utilities|IsValid _vehicle
      (:Is%20Valid
        (Transformation|SetActorLocation _returnvalue_2 false false)
        (Transformation|SetWorldLocation (Variables|Default|GetCube) _returnvalue_2 false false)
        (Default|DropCar _vehicle))
      (:Is%20Not%20Valid
        _))
    (|CallParentFunction)))

(fn ConstructionScript
  (|CallParentFunction))