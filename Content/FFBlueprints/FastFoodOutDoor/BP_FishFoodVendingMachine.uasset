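; BP_FishFoodVendingMachine is an interactable fish food vending machine that turns metal when combined with a BoltCup item.
; CombineWithItem accepts only a BoltCup, calling Change to apply MI_metal to the Sphere and set IsMetal.
; It can never be picked up and reports ready to use only until it has turned metal.
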(event Custom|Change
  (Rendering|Material|SetMaterial (Variables|Default|GetSphere) 0 "/Game/assets/stall/MI_metal.MI_metal")
  (Variables|Default|SetIsMetal true))

(event EventBeginPlay)

(event Collision|EventActorBeginOverlap
  (params (OtherActor :type Actor%20Object%20Reference)))

(event EventTick
  (params (DeltaSeconds :type Float%20%28single-precision%29)))

(fn ConstructionScript)

(fn CombinewithItem
  (params (ItemToCombine :type Actor%20Object%20Reference))
  (Utilities|Casting|CastToBoltCup ItemToCombine
    (:then
      (CallFunction|Change)
      (return true false false false))
    (:CastFailed
      (return false false false false))))

(fn IsReadytoPickUp
  (return false))

(fn IsReadytoUse
  (return (not (Variables|Default|GetIsMetal))))