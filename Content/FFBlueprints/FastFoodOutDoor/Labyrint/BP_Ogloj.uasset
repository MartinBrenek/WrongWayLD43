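; BP_Ogloj is a segmented actor in the outdoor labyrinth, built from cylinders and a sphere along a spline.
; UpdateSkeleton spreads the PartArray components by spline length in local space, changing only their location.
; The construction script fills the array and runs that layout.
; BeginPlay starts the PFPathFollower and refills the array, while Tick is empty, so this graph does not refresh the layout at runtime.
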(event Custom|UpdateSkeleton
  (bind _partarray (Variables|Default|GetPartArray))
  (for (_array_element _array_index) _partarray
    (Transformation|SetRelativeLocation _array_element (.Location (Math|Transform|BreakTransform (Spline|GetTransformatDistanceAlongSpline (Variables|Default|GetSpline) (* _array_index (/ (Spline|GetSplineLength (Variables|Default|GetSpline)) (Math|Conversions|ToFloat(Integer) (- (Utilities|Array|Length _partarray) 2)))) "Local" false))) false false)))

(event EventBeginPlay
  (Class|PFPathFollowerComponent|Start (Variables|Default|GetPFPathFollower) 0.0)
  (Variables|Default|SetPartArray (Utilities|Array|MakeArray (Variables|Default|GetCylinder0) (Variables|Default|GetCylinder1) (Variables|Default|GetCylinder2) (Variables|Default|GetCylinder3) (Variables|Default|GetSphere) 0)))

(event Collision|EventActorBeginOverlap
  (params (OtherActor :type Actor%20Object%20Reference)))

(event EventTick
  (params (DeltaSeconds :type Float%20%28single-precision%29)))

(fn ConstructionScript
  (Variables|Default|SetPartArray (Utilities|Array|MakeArray (Variables|Default|GetCylinder0) (Variables|Default|GetCylinder1) (Variables|Default|GetCylinder2) (Variables|Default|GetCylinder3) (Variables|Default|GetSphere) 0))
  (CallFunction|UpdateSkeleton))