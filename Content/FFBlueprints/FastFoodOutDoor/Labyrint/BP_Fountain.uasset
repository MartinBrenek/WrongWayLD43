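; BP_Fountain is an interactable fountain in the outdoor labyrinth that fills a bucket and ends the player's LSD sequence.
; CombineWithItem accepts only a BP_Bucket, fills it, triggers DelayedAction and returns success while keeping the bucket from being destroyed or released.
; After a short delay, DelayedAction teleports the FirstPersonCharacter to the LSD exit and turns off the LSD effect.
; The fountain always reports itself ready to use.
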(event Custom|DelayedAction
  (Utilities|FlowControl|Delay 0.5)
  (bind _asfirst_person_character (Utilities|Casting|CastToFirstPersonCharacter (Game|GetPlayerCharacter 0)))
  (Default|TeleporttoLSDExit _asfirst_person_character)
  (Default|TurnLSDEffect _asfirst_person_character false))

(event EventBeginPlay)

(event Collision|EventActorBeginOverlap
  (params (OtherActor :type Actor%20Object%20Reference)))

(event EventTick
  (params (DeltaSeconds :type Float%20%28single-precision%29)))

(fn ConstructionScript)

(fn CombinewithItem
  (params (ItemToCombine :type Actor%20Object%20Reference))
  (bind _asbp_bucket (Utilities|Casting|CastToBP_Bucket ItemToCombine))
  (Default|FillBucket _asbp_bucket)
  (CallFunction|DelayedAction)
  (return true true true))

(fn IsReadytoUse
  (return true))