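; UFO actor that flies above a target actor to abduct it, then accelerates to an exit point and destroys itself.
; Tick steps horizontally toward the target, then sphere-traces down to choose a response through the target's LiftComponent.
; Hitting the target or a player lifts it, releasing it from that player's grip; otherwise it disappears unless the player holds it.
; Completion callbacks destroy the target and resume flight, triggering the departure.
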(event Custom|SetupUfo
  (params (EndPoint :type Vector) (Target :type Actor%20Object%20Reference))
  (Variables|Default|SetEndPoint EndPoint)
  (Variables|Default|SetTargetActor Target))

(event Custom|PickedUp
  (params (Tween :type Tween%20Vector%20Object%20Reference))
  (Actor|DestroyActor (Variables|Default|GetTargetActor))
  (Variables|Default|SetStop false)
  (Variables|Default|SetTargetActor 0))

(event Custom|LiftTarget
  (bind _targetactor (Variables|Default|GetTargetActor))
  (bind _returnvalue (Actor|GetComponentbyClass _targetactor "/Game/FFBlueprints/LiftComponent.LiftComponent_C"))
  (Utilities|IsValid _returnvalue
    (:Is%20Valid
      (Variables|Default|SetStop true)
      (Default|Lift _returnvalue (Transformation|GetWorldLocation (Variables|Default|GetStaticMesh)) true (delegate Custom|PickedUp)))))

(event Custom|DisappearTarget
  (bind _targetactor (Variables|Default|GetTargetActor))
  (bind _returnvalue (Actor|GetComponentbyClass _targetactor "/Game/FFBlueprints/LiftComponent.LiftComponent_C"))
  (Utilities|IsValid _returnvalue
    (:Is%20Valid
      (Variables|Default|SetStop true)
      (Default|Disappear _returnvalue 0 true (delegate Custom|Disappeared)))))

(event Custom|Disappeared
  (params (Tween :type Tween%20Float%20Object%20Reference))
  (CallFunction|PickedUp))

(event EventBeginPlay)

(event Collision|EventActorBeginOverlap
  (params (OtherActor :type Actor%20Object%20Reference)))

(event EventTick
  (params (DeltaSeconds :type Float%20%28single-precision%29))
  (bind _returnvalue (Transformation|GetActorLocation))
  (if (not (Variables|Default|GetStop))
    (Utilities|IsValid (Variables|Default|GetTargetActor)
      (:Is%20Valid
        (bind (_newloction _reached) (CallFunction|MoveTowardsLocation (Variables|Default|GetSpeed) DeltaSeconds (Transformation|GetActorLocation (Variables|Default|GetTargetActor)) true 5e+01))
        (if _reached
          (bind _outhit (Collision|SphereTraceForObjects _returnvalue (- _returnvalue "0, 0,2000.000000") 1e+02 (Utilities|Array|MakeArray "ObjectTypeQuery8" "ObjectTypeQuery11" "ObjectTypeQuery1") false 0 "ForOneFrame"))
          (if (== (.HitActor (Collision|BreakHitResult _outhit)) (Variables|Default|GetTargetActor))
            (CallFunction|LiftTarget)
            (else
              (bind _asfirst_person_character (Utilities|Casting|CastToFirstPersonCharacter (.HitActor (Collision|BreakHitResult _outhit)))
                (:then
                  (if (== (Variables|/Game/FirstPersonBP/Blueprints/FirstPersonCharacter.FirstPersonCharacter_C|GetPickedActor _asfirst_person_character) (Variables|Default|GetTargetActor))
                    (Default|ReleaseItem _asfirst_person_character))
                  (CallFunction|LiftTarget))
                (:CastFailed
                  (if (not (== (Variables|/Game/FirstPersonBP/Blueprints/FirstPersonCharacter.FirstPersonCharacter_C|GetPickedActor (CallFunction|GetPlayer)) (Variables|Default|GetTargetActor)))
                    (CallFunction|DisappearTarget))))))
          (else
            (Transformation|SetActorLocation _newloction false false))))
      (:Is%20Not%20Valid
        (bind (_newloction_2 _reached_2) (CallFunction|MoveTowardsLocation (* (Variables|Default|GetSpeed) 2.0) DeltaSeconds (Variables|Default|GetEndPoint) false 5e+01))
        (if _reached_2
          (Actor|DestroyActor)
          (else
            (Transformation|SetActorLocation _newloction_2 false false)
            (Variables|Default|SetSpeed (Math|Float|Min(Float) (+ (* (* (Variables|Default|GetSpeed) 1e+01) DeltaSeconds) (Variables|Default|GetSpeed)) 5e+03))))))))

(fn ConstructionScript)

(fn MoveTowardsLocation
  (params (Speed :type Float%20%28single-precision%29) (DeltaTime :type Float%20%28single-precision%29) (Target :type Vector) (KeeepZ :type Boolean) (ReachRadius :type Float%20%28single-precision%29))
  (bind _returnvalue (Transformation|GetActorLocation))
  (bind (_x _y) (Math|Vector|BreakVector Target))
  (LocalVariables|SetTargetLocation Target)
  (if KeeepZ
    (LocalVariables|SetTargetLocation (Math|Vector|MakeVector _x _y (.Z (Math|Vector|BreakVector _returnvalue)))))
  (return (Math|Vector|Lerp(Vector) _returnvalue (LocalVariables|GetTargetLocation) (/ (* DeltaTime Speed) (Math|Vector|Distance(Vector) (LocalVariables|GetTargetLocation) _returnvalue))) (<= (Math|Vector|Distance(Vector) (LocalVariables|GetTargetLocation) _returnvalue) ReachRadius)))