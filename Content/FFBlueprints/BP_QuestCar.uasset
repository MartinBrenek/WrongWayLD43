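; BP_QuestCar is a quest car actor that drops on command and then reveals blood.
; DropCar plays a timeline that animates the car mesh's relative height and roll, then fires CarFell and calls ActivateBlood.
; ActivateBlood shows the Blood component and enables BloodObj, which BeginPlay hides with collision off.
; SetCarAtDistance aligns the mesh pivot along a spline, resetting past its end, but nothing here calls it.
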(event Custom|DropCar
  (bind _car_test3 (Variables|Default|Getcar_test3))
  (bind _car_moving_loop (Timeline|Car%20moving%20loop Play)
    (:Update
      (Transformation|SetRelativeLocation _car_test3 (Math|Vector|MakeVector 0.0 0.0 (Math|Float|MapRangeClamped _car_moving_loop 0.0 1.0 25.0 0.0)) false false)
      (Transformation|SetRelativeRotation _car_test3 (Math|Rotator|MakeRotator (Math|Float|MapRangeClamped _car_moving_loop 0.0 1.0 25.0 0.0) 0.0 0.0) false false))
    (:Finished
      (Default|CallCarFell)
      (CallFunction|ActivateBlood))))

(event EventBeginPlay
  (bind _bloodobj (Variables|Default|GetBloodObj))
  (Rendering|SetActorHiddenInGame _bloodobj true)
  (Collision|SetActorEnableCollision _bloodobj false))

(event Collision|EventActorBeginOverlap
  (params (OtherActor :type Actor%20Object%20Reference)))

(event EventTick
  (params (DeltaSeconds :type Float%20%28single-precision%29)))

(fn ConstructionScript)

(fn SetCaratDistance
  (bind _spline (Variables|Default|GetSpline))
  (if (> (Variables|Default|GetDistance) (Spline|GetSplineLength (Variables|Default|GetSpline)))
    (Variables|Default|SetDistance 0.0))
  (Transformation|SetWorldTransform (Variables|Default|GetMeshPivot) (Math|Transform|MakeTransform (Spline|GetLocationatDistanceAlongSpline _spline (Variables|Default|GetDistance) "World") (Math|Rotator|MakeRotfromX (Spline|GetTangentatDistanceAlongSpline _spline (Variables|Default|GetDistance) "World"))) false false))

(fn ActivateBlood
  (bind _bloodobj (Variables|Default|GetBloodObj))
  (Rendering|SetVisibility (Variables|Default|GetBlood) true false)
  (Rendering|SetActorHiddenInGame _bloodobj false)
  (Collision|SetActorEnableCollision _bloodobj true))