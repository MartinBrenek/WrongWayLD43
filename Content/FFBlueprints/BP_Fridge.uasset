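; BP_Fridge is a fridge actor with a door and interior light, apparently scripted for cinematics.
; FridgeCineOpen and FridgeCineClose trigger events that each run once, playing a timeline that rotates the door in opposite directions.
; The door turns by a fixed increment per timeline update rather than interpolating, so total swing depends on frame rate.
; FridgeLightOn and FridgeLightOff switch the point light by setting its intensity.
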(event Custom|CineOpen
  (Utilities|FlowControl|DoOnce false
    (:Completed
      (Timeline|Timeline_0 Play
        (:Update
          (Transformation|AddLocalRotation (Variables|Default|Getfridge_door) "0,-1.000000,0.000000" false false))))))

(event Custom|CineClose
  (Utilities|FlowControl|DoOnce false
    (:Completed
      (Timeline|Timeline_1 Play
        (:Update
          (Transformation|AddLocalRotation (Variables|Default|Getfridge_door) "0,1.000000,0.000000" false false))))))

(event EventBeginPlay)

(event Collision|EventActorBeginOverlap
  (params (OtherActor :type Actor%20Object%20Reference)))

(event EventTick
  (params (DeltaSeconds :type Float%20%28single-precision%29)))

(fn ConstructionScript)

(fn FridgeLighton
  (Rendering|Components|Light|SetIntensity (Variables|Default|GetPointLight) 3e+02))

(fn FridgeLightOff
  (Rendering|Components|Light|SetIntensity (Variables|Default|GetPointLight) 0.0))

(fn FridgeCineOpen
  (CallFunction|CineOpen))

(fn FridgeCineClose
  (CallFunction|CineClose))