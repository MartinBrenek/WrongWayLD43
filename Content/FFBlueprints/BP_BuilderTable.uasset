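; BP_BuilderTable is the builder's table, spawning and removing a hammer and hook at arm positions, with the hammer placed on BeginPlay.
; Spawned hooks bind a pickup event.
; The hook pickup handler, only when the player's SlowTime is set, calls BulletTime and notifies BP_Builder that the hook was stolen.
; A SetupOperator macro lazily finds and caches that builder from the game state's QuestManager reference list.
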(event Custom|HookPickUp
  (bind _asfirst_person_character (Utilities|Casting|CastToFirstPersonCharacter (Game|GetPlayerCharacter 0)))
  (if (Variables|/Game/FirstPersonBP/Blueprints/FirstPersonCharacter.FirstPersonCharacter_C|GetSlowTime _asfirst_person_character)
    (Default|BulletTime _asfirst_person_character)
    (Utilities|SetupOperator
      (:Out
        (bind _asbp_builder (Utilities|Casting|CastToBP_Builder (Variables|Default|GetOperator)))
        (Default|HookStolen _asbp_builder)))))

(event EventBeginPlay
  (CallFunction|UpdateHammer true))

(event Collision|EventActorBeginOverlap
  (params (OtherActor :type Actor%20Object%20Reference)))

(event EventTick
  (params (DeltaSeconds :type Float%20%28single-precision%29)))

(fn ConstructionScript)

(fn UpdateHook
  (params (ShouldSpawn :type Boolean))
  (bind _larmposition (Variables|Default|GetLArmPosition))
  (bind _returnvalue (Transformation|GetWorldTransform _larmposition))
  (if ShouldSpawn
    (bind _returnvalue_2 (Game|SpawnActorfromClass "/Game/FFBlueprints/FastFoodOutDoor/Hook.Hook_C" (Math|Transform|MakeTransform (.location _returnvalue) (.rotation _returnvalue) "1,1,1") "AdjustIfPossibleButAlwaysSpawn" 0 0))
    (EventDispatchers|BindEventtoPickUpEvent _returnvalue_2 (EventDispatchers|CreateEvent :!event Custom|HookPickUp))
    (bind _output_get (Variables|Default|SetLPositionObj _returnvalue_2))
    (Variables|Default|SetCurrentItem _output_get)
    (else
      (Utilities|IsValid (Variables|Default|GetLPositionObj)
        (:Is%20Valid
          (bind _ashook (Utilities|Casting|CastToHook (Variables|Default|GetLPositionObj))
            (:then
              (EventDispatchers|UnbindallEventsfromItemPickedbyPlayer _ashook))
            (:CastFailed
              _))
          (Actor|DestroyActor (Variables|Default|GetLPositionObj)))))))

(fn UpdateHammer
  (params (ShouldSpawn :type Boolean))
  (bind _rarmposition (Variables|Default|GetRArmPosition))
  (bind _returnvalue (Transformation|GetWorldTransform _rarmposition))
  (if ShouldSpawn
    (bind _returnvalue_2 (Game|SpawnActorfromClass "/Game/FFBlueprints/FastFoodOutDoor/Hammer.Hammer_C" (Math|Transform|MakeTransform (.location _returnvalue) (.rotation _returnvalue) "1,1,1") "AdjustIfPossibleButAlwaysSpawn" 0 0))
    (bind _output_get (Variables|Default|SetRPositionObj _returnvalue_2))
    (Variables|Default|SetCurrentItem _output_get)
    (else
      (Utilities|IsValid (Variables|Default|GetRPositionObj)
        (:Is%20Valid
          (Actor|DestroyActor (Variables|Default|GetRPositionObj)))))))