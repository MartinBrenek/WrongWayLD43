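; Base animation instance Blueprint for crowd characters, caching its owning CrowdCharacter at BeginPlay.
; UpdateBaseAnimatorState converts a key to a byte through the owner and checks whether it is a base action.
; Base keys switch on shared actions (Sitting, Walking, Running, Idle) with empty branches, then clear UseCustomAnimGraph.
; Other keys pass their byte to UpdateAnimatorState; the per-frame update event is unused.
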(event Custom|Event%20Update%20Base%20Animator%20State
  (params (Key :type Blackboard%20Key%20Selector%20Structure))
  (bind (_byte _base) (Default|GetBytefromKey (Variables|Default|GetBaseOwner) Key))
  (if _base
    (switch Utilities|FlowControl|Switch|SwitchonE_SharedActions (Utilities|Enum|ByteToEnumE_SharedActions _byte)
      (:NewEnumerator0
        _)
      (:NewEnumerator1
        _)
      (:NewEnumerator2
        _)
      (:NewEnumerator3
        _))
    (Variables|Default|SetUseCustomAnimGraph 0.0)
    (else
      (Class|BaseAnimInstance|UpdateAnimatorState _byte))))

(event EventBlueprintUpdateAnimation
  (params (DeltaTimeX :type Float%20%28single-precision%29)))

(event EventBlueprintBeginPlay
  (bind _returnvalue (Class|AnimInstance|TryGetPawnOwner))
  (Utilities|IsValid _returnvalue
    (:Is%20Valid
      (bind _ascrowd_character (Utilities|Casting|CastToCrowdCharacter _returnvalue))
      (Variables|Default|SetBaseOwner _ascrowd_character))))