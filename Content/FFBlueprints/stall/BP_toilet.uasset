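; Toilet prop actor in a stall that plays a one-shot water effect five seconds after play begins.
; The construction script creates dynamic material instances for the toilet and its water mesh.
; A timeline drives the toilet material's water_opacity for leaks; after a further short delay, the water mesh plays its animation while a second timeline drives the water material's normal_power.
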(event EventBeginPlay
  (Utilities|FlowControl|Delay 5.0)
  (Utilities|FlowControl|Sequence
    (:then_0
      (bind _toilet_leaks (Timeline|toilet_water_anim Play)
        (:Update
          (Rendering|Material|SetScalarParameterValue (Variables|Default|Gettoilet_material) "water_opacity" _toilet_leaks :!class /Script/Engine.MaterialInstanceDynamic))))
    (:then_1
      (Utilities|FlowControl|Delay 1.2)
      (Components|Animation|PlayAnimation (Variables|Default|Gettoilet_water) "/Game/assets/stall/furniture/toilet_water_Anim.toilet_water_Anim" false)
      (bind _normal_power (Timeline|Water_material_parameters PlayFromStart)
        (:Update
          (Rendering|Material|SetScalarParameterValue (Variables|Default|Getwater_material) "normal_power" _normal_power :!class /Script/Engine.MaterialInstanceDynamic))))))

(event Collision|EventActorBeginOverlap
  (params (OtherActor :type Actor%20Object%20Reference)))

(event EventTick
  (params (DeltaSeconds :type Float%20%28single-precision%29)))

(fn ConstructionScript
  (bind _returnvalue (Rendering|Material|CreateDynamicMaterialInstance (Variables|Default|Gettoilet_water) 0 "/Game/assets/stall/furniture/M_toilet_water_Inst.M_toilet_water_Inst" "None" :!class /Script/Engine.PrimitiveComponent))
  (Variables|Default|Setwater_material _returnvalue)
  (bind _returnvalue_2 (Rendering|Material|CreateDynamicMaterialInstance (Variables|Default|Gettoilet) 0 "/Game/assets/stall/furniture/MI_toilet.MI_toilet" "None" :!class /Script/Engine.PrimitiveComponent))
  (Variables|Default|Settoilet_material _returnvalue_2))