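; BP_FlushHandle is a usable toilet flush handle in a stall that is always ready to use and rejects item combining.
; On use it calls CallFlushed and tweens the Handle component's rotation to a pressed pitch or yaw angle.
; When that tween ends it waits briefly, then tweens the handle's rotation to the opposite angle.
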(event Custom|CustomEvent_0
  (params (Tween :type Tween%20Rotator%20Object%20Reference))
  (Utilities|FlowControl|Delay 1.0)
  (Class|TweenRotatorStandardFactory|CreateTweenRotateSceneComponentto 0 (Variables|Default|GetHandle) "-70.000000,0.000000,0.000000" 1.0 "Linear"))

(event EventBeginPlay)

(event Collision|EventActorBeginOverlap
  (params (OtherActor :type Actor%20Object%20Reference)))

(event EventTick
  (params (DeltaSeconds :type Float%20%28single-precision%29)))

(event EventUseItem
  (Default|CallFlushed)
  (bind _tween (Class|TweenRotatorStandardFactory|CreateTweenRotateSceneComponentto 0 (Variables|Default|GetHandle) "70.000000,0.000000,0.000000" 1.0 "Linear"))
  (EventDispatchers|BindEventtoOnTweenEnd _tween (delegate Custom|CustomEvent_0)))

(fn ConstructionScript)

(fn CombinewithItem
  (params (ItemToCombine :type Actor%20Object%20Reference))
  (return false false false false))

(fn IsReadytoUse
  (return true))