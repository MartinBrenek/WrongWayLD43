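; BP_UfoSpline is a UFO actor that flies in, lifts a target object away, then leaves and destroys itself.
; RunTask, given a valid LiftComponent on the target, tweens the UFO along an inbound spline, then random per-tick nudges shake it during the lift.
; The lift callback destroys the object and tweens the UFO out along a second spline.
; The target's pick-up event clears the references, so an arriving UFO leaves empty-handed.
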(event Custom|RunTask
  (Utilities|IsValid (Variables|Default|GetLiftObjectComponent)
    (:Is%20Valid
      (bind _tween (Class|TweenFloatStandardFactory|CreateTweenSceneComponentFollowSpline 0 (Variables|Default|GetUfoObject) (Variables|Default|GetInNavSpline) 3.0 true false true "Linear"))
      (EventDispatchers|BindEventtoOnTweenEnd _tween (delegate Custom|Complete)))))

(event Custom|Complete
  (params (Tween :type Tween%20Float%20Object%20Reference))
  (Variables|Default|SetShaking true)
  (Utilities|IsValid (Variables|Default|GetLiftObjectComponent)
    (:Is%20Valid
      (Default|Lift (Actor|GetComponentbyClass (Variables|Default|GetObjectToPickUp) "/Game/FFBlueprints/LiftComponent.LiftComponent_C") (Transformation|GetActorLocation) (delegate Custom|FlyAway)))
    (:Is%20Not%20Valid
      (CallFunction|FlyAway))))

(event Custom|End
  (params (Tween :type Tween%20Float%20Object%20Reference))
  (Actor|DestroyActor))

(event Custom|FlyAway
  (params (Tween :type Tween%20Vector%20Object%20Reference))
  (bind _objecttopickup (Variables|Default|GetObjectToPickUp))
  (Utilities|IsValid _objecttopickup
    (:Is%20Valid
      (Actor|DestroyActor _objecttopickup))
    (:Is%20Not%20Valid
      _))
  (Variables|Default|SetShaking false)
  (bind _tween (Class|TweenFloatStandardFactory|CreateTweenSceneComponentFollowSpline 0 (Variables|Default|GetUfoObject) (Variables|Default|GetOutNavSpline) 1e+01 true false true "EaseInOutQuad"))
  (EventDispatchers|BindEventtoOnTweenEnd _tween (delegate Custom|End)))

(event Custom|PickedTarget
  (params (RefToSelf :type Pickable%20Item%20Object%20Reference))
  (Variables|Default|SetLiftObjectComponent 0)
  (Variables|Default|SetObjectToPickUp 0))

(event EventBeginPlay
  (bind _objecttopickup (Variables|Default|GetObjectToPickUp))
  (Transformation|SetWorldLocation (Variables|Default|GetUfoObject) (Spline|GetLocationatSplinePoint (Variables|Default|GetInNavSpline) 0 "World") true true)
  (Utilities|IsValid _objecttopickup
    (:Is%20Valid
      (Variables|Default|SetLiftObjectComponent (Actor|GetComponentbyClass _objecttopickup "/Game/FFBlueprints/LiftComponent.LiftComponent_C"))
      (EventDispatchers|AssignPickUpEvent _objecttopickup (delegate Custom|PickedTarget)))))

(event EventTick
  (params (DeltaSeconds :type Float%20%28single-precision%29))
  (if (Variables|Default|GetShaking)
    (Class|TweenVectorStandardFactory|CreateTweenMoveSceneComponentby 0 (Variables|Default|GetUfoObject) (Math|Random|RandomUnitVector) 0.05 "Linear")))

(fn ConstructionScript)