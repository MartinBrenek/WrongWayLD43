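; Cinematic manager that registers with FastFoodGameState and plays cutscene Level Sequences requested by clip enum.
; PlayClip wraps a sequence player in a ClipData object, playing it immediately or queuing it while another plays; the last queued clip plays next.
; Start and finish callbacks broadcast dispatchers and apply or revert per-clip setup: player input lock, UI hiding and skippability.
; Spacebar skips the current clip, with manager input enabled for skippable clips.
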(event Custom|StartedSequance)

(event Custom|FinishedSequence)

(event Custom|PlayClip
  (params (Clip :type CinematicClips%20Enum :default "NewEnumerator0") (Setup :type Sequence%20Setup%20Structure))
  (bind _cutscenes (Variables|Default|GetCutScenes))
  (bind (_value _returnvalue) (Utilities|Map|Find _cutscenes Clip))
  (if _returnvalue
    (bind _outactor (Sequencer|Player|CreateLevelSequencePlayer _value (Utilities|MakePlaybackSettingfromSetup Setup)))
    (bind _returnvalue_2 (Game|ConstructObjectfromClass "/Game/FFBlueprints/CinematicSequance/ClipData.ClipData_C" self Clip Setup _outactor))
    (Default|SetupCallbacks _returnvalue_2 (delegate Custom|Started) (delegate Custom|Finished))
    (Utilities|IsValid (Variables|Default|GetCurrentPlaying)
      (:Is%20Valid
        (Utilities|Array|Add (Variables|Default|GetQueue) _returnvalue_2))
      (:Is%20Not%20Valid
        (Utilities|PlayThis _returnvalue_2)))))

(event Custom|Finished
  (params (ClipData :type Clip%20Data%20Object%20Reference))
  (CallFunction|AfterEndPlay ClipData)
  (Default|CallOnFinishedSequence (Variables|/Game/FFBlueprints/CinematicSequance/ClipData.ClipData_C|GetClipEnum ClipData))
  (Variables|Default|SetCurrentPlaying 0)
  (CallFunction|CheckQueue))

(event Custom|Started
  (params (ClipData :type Clip%20Data%20Object%20Reference))
  (CallFunction|AfterSatrtPlay ClipData)
  (Default|CallOnStartSequence (Variables|/Game/FFBlueprints/CinematicSequance/ClipData.ClipData_C|GetClipEnum ClipData)))

(event EventBeginPlay
  (bind _asfast_food_game_state (Utilities|Casting|CastToFastFoodGameState (Game|GetGameState)))
  (Variables|/Game/FFBlueprints/GameMode/FastFoodGameState.FastFoodGameState_C|SetCinematicManager _asfast_food_game_state self))

(event Collision|EventActorBeginOverlap
  (params (OtherActor :type Actor%20Object%20Reference)))

(event EventTick
  (params (DeltaSeconds :type Float%20%28single-precision%29)))

(event Input|KeyboardEvents|SpaceBar
  (params (Key :type Key%20Structure :default "None"))
  (:Pressed
    (Default|Skip (Variables|Default|GetCurrentPlaying))))

(fn ConstructionScript)

(fn CheckQueue
  (bind _queue (Variables|Default|GetQueue))
  (bind _returnvalue (Utilities|Array|LastIndex _queue))
  (if (> (Utilities|Array|Length _queue) 0)
    (Utilities|PlayThis (Utilities|Array|Get(acopy) (Variables|Default|GetQueue) _returnvalue))
    (Utilities|Array|RemoveIndex (Variables|Default|GetQueue) _returnvalue)))

(fn AfterSatrtPlay
  (params (ClipData :type Clip%20Data%20Object%20Reference))
  (bind _player (CallFunction|GetPlayer))
  (bind _setup (Variables|/Game/FFBlueprints/CinematicSequance/ClipData.ClipData_C|GetSetup ClipData))
  (bind (_hideui _skipable _disableplayersinput) (Utilities|Struct|BreakSequenceSetup _setup))
  (Utilities|FlowControl|Sequence
    (:then_0
      (if _disableplayersinput
        (Input|DisableInput _player 0)))
    (:then_1
      (if _skipable
        (Input|EnableInput (Game|GetPlayerController 0))))
    (:then_2
      (if _hideui
        (Default|HideUI _player true)))))

(fn AfterEndPlay
  (params (ClipData :type Clip%20Data%20Object%20Reference))
  (bind _setup (Variables|/Game/FFBlueprints/CinematicSequance/ClipData.ClipData_C|GetSetup ClipData))
  (bind (_hideui _skipable _disableplayersinput) (Utilities|Struct|BreakSequenceSetup _setup))
  (Utilities|FlowControl|Sequence
    (:then_0
      (if _disableplayersinput
        (Input|EnableInput (CallFunction|GetPlayer) 0)))
    (:then_1
      (if _skipable
        (Input|DisableInput 0)))
    (:then_2
      (if _hideui
        (Default|HideUI (CallFunction|GetPlayer) false)))))