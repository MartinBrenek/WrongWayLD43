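; Dog NPC Blueprint that poops on demand and exposes item-use hooks.
; StartShiting pulses an animation flag on the lazily cached Dog_Anim instance and marks pooping in progress until StopShit.
; When capped, each call raises the dog_inflated morph target instead of spawning a Shit actor at Arrow1.
; CombineWithItem accepts any item despite its BP_BottleCap cast, and IsReadyToUse is always true.
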(event Custom|StartShiting
  (if (Utilities|IsValid (Variables|Default|GetAnimator))
    _
    (else
      (bind _asdog_anim (Utilities|Casting|CastToDog_Anim (Components|SkeletalMesh|GetAnimInstance (Variables|Character|GetMesh))))
      (Variables|Default|SetAnimator _asdog_anim)))
  (Variables|/Game/FFBlueprints/NPC/Dog/Dog_Anim.Dog_Anim_C|SetShit (Variables|Default|GetAnimator) true)
  (Variables|Default|SetPoopInProgress true)
  (if (Variables|Default|GetCaped)
    (Variables|Default|SetValue (+ (Variables|Default|GetValue) 0.3))
    (Components|SkeletalMesh|SetMorphTarget (Variables|Character|GetMesh) "dog_inflated" (Variables|Default|GetValue) true)
    (else
      (Game|SpawnActorfromClass "/Game/FFBlueprints/FastFoodOutDoor/Shit.Shit_C" (Transformation|GetWorldTransform (Variables|Default|GetArrow1)) "Undefined" 0 0)))
  (Utilities|FlowControl|Delay 0.2)
  (Variables|/Game/FFBlueprints/NPC/Dog/Dog_Anim.Dog_Anim_C|SetShit (Variables|Default|GetAnimator) false))

(event Custom|StopShit
  (Variables|Default|SetPoopInProgress false))

(event EventBeginPlay)

(event Collision|EventActorBeginOverlap
  (params (OtherActor :type Actor%20Object%20Reference)))

(event EventTick
  (params (DeltaSeconds :type Float%20%28single-precision%29)))

(fn ConstructionScript)

(fn CombinewithItem
  (params (ItemToCombine :type Actor%20Object%20Reference))
  (Utilities|Casting|CastToBP_BottleCap ItemToCombine
    (:then
      (return true))
    (:CastFailed
      (return true))))

(fn IsReadytoUse
  (return true))