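; Base behavior tree task that assigns an NPC crowd character to a named point of interest (POI).
; SetupPOI gets the POI from the NPC manager and asks it for that pawn's transform and task.
; It writes the POI and world-space move location to the blackboard, then sets the new task.
; Its own execute event is empty, and SetupPOI finishes execution only when the POI is found.
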(event EventReceiveExecute
  (params (OwnerActor :type Actor%20Object%20Reference)))

(fn SetupActorLocation
  (params (POI :type Base%20POI%20Actor%20Object%20Reference) (AIController :type BP%20NPC%20Base%20AI%20Controller%20Object%20Reference) (RelativeCompLoc :type Vector))
  (bind _returnvalue (Transformation|GetActorTransform POI))
  (bind _returnvalue_2 (AI|GetBlackboard AIController))
  (bind _returnvalue_3 (Math|Transform|TransformLocation _returnvalue RelativeCompLoc))
  (AI|Components|Blackboard|SetValueasObject _returnvalue_2 (Variables|Default|GetActualObject) POI)
  (AI|Components|Blackboard|SetValueasVector _returnvalue_2 (Variables|Default|GetMoveToLocation_0) (Math|Vector|MakeVector (.x _returnvalue_3) (.y _returnvalue_3) (.z _returnvalue_3))))

(fn SetupPOI
  (params (POIName :type String) (OwnerActor :type Actor%20Object%20Reference))
  (bind _asbp_npcbase_aicontroller (Utilities|Casting|CastToBP_NPCBaseAIController OwnerActor))
  (bind _ascrowd_character (Utilities|Casting|CastToCrowdCharacter (Pawn|GetControlledPawn _asbp_npcbase_aicontroller)))
  (bind (_poi _found) (Default|GetBasePOI (CallFunction|GetNPCManager) POIName))
  (if _found
    (bind (_transform _task) (Default|GetNPCInfobyPawn _poi _ascrowd_character))
    (CallFunction|SetupActorLocation _poi _asbp_npcbase_aicontroller (.location _transform))
    (CallFunction|SetNewTask OwnerActor _task)
    (AI|BehaviorTree|FinishExecute true)))