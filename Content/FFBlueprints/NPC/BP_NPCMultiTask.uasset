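; BP_NPCMultiTask is a behavior tree task that moves an NPC on to its next point of interest and that point's behavior.
; It asks BP_NPCBaseAIController for the POI following the current ActualObject blackboard value.
; The POI's Task asset is injected as a dynamic subtree on the BTDynamicTask tag, and the POI becomes the new ActualObject.
; The task then finishes successfully; a failed cast leaves it unfinished.
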(event EventReceiveExecute
  (params (OwnerActor :type Actor%20Object%20Reference))
  (bind _actualobject (Variables|Default|GetActualObject))
  (bind _asbp_npcbase_aicontroller (Utilities|Casting|CastToBP_NPCBaseAIController OwnerActor))
  (bind _nextpoi (Default|GetNextPoi _asbp_npcbase_aicontroller (AI|Components|Blackboard|GetValueasObject (AI|GetBlackboard _asbp_npcbase_aicontroller) _actualobject)))
  (bind _asbehavior_tree_component (Utilities|Casting|CastToBehaviorTreeComponent (Variables|/Script/AIModule.AIController|GetBrainComponent _asbp_npcbase_aicontroller)))
  (Class|BehaviorTreeComponent|SetDynamicSubtree _asbehavior_tree_component "(TagName=\"BTDynamicTask\")" (Variables|/Game/FFBlueprints/NPC/BP_NPCPOI.BP_NPCPOI_C|GetTask _nextpoi))
  (AI|Components|Blackboard|SetValueasObject (AI|GetBlackboard _asbp_npcbase_aicontroller) _actualobject _nextpoi)
  (AI|BehaviorTree|FinishExecute true))