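; AI controller for the builder NPC that switches it between idle crowd, woodcutter and hook builder behaviors.
; SetupAI selects the matching blackboard for the requested state and, for the two work roles, copies target objects from the controlled BP_Builder and flags InQuest.
; Each branch passes the blackboard to SetOwnerPawn, sets the current behavior tree asset and converges on TryChangeBT to apply it.
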(event Custom|SetupAI
  (params (AIState :type BuilderState%20Enum :default "NewEnumerator0"))
  (bind _asbp_builder (Utilities|Casting|CastToBP_Builder (Pawn|GetControlledPawn)))
  (switch Utilities|FlowControl|Switch|SwitchonBuilderState AIState
    (:NewEnumerator0
      (bind _blackboardcomponent (Class|AIController|UseBlackboard "/Game/FFBlueprints/Crowd/BBCrowd.BBCrowd"))
      (CallFunction|SetOwnerPawn _blackboardcomponent)
      (Variables|Default|SetCurrentBTAsset "/Game/FFBlueprints/Crowd/BTCrowd.BTCrowd"))
    (:NewEnumerator1
      (bind _blackboardcomponent_2 (Class|AIController|UseBlackboard "/Game/FFBlueprints/NPC/Builder/WoodCutter/BB_Woodcutter.BB_Woodcutter"))
      (AI|Components|Blackboard|SetValueasObject _blackboardcomponent_2 (Variables|Default|GetWoodCutter) (Variables|/Game/FFBlueprints/NPC/Builder/BP_Builder.BP_Builder_C|GetWoodCutter _asbp_builder))
      (AI|Components|Blackboard|SetValueasObject _blackboardcomponent_2 (Variables|Default|GetStorage) (Variables|/Game/FFBlueprints/NPC/Builder/BP_Builder.BP_Builder_C|GetStorage _asbp_builder))
      (AI|Components|Blackboard|SetValueasObject _blackboardcomponent_2 (Variables|Default|GetHouse) (Variables|/Game/FFBlueprints/NPC/Builder/BP_Builder.BP_Builder_C|GetHouse _asbp_builder))
      (AI|Components|Blackboard|SetValueasBool _blackboardcomponent_2 (Variables|Default|GetInQuest) true)
      (CallFunction|SetOwnerPawn _blackboardcomponent_2)
      (Variables|Default|SetCurrentBTAsset "/Game/FFBlueprints/NPC/Builder/WoodCutter/BT_Woodcutter.BT_Woodcutter"))
    (:NewEnumerator2
      (bind _blackboardcomponent_3 (Class|AIController|UseBlackboard "/Game/FFBlueprints/NPC/Builder/HookBuilder/BB_HookBuilder.BB_HookBuilder"))
      (AI|Components|Blackboard|SetValueasObject _blackboardcomponent_3 (Variables|Default|GetPolystyrene) (Variables|/Game/FFBlueprints/NPC/Builder/BP_Builder.BP_Builder_C|GetPolystyrene _asbp_builder))
      (AI|Components|Blackboard|SetValueasObject _blackboardcomponent_3 (Variables|Default|GetHouse) (Variables|/Game/FFBlueprints/NPC/Builder/BP_Builder.BP_Builder_C|GetPolystyreneHouse _asbp_builder))
      (AI|Components|Blackboard|SetValueasObject _blackboardcomponent_3 (Variables|Default|GetTable) (Variables|/Game/FFBlueprints/NPC/Builder/BP_Builder.BP_Builder_C|GetTable _asbp_builder))
      (AI|Components|Blackboard|SetValueasObject _blackboardcomponent_3 (Variables|Default|GetRopeStand) (Variables|/Game/FFBlueprints/NPC/Builder/BP_Builder.BP_Builder_C|GetRopeStand _asbp_builder))
      (AI|Components|Blackboard|SetValueasObject _blackboardcomponent_3 (Variables|Default|GetPolystyrenePlace) (Variables|/Game/FFBlueprints/NPC/Builder/BP_Builder.BP_Builder_C|GetPolystyrenePlace _asbp_builder))
      (AI|Components|Blackboard|SetValueasBool _blackboardcomponent_3 (Variables|Default|GetInQuest) true)
      (CallFunction|SetOwnerPawn _blackboardcomponent_3)
      (Variables|Default|SetCurrentBTAsset "/Game/FFBlueprints/NPC/Builder/HookBuilder/BT_HookBuilder.BT_HookBuilder")))
  (CallFunction|TryChangeBT))

(fn ConstructionScript
  (|CallParentFunction))