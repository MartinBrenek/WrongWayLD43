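; AI controller for the woodcutter NPC that prepares its blackboard when play begins.
; It requires a BP_Builder pawn and copies that pawn's WoodCutter, Storage and House references into BB_Woodcutter, along with an InQuest flag set to true.
; It then passes the blackboard to SetOwnerPawn and calls the parent BeginPlay last, which is skipped if the pawn cast fails.
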(event EventBeginPlay
  (bind _asbp_builder (Utilities|Casting|CastToBP_Builder (Pawn|GetControlledPawn)))
  (bind _blackboardcomponent (Class|AIController|UseBlackboard "/Game/FFBlueprints/NPC/Builder/WoodCutter/BB_Woodcutter.BB_Woodcutter"))
  (AI|Components|Blackboard|SetValueasObject _blackboardcomponent (Variables|Default|GetWoodCutter) (Variables|/Game/FFBlueprints/NPC/Builder/BP_Builder.BP_Builder_C|GetWoodCutter _asbp_builder))
  (AI|Components|Blackboard|SetValueasObject _blackboardcomponent (Variables|Default|GetStorage) (Variables|/Game/FFBlueprints/NPC/Builder/BP_Builder.BP_Builder_C|GetStorage _asbp_builder))
  (AI|Components|Blackboard|SetValueasObject _blackboardcomponent (Variables|Default|GetHouse) (Variables|/Game/FFBlueprints/NPC/Builder/BP_Builder.BP_Builder_C|GetHouse _asbp_builder))
  (AI|Components|Blackboard|SetValueasBool _blackboardcomponent (Variables|Default|GetInQuest) true)
  (CallFunction|SetOwnerPawn _blackboardcomponent)
  (|CallParentFunction))

(event EventTick
  (params (DeltaSeconds :type Float%20%28single-precision%29)))

(fn ConstructionScript
  (|CallParentFunction))