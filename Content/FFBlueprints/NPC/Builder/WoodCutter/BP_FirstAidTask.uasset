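; Behavior tree task that applies first aid to a builder NPC, ending its bleeding effect.
; On execute it reads the Owner object from the blackboard and casts it to BP_Builder.
; It deactivates and clears any valid bleeding particle system, resets max walk speed to the builder's WalkSpeed and finishes successfully.
; A failed cast stops without finishing the task.
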(event EventReceiveExecute
  (params (OwnerActor :type Actor%20Object%20Reference))
  (bind _asbp_builder (Utilities|Casting|CastToBP_Builder (AI|Components|Blackboard|GetValueasObject (AI|GetBlackboard OwnerActor) (Variables|Default|GetOwner))))
  (Utilities|IsValid (Variables|/Game/FFBlueprints/NPC/Builder/BP_Builder.BP_Builder_C|GetBleedingPS _asbp_builder)
    (:Is%20Valid
      (Components|Activation|Deactivate (Variables|/Game/FFBlueprints/NPC/Builder/BP_Builder.BP_Builder_C|GetBleedingPS _asbp_builder))
      (Variables|/Game/FFBlueprints/NPC/Builder/BP_Builder.BP_Builder_C|SetBleedingPS _asbp_builder 0))
    (:Is%20Not%20Valid
      _))
  (Variables|/Script/Engine.CharacterMovementComponent|SetMaxWalkSpeed (Variables|/Script/Engine.Character|GetCharacterMovement _asbp_builder) (Variables|/Game/FFBlueprints/Crowd/CrowdCharacter.CrowdCharacter_C|GetWalkSpeed _asbp_builder))
  (AI|BehaviorTree|FinishExecute true))