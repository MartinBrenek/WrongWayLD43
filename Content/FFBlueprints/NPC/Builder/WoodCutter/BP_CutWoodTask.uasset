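; Behavior tree task that makes a woodcutter builder NPC perform its wood-cutting animation.
; On execute it sets the AnimationRunning blackboard flag and calls Cutting on the BP_Builder stored as Owner.
; Tick polls that flag until it is cleared outside this task, then hides the log, sets desk wood visibility from HandCut, resets animator values and finishes successfully.
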(event EventReceiveExecute
  (params (OwnerActor :type Actor%20Object%20Reference))
  (bind _returnvalue (AI|GetBlackboard OwnerActor))
  (AI|Components|Blackboard|SetValueasBool _returnvalue (Variables|Default|GetAnimationRunning) true)
  (bind _asbp_builder (Utilities|Casting|CastToBP_Builder (AI|Components|Blackboard|GetValueasObject _returnvalue (Variables|Default|GetOwner))))
  (Default|Cutting _asbp_builder))

(event EventTick
  (params (OwnerActor :type Actor%20Object%20Reference) (DeltaSeconds :type Float%20%28single-precision%29))
  (bind _returnvalue (AI|GetBlackboard OwnerActor))
  (if (not (ScalableFloat|GetValueasBool _returnvalue (Variables|Default|GetAnimationRunning)))
    (bind _asbp_builder (Utilities|Casting|CastToBP_Builder (AI|Components|Blackboard|GetValueasObject _returnvalue (Variables|Default|GetOwner))))
    (Rendering|SetVisibility (Variables|/Game/FFBlueprints/NPC/Builder/BP_Builder.BP_Builder_C|GetLogWood _asbp_builder) false false)
    (Rendering|SetVisibility (Variables|/Game/FFBlueprints/NPC/Builder/BP_Builder.BP_Builder_C|GetDeskWood _asbp_builder) (not (ScalableFloat|GetValueasBool _returnvalue (Variables|Default|GetHandCut))) false)
    (Variables|/Game/FFBlueprints/NPC/Builder/BPA_Builder.BPA_Builder_C|SetIsCutting (Variables|/Game/FFBlueprints/NPC/Builder/BP_Builder.BP_Builder_C|GetAnimator _asbp_builder) false)
    (Variables|/Game/FFBlueprints/NPC/Builder/BPA_Builder.BPA_Builder_C|SetUseBabushkaCustom (Variables|/Game/FFBlueprints/NPC/Builder/BP_Builder.BP_Builder_C|GetAnimator _asbp_builder) 1.0)
    (AI|BehaviorTree|FinishExecute true)))