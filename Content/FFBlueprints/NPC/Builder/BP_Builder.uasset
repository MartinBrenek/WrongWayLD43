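; Builder NPC whose roles include wood cutter, hook builder and car repairman, with hand-cutting and death gore.
; BuilderState changes reconfigure BP_NPCBuilderAI, hand morph and tool visibility, while blackboard flags report injury and death.
; Events drive cutting animation, hook/hammer swaps between hands and table, rope slides and a slow-motion use interaction.
; SetupNPC caches named POIs, whose action objects link it to saw, table, rope stand and car.
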(event Custom|Cutting
  (Rendering|SetVisibility (Variables|Default|GetLogWood) true false)
  (Utilities|IsValid (Variables|Default|GetAnimator)
    (:Is%20Valid
      _)
    (:Is%20Not%20Valid
      (bind _asbpa_builder (Utilities|Casting|CastToBPA_Builder (Components|SkeletalMesh|GetAnimInstance (Variables|Character|GetMesh))))
      (Variables|Default|SetAnimator _asbpa_builder)))
  (Variables|/Game/FFBlueprints/NPC/Builder/BPA_Builder.BPA_Builder_C|SetChainSawBS (Variables|Default|GetAnimator) 0.0)
  (Variables|/Game/FFBlueprints/NPC/Builder/BPA_Builder.BPA_Builder_C|SetUseBabushkaCustom (Variables|Default|GetAnimator) 1.0)
  (Variables|/Game/FFBlueprints/NPC/Builder/BPA_Builder.BPA_Builder_C|SetIsCutting (Variables|Default|GetAnimator) true))

(event Custom|HandOn
  (bind _l_hook (Variables|Default|GetL_Hook))
  (bind _l_hammer (Variables|Default|GetL_Hammer))
  (Utilities|FlowControl|Sequence
    (:then_0
      (if (Rendering|IsVisible _l_hook)
        (Rendering|SetVisibility _l_hook false false)
        (Rendering|SetVisibility (Variables|Default|GetR_Hook) true false)))
    (:then_1
      (if (Rendering|IsVisible _l_hammer)
        (Rendering|SetVisibility _l_hammer false false)
        (Rendering|SetVisibility (Variables|Default|GetR_Hammer) true false)))))

(event Custom|RopeSlide
  (Variables|Default|SetPerformingSlide true)
  (bind _asbp_npcpoi (Utilities|Casting|CastToBP_NPCPOI (Variables|Default|GetRopeStand)))
  (bind _asbp_rope_stand (Utilities|Casting|CastToBP_RopeStand (Variables|/Game/FFBlueprints/NPC/BP_NPCPOI.BP_NPCPOI_C|GetActionObject _asbp_npcpoi)))
  (bind _asbp_projectile_harpoon (Utilities|Casting|CastToBP_ProjectileHarpoon (Variables|/Game/FFBlueprints/BP_RopeStand.BP_RopeStand_C|GetAttachedRope _asbp_rope_stand)))
  (Default|PerformSlide _asbp_projectile_harpoon (Variables|/Game/FFBlueprints/BP_RopeStand.BP_RopeStand_C|GetAttachedHandle _asbp_rope_stand) self))

(event Custom|TableOn
  (bind _l_hook (Variables|Default|GetL_Hook))
  (bind _l_hammer (Variables|Default|GetL_Hammer))
  (bind _table (Variables|Default|GetTable))
  (Utilities|FlowControl|Sequence
    (:then_0
      (if (Rendering|IsVisible _l_hook)
        (Rendering|SetVisibility _l_hook false false)
        (bind _asbp_npcpoi (Utilities|Casting|CastToBP_NPCPOI _table))
        (bind _asbp_builder_table (Utilities|Casting|CastToBP_BuilderTable (Variables|/Game/FFBlueprints/NPC/BP_NPCPOI.BP_NPCPOI_C|GetActionObject _asbp_npcpoi)))
        (Default|UpdateHook _asbp_builder_table true)))
    (:then_1
      (if (Rendering|IsVisible _l_hammer)
        (Rendering|SetVisibility _l_hammer false false)
        (bind _asbp_npcpoi_2 (Utilities|Casting|CastToBP_NPCPOI _table))
        (bind _asbp_builder_table_2 (Utilities|Casting|CastToBP_BuilderTable (Variables|/Game/FFBlueprints/NPC/BP_NPCPOI.BP_NPCPOI_C|GetActionObject _asbp_npcpoi_2)))
        (Default|UpdateHammer _asbp_builder_table_2 true)))))

(event Custom|TableOff
  (bind _asbp_npcpoi (Utilities|Casting|CastToBP_NPCPOI (Variables|Default|GetTable)))
  (bind _asbp_builder_table (Utilities|Casting|CastToBP_BuilderTable (Variables|/Game/FFBlueprints/NPC/BP_NPCPOI.BP_NPCPOI_C|GetActionObject _asbp_npcpoi)))
  (Utilities|FlowControl|Sequence
    (:then_0
      (Utilities|Casting|CastToHammer (Variables|/Game/FFBlueprints/BP_BuilderTable.BP_BuilderTable_C|GetCurrentItem _asbp_builder_table))
      (Default|UpdateHook _asbp_builder_table false)
      (Rendering|SetVisibility (Variables|Default|GetL_Hook) true false))
    (:then_1
      (Utilities|Casting|CastToHook (Variables|/Game/FFBlueprints/BP_BuilderTable.BP_BuilderTable_C|GetCurrentItem _asbp_builder_table))
      (Default|UpdateHammer _asbp_builder_table false)
      (Rendering|SetVisibility (Variables|Default|GetL_Hammer) true false))))

(event Custom|HandOff
  (bind _r_hook (Variables|Default|GetR_Hook))
  (bind _r_hammer (Variables|Default|GetR_Hammer))
  (Utilities|FlowControl|Sequence
    (:then_0
      (if (Rendering|IsVisible _r_hook)
        (Rendering|SetVisibility _r_hook false false)
        (Rendering|SetVisibility (Variables|Default|GetL_Hook) true false)))
    (:then_1
      (if (Rendering|IsVisible _r_hammer)
        (Rendering|SetVisibility _r_hammer false false)
        (Rendering|SetVisibility (Variables|Default|GetL_Hammer) true false)))))

(event Custom|SlideComplete
  (Variables|Default|SetPerformingSlide false))

(event Custom|ChangeRole
  (params (NewParam :type BuilderState%20Enum :default "NewEnumerator0"))
  (bind _self self)
  (bind _returnvalue (AI|GetAIController _self))
  (Utilities|IsValid _returnvalue
    (:Is%20Valid
      (bind _asbp_npcbuilder_ai (Utilities|Casting|CastToBP_NPCBuilderAI _returnvalue))
      (Default|SetupAI _asbp_npcbuilder_ai NewParam)
      (CallFunction|Initialize NewParam)
      (if (Utilities|Enum|Equal(Enum) NewParam "NewEnumerator3")
        (bind _asbp_npcpoi (Utilities|Casting|CastToBP_NPCPOI (Variables|Default|GetCar)))
        (bind _asbp_car (Utilities|Casting|CastToBP_car (Variables|/Game/FFBlueprints/NPC/BP_NPCPOI.BP_NPCPOI_C|GetActionObject _asbp_npcpoi)))
        (EventDispatchers|AssignCarFell _asbp_car (delegate Custom|CarFell_Event_0))))))

(event Custom|NewStateSet
  (params (NewState :type BuilderState%20Enum :default "NewEnumerator5"))
  (CallFunction|ChangeRole NewState)
  (Rendering|Components|TextRender|SetText (Variables|Default|GetTextRender) (Utilities|Text|ToText(String) (Utilities|String|EnumtoString (Default|GetActualStateBuilder (Variables|Default|GetBuilderState))))))

(event Custom|CarFell_Event_0
  (AI|Components|Blackboard|SetValueasBool (AI|GetBlackboard (Pawn|GetController)) (Variables|Default|GetIsDead) true)
  (CallFunction|MakeBloodMess))

(event EventBeginPlay
  (bind _self self)
  (bind _returnvalue (AI|GetAIController _self))
  (EventDispatchers|BindEventtoNewStateBuilder (Variables|Default|GetBuilderState) (delegate Custom|NewStateSet))
  (Utilities|FlowControl|Delay 0.2)
  (Utilities|IsValid _returnvalue
    (:Is%20Valid
      (bind _asbp_npcbuilder_ai (Utilities|Casting|CastToBP_NPCBuilderAI _returnvalue))
      (Default|SetupAI _asbp_npcbuilder_ai "NewEnumerator0")
      (CallFunction|Initialize "NewEnumerator0"))))

(event Collision|EventActorBeginOverlap
  (params (OtherActor :type Actor%20Object%20Reference))
  (|CallParentFunction OtherActor) ; This node is disabled and will not be called.\nDrag off pins to build functionality.
)

(event EventUseItem
  (bind _animator (Variables|Default|GetAnimator))
  (bind _asfirst_person_character (Utilities|Casting|CastToFirstPersonCharacter (Game|GetPlayerCharacter 0)))
  (if (Variables|/Game/FirstPersonBP/Blueprints/FirstPersonCharacter.FirstPersonCharacter_C|GetSlowTime _asfirst_person_character)
    (Default|BulletTime _asfirst_person_character)
    (bind _value (Timeline|UpdateHandTimeline Play)
      (:Update
        (Utilities|IsValid _animator
          (:Is%20Valid
            (Variables|/Game/FFBlueprints/NPC/Builder/BPA_Builder.BPA_Builder_C|SetChainSawBS _animator _value)))))))

(fn ConstructionScript
  (|CallParentFunction))

(fn NotifSawChanged
  (params (State :type Boolean))
  (bind _asbp_npcpoi (Utilities|Casting|CastToBP_NPCPOI (Variables|Default|GetWoodCutter)))
  (bind _asbp_saw (Utilities|Casting|CastToBP_Saw (Variables|/Game/FFBlueprints/NPC/BP_NPCPOI.BP_NPCPOI_C|GetActionObject _asbp_npcpoi)))
  (bind _asbpa_saw (Utilities|Casting|CastToBPA_Saw (Components|SkeletalMesh|GetAnimInstance (Variables|/Game/FFBlueprints/BP_Saw.BP_Saw_C|GetMesh _asbp_saw))))
  (Variables|/Game/FFBlueprints/BPA_Saw.BPA_Saw_C|SetIsOn _asbpa_saw State))

(fn CutOffHand
  (bind _self self)
  (bind _mesh (Variables|Character|GetMesh))
  (bind _returnvalue (Transformation|GetSocketTransform _mesh "RH_socket" "RTS_World"))
  (bind _returnvalue_2 (AI|GetAIController _self))
  (Components|SkeletalMesh|SetMorphTarget _mesh "cut_hand" 1.0 true)
  (bind _returnvalue_3 (Effects|SpawnEmitterAttached "/Game/assets/particles/PS_redpaint.PS_redpaint" _mesh "RH_socket" (.location _returnvalue) (.rotation _returnvalue) "1.000000,1.000000,1.000000" "KeepWorldPosition"))
  (Variables|Default|SetBleedingPS _returnvalue_3)
  (bind _asbp_npcpoi (Utilities|Casting|CastToBP_NPCPOI (Variables|Default|GetWoodCutter)))
  (bind _asbp_saw (Utilities|Casting|CastToBP_Saw (Variables|/Game/FFBlueprints/NPC/BP_NPCPOI.BP_NPCPOI_C|GetActionObject _asbp_npcpoi)))
  (Game|SpawnActorfromClass "/Game/FFBlueprints/BP_Hand.BP_Hand_C" (Math|Transform|MakeTransform (Transformation|GetWorldLocation (Variables|/Game/FFBlueprints/BP_Saw.BP_Saw_C|GetSpawningPoint _asbp_saw)) "0, 0, 0" "1,1,1") "AdjustIfPossibleButAlwaysSpawn" 0 0)
  (Utilities|IsValid _returnvalue_2
    (:Is%20Valid
      (AI|Components|Blackboard|SetValueasBool (AI|GetBlackboard _returnvalue_2) (Variables|Default|GetHandCut) true)
      (Variables|/Script/Engine.CharacterMovementComponent|SetMaxWalkSpeed (Variables|Character|GetCharacterMovement) (Variables|Default|GetRunningSpeed))
      (Rendering|SetVisibility (Variables|Default|GetLogWood) false false))))

(fn HookStolen
  (Default|NextStateBuilder (Variables|Default|GetBuilderState) "NewEnumerator3"))

(fn Initialize
  (params (state :type BuilderState%20Enum :default "NewEnumerator0"))
  (bind _mesh (Variables|Character|GetMesh))
  (Utilities|Casting|CastToBP_NPCBuilderAI (AI|GetAIController self))
  (switch Utilities|FlowControl|Switch|SwitchonBuilderState state
    (:NewEnumerator1
      (Components|SkeletalMesh|SetMorphTarget _mesh "cut_hand" 0.0 true)
      (Rendering|SetVisibility (Variables|Default|GetR_Hook) false false)
      (Rendering|SetVisibility (Variables|Default|GetR_Hammer) false false)
      (Rendering|SetVisibility (Variables|Default|GetL_Hook) false false)
      (Rendering|SetVisibility (Variables|Default|GetL_Hammer) false false))
    (:NewEnumerator2
      (Components|SkeletalMesh|SetMorphTarget _mesh "cut_hand" 1.0 true)
      (Rendering|SetVisibility (Variables|Default|GetR_Hook) true false)
      (Rendering|SetVisibility (Variables|Default|GetR_Hammer) false false)
      (Rendering|SetVisibility (Variables|Default|GetL_Hook) false false)
      (Rendering|SetVisibility (Variables|Default|GetL_Hammer) false false))))

(fn MakeBloodMess
  (bind _capsulecomponent (Variables|Default|GetCapsuleComponent))
  (bind _returnvalue (Transformation|GetWorldLocation _capsulecomponent))
  (for _index (range 0 20)
    (bind _returnvalue_2 (Game|SpawnActorfromClass "/Game/FFBlueprints/NPC/Dog/ShitProjectile.ShitProjectile_C" (Math|Transform|MakeTransform (Math|Vector|MakeVector (.x _returnvalue) (.y _returnvalue) (- (.z _returnvalue) 7e+01)) (Math|Rotator|MakeRotfromZ (Math|Random|RandomUnitVectorinConeinDegrees "0, 0,1.000000" 8e+01))) "AlwaysSpawn" 0 0))
    (Physics|SetPhysicsLinearVelocity (Variables|/Game/FFBlueprints/NPC/Dog/ShitProjectile.ShitProjectile_C|GetCollision _returnvalue_2) (* (Math|Vector|GetUpVector (Variables|/Game/FFBlueprints/NPC/Dog/ShitProjectile.ShitProjectile_C|GetCollision _returnvalue_2)) -9e+02) false "None")))

(fn SetupHook
  (Utilities|CheckAnimator
    (:Output
      (Variables|/Game/FFBlueprints/NPC/Builder/BPA_Builder.BPA_Builder_C|SetSetupHook (Variables|Default|GetAnimator) true)
      (Default|NextStateBuilder (Variables|Default|GetBuilderState) "NewEnumerator3"))))

(fn SetupNPC
  (bind _asfast_food_game_state (Utilities|Casting|CastToFastFoodGameState (Game|GetGameState)))
  (bind _point (Default|GetSpecificPoi (Variables|/Game/FFBlueprints/GameMode/FastFoodGameState.FastFoodGameState_C|GetNPCPOIManager _asfast_food_game_state) "WoodCutter"))
  (Variables|Default|SetWoodCutter _point)
  (bind _point_2 (Default|GetSpecificPoi (Variables|/Game/FFBlueprints/GameMode/FastFoodGameState.FastFoodGameState_C|GetNPCPOIManager _asfast_food_game_state) "House"))
  (Variables|Default|SetHouse _point_2)
  (bind _point_3 (Default|GetSpecificPoi (Variables|/Game/FFBlueprints/GameMode/FastFoodGameState.FastFoodGameState_C|GetNPCPOIManager _asfast_food_game_state) "FirstAid"))
  (Variables|Default|SetFirstAid _point_3)
  (bind _point_4 (Default|GetSpecificPoi (Variables|/Game/FFBlueprints/GameMode/FastFoodGameState.FastFoodGameState_C|GetNPCPOIManager _asfast_food_game_state) "PolystyrenePlace"))
  (Variables|Default|SetPolystyrenePlace _point_4)
  (bind _point_5 (Default|GetSpecificPoi (Variables|/Game/FFBlueprints/GameMode/FastFoodGameState.FastFoodGameState_C|GetNPCPOIManager _asfast_food_game_state) "PolystyreneHouse"))
  (Variables|Default|SetPolystyreneHouse _point_5)
  (bind _point_6 (Default|GetSpecificPoi (Variables|/Game/FFBlueprints/GameMode/FastFoodGameState.FastFoodGameState_C|GetNPCPOIManager _asfast_food_game_state) "WoodStorage"))
  (Variables|Default|SetStorage _point_6)
  (bind _point_7 (Default|GetSpecificPoi (Variables|/Game/FFBlueprints/GameMode/FastFoodGameState.FastFoodGameState_C|GetNPCPOIManager _asfast_food_game_state) "RopeStand"))
  (Variables|Default|SetRopeStand _point_7)
  (bind _point_8 (Default|GetSpecificPoi (Variables|/Game/FFBlueprints/GameMode/FastFoodGameState.FastFoodGameState_C|GetNPCPOIManager _asfast_food_game_state) "Polystyrene"))
  (Variables|Default|SetPolystyrene _point_8)
  (bind _point_9 (Default|GetSpecificPoi (Variables|/Game/FFBlueprints/GameMode/FastFoodGameState.FastFoodGameState_C|GetNPCPOIManager _asfast_food_game_state) "Table"))
  (Variables|Default|SetTable _point_9)
  (bind _point_10 (Default|GetSpecificPoi (Variables|/Game/FFBlueprints/GameMode/FastFoodGameState.FastFoodGameState_C|GetNPCPOIManager _asfast_food_game_state) "Car"))
  (Variables|Default|SetCar _point_10))

(fn CombinewithItem
  (params (ItemToCombine :type Actor%20Object%20Reference))
  (return false false false false))

(fn IsReadytoUse
  (return (Variables|Default|GetPerformCutting)))