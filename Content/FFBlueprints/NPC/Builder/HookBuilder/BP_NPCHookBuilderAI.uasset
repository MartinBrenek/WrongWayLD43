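; AI controller for the hook builder NPC that prepares its blackboard when play begins.
; It casts the controlled pawn to BP_Builder, initializes BB_HookBuilder, copies the builder's polystyrene, polystyrene house and table references into keys, and flags InQuest as true.
; It then passes the blackboard to SetOwnerPawn before calling the parent BeginPlay, both of which are skipped if the cast fails.
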(event EventBeginPlay
  (bind _asbp_builder (Utilities|Casting|CastToBP_Builder (Pawn|GetControlledPawn)))
  (bind _blackboardcomponent (Class|AIController|UseBlackboard "/Game/FFBlueprints/NPC/Builder/HookBuilder/BB_HookBuilder.BB_HookBuilder"))
  (AI|Components|Blackboard|SetValueasObject _blackboardcomponent (Variables|Default|GetPolystyrene) (Variables|/Game/FFBlueprints/NPC/Builder/BP_Builder.BP_Builder_C|GetPolystyrene _asbp_builder))
  (AI|Components|Blackboard|SetValueasObject _blackboardcomponent (Variables|Default|GetHouse) (Variables|/Game/FFBlueprints/NPC/Builder/BP_Builder.BP_Builder_C|GetPolystyreneHouse _asbp_builder))
  (AI|Components|Blackboard|SetValueasObject _blackboardcomponent (Variables|Default|GetTable) (Variables|/Game/FFBlueprints/NPC/Builder/BP_Builder.BP_Builder_C|GetTable _asbp_builder))
  (AI|Components|Blackboard|SetValueasBool _blackboardcomponent (Variables|Default|GetInQuest) true)
  (CallFunction|SetOwnerPawn _blackboardcomponent)
  (|CallParentFunction))

(event EventTick
  (params (DeltaSeconds :type Float%20%28single-precision%29)))

(fn ConstructionScript
  (|CallParentFunction))