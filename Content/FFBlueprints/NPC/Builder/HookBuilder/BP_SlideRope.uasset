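; Behavior tree task that starts the rope slide for a Builder NPC.
; On execute it sets the IsSlidingRope blackboard flag, casts the blackboard's Owner object to BP_Builder and calls its RopeSlide.
; The nodes that would clear the flag and finish the task are disconnected, so the task never calls FinishExecute itself.
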(event EventReceiveExecute
  (params (OwnerActor :type Actor%20Object%20Reference))
  (bind _returnvalue (AI|GetBlackboard OwnerActor))
  (AI|Components|Blackboard|SetValueasBool _returnvalue (Variables|Default|GetIsSlidingRope) true)
  (bind _asbp_builder (Utilities|Casting|CastToBP_Builder (AI|Components|Blackboard|GetValueasObject _returnvalue (Variables|Default|GetOwner))))
  (Default|RopeSlide _asbp_builder))

(event EventTick
  (params (OwnerActor :type Actor%20Object%20Reference) (DeltaSeconds :type Float%20%28single-precision%29)))