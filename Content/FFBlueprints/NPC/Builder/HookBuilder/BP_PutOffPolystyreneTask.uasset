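; BP_PutOffPolystyreneTask is a behavior tree task in which a builder NPC puts off the polystyrene board it holds.
; On execute it sets the IsPicking and AnimationRunning blackboard flags to true.
; Tick polls AnimationRunning until it is cleared elsewhere, then resets IsPicking, hides the PolystyreneDesk component on the Owner BP_Builder and finishes successfully.
; If that Owner cast fails, the task never calls FinishExecute.
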(event EventReceiveExecute
  (params (OwnerActor :type Actor%20Object%20Reference))
  (bind _returnvalue (AI|GetBlackboard OwnerActor))
  (AI|Components|Blackboard|SetValueasBool _returnvalue (Variables|Default|GetIsPicking) true)
  (AI|Components|Blackboard|SetValueasBool _returnvalue (Variables|Default|GetAnimationRunning) true))

(event EventTick
  (params (OwnerActor :type Actor%20Object%20Reference) (DeltaSeconds :type Float%20%28single-precision%29))
  (bind _returnvalue (AI|GetBlackboard OwnerActor))
  (if (not (ScalableFloat|GetValueasBool _returnvalue (Variables|Default|GetAnimationRunning)))
    (AI|Components|Blackboard|SetValueasBool _returnvalue (Variables|Default|GetIsPicking) false)
    (bind _asbp_builder (Utilities|Casting|CastToBP_Builder (AI|Components|Blackboard|GetValueasObject _returnvalue (Variables|Default|GetOwner))))
    (Rendering|SetVisibility (Variables|/Game/FFBlueprints/NPC/Builder/BP_Builder.BP_Builder_C|GetPolystyreneDesk _asbp_builder) false false)
    (AI|BehaviorTree|FinishExecute true)))