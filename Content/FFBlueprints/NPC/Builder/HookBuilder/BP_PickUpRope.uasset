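; Behavior tree task that attaches a builder NPC to a rope handle.
; On execute it sets the rope and animation blackboard flags and gives the builder slight negative gravity.
; Once the animation flag clears, Tick finds the handle via the rope stand POI, enables physics, constrains the capsule to its dock sphere, restores gravity and finishes.
; An alternative physics-handle grab is left unconnected.
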(event EventReceiveExecute
  (params (OwnerActor :type Actor%20Object%20Reference))
  (bind _returnvalue (AI|GetBlackboard OwnerActor))
  (AI|Components|Blackboard|SetValueasBool _returnvalue (Variables|Default|GetIsOnRope) true)
  (AI|Components|Blackboard|SetValueasBool _returnvalue (Variables|Default|GetAnimationRunning) true)
  (bind _asbp_builder (Utilities|Casting|CastToBP_Builder (AI|Components|Blackboard|GetValueasObject _returnvalue (Variables|Default|GetOwner))))
  (Variables|/Script/Engine.CharacterMovementComponent|SetGravityScale (Variables|/Script/Engine.Character|GetCharacterMovement _asbp_builder) -0.05))

(event EventTick
  (params (OwnerActor :type Actor%20Object%20Reference) (DeltaSeconds :type Float%20%28single-precision%29))
  (bind _returnvalue (AI|GetBlackboard OwnerActor))
  (if (not (ScalableFloat|GetValueasBool _returnvalue (Variables|Default|GetAnimationRunning)))
    (bind _asbp_builder (Utilities|Casting|CastToBP_Builder (AI|Components|Blackboard|GetValueasObject _returnvalue (Variables|Default|GetOwner))))
    (bind _asbp_npcpoi (Utilities|Casting|CastToBP_NPCPOI (Variables|/Game/FFBlueprints/NPC/Builder/BP_Builder.BP_Builder_C|GetRopeStand _asbp_builder)))
    (bind _asbp_rope_stand (Utilities|Casting|CastToBP_RopeStand (Variables|/Game/FFBlueprints/NPC/BP_NPCPOI.BP_NPCPOI_C|GetActionObject _asbp_npcpoi)))
    (bind _asbp_rope_handle (Utilities|Casting|CastToBP_RopeHandle (Variables|/Game/FFBlueprints/BP_RopeStand.BP_RopeStand_C|GetAttachedHandle _asbp_rope_stand)))
    (Collision|SetCollisionResponsetoChannel (Variables|/Script/Engine.Character|GetCapsuleComponent _asbp_builder) "ECC_Pawn" "ECR_Ignore")
    (Physics|SetSimulatePhysics (Variables|/Script/Engine.Character|GetCapsuleComponent _asbp_builder) true)
    (Collision|SetCollisionResponsetoChannel (Variables|/Script/Engine.Character|GetMesh _asbp_builder) "ECC_Pawn" "ECR_Ignore")
    (Physics|SetSimulatePhysics (Variables|/Script/Engine.Character|GetMesh _asbp_builder) true)
    (Class|PhysicsConstraintComponent|SetConstrainedComponents (Variables|/Game/FFBlueprints/BP_RopeHandle.BP_RopeHandle_C|GetPhysicsConstraint _asbp_rope_handle) (Variables|/Game/FFBlueprints/BP_RopeHandle.BP_RopeHandle_C|GetDockSphere _asbp_rope_handle) "None" (Variables|/Script/Engine.Character|GetCapsuleComponent _asbp_builder) "None")
    (Variables|/Script/Engine.CharacterMovementComponent|SetGravityScale (Variables|/Script/Engine.Character|GetCharacterMovement _asbp_builder) 1.0)
    (AI|BehaviorTree|FinishExecute true)))