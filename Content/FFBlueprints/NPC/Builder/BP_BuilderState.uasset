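; BP_BuilderState is the Builder NPC's state machine, specializing a parent state class with Builder-specific state and transition enums.
; Typed wrappers get, set and advance the state through the parent, and SetState also raises CallNewStateBuilder with the converted state.
; It supplies the transition count, a name-to-state map and per-row arrays built from a DataTable, indexed by transition and holding target states as integers.
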(event EventBeginPlay
  (|CallParentFunction) ; This node is disabled and will not be called.\nDrag off pins to build functionality.
)

(event EventTick
  (params (DeltaSeconds :type Float%20%28single-precision%29)))

(event EventSetState
  (params (State :type Byte :default 0))
  (|CallParentFunction State)
  (Default|CallNewStateBuilder (Utilities|Enum|ByteToEnumBuilderState State)))

(fn NextStateBuilder
  (params (Transition :type TransitionStateBuilder%20Enum :default "NewEnumerator0"))
  (bind (_nextstatefound _newstate) (CallFunction|NextState Transition))
  (return _nextstatefound (Utilities|Enum|ByteToEnumBuilderState _newstate)))

(fn GetActualStateBuilder
  (bind _state (CallFunction|GetActualState))
  (return (Utilities|Enum|ByteToEnumBuilderState _state)))

(fn SetStateBuilder
  (params (State :type BuilderState%20Enum :default "NewEnumerator5"))
  (CallFunction|SetState State))

(fn GetNumOfTransition
  (|ForEachTransitionStateBuilder
    (:LoopBody
      (Math|Integer|IncrementInt (LocalVariables|GetNumTransition)))
    (:then
      (return (LocalVariables|GetNumTransition)))))

(fn GetStringtoState
  (bind _enumvalue (|ForEachBuilderState)
    (:LoopBody
      (Utilities|Map|Add (LocalVariables|GetStatefromString) (Utilities|String|EnumtoString _enumvalue) (Math|Conversions|ToInteger(Byte) _enumvalue)))
    (:then
      (return (LocalVariables|GetStatefromString)))))

(fn GetRowArrayfromTable
  (params (Row :type Name :default "None") (Table :type Data%20Table%20Object%20Reference) (NumTransition :type Integer))
  (bind _returnvalue (Utilities|GetDataTableRow Table Row)
    (:then
      (Utilities|FlowControl|Sequence
        (:then_0
          (Utilities|Array|SetArrayElem (LocalVariables|GetTempArray) (- NumTransition 1) 0 true))
        (:then_1
          (bind _output_get (LocalVariables|SetRowStruct _returnvalue))
          (for _array_element (Utilities|Struct|BreakTableTransitionStructBuilder _output_get)
            (Utilities|Array|SetArrayElem (LocalVariables|GetTempArray) (Math|Conversions|ToInteger(Byte) (.Transition (Utilities|Struct|BreakTransPairBuilder _array_element))) (Math|Conversions|ToInteger(Byte) (.State (Utilities|Struct|BreakTransPairBuilder _array_element)))))
          (return (LocalVariables|GetTempArray)))))))