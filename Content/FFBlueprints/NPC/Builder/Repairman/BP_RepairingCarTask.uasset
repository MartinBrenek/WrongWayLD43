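; Behavior tree task for the repairman builder NPC's car-repairing activity.
; On execute it sets the AnimationRunning and IsLaying blackboard flags, then casts the Owner key to BP_Builder without using the result.
; The task stays active until Tick sees IsDead on the blackboard, when it clears InQuest and finishes successfully.
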(event EventReceiveExecute
  (params (OwnerActor :type Actor%20Object%20Reference))
  (bind _returnvalue (AI|GetBlackboard OwnerActor))
  (AI|Components|Blackboard|SetValueasBool _returnvalue (Variables|Default|GetAnimationRunning) true)
  (AI|Components|Blackboard|SetValueasBool _returnvalue (Variables|Default|GetIsLaying) true)
  (Utilities|Casting|CastToBP_Builder (AI|Components|Blackboard|GetValueasObject _returnvalue (Variables|Default|GetOwner))))

(event EventTick
  (params (OwnerActor :type Actor%20Object%20Reference) (DeltaSeconds :type Float%20%28single-precision%29))
  (bind _returnvalue (AI|GetBlackboard OwnerActor))
  (if (ScalableFloat|GetValueasBool _returnvalue (Variables|Default|GetIsDead))
    (AI|Components|Blackboard|SetValueasBool _returnvalue (Variables|Default|GetInQuest) false)
    (AI|BehaviorTree|FinishExecute true)))