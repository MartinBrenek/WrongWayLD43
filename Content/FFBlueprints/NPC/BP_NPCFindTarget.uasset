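; Behavior tree task that picks a point of interest for an NPC by name and stores it in the blackboard.
; It queries the game state's NPC POI manager with FindObjectName and writes the point to the ActualObject key.
; A loop re-queries while the result matches the current target and several points exist, but the write uses the first query's point, not the re-rolled one.
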(event EventReceiveExecute
  (params (OwnerActor :type Actor%20Object%20Reference))
  (bind _returnvalue (AI|GetBlackboard OwnerActor))
  (bind _asfast_food_game_state (Utilities|Casting|CastToFastFoodGameState (Game|GetGameState)))
  (bind (_point _countofpoints) (Default|GetSpecificPoi (Variables|/Game/FFBlueprints/GameMode/FastFoodGameState.FastFoodGameState_C|GetNPCPOIManager _asfast_food_game_state) (Variables|Default|GetFindObjectName)))
  (Variables|Default|Settemp _point)
  (while (and (== (AI|Components|Blackboard|GetValueasObject _returnvalue (Variables|Default|GetActualObject)) (Variables|Default|Gettemp)) (> _countofpoints 1))
    (bind _point_2 (Default|GetSpecificPoi (Variables|/Game/FFBlueprints/GameMode/FastFoodGameState.FastFoodGameState_C|GetNPCPOIManager _asfast_food_game_state) (Variables|Default|GetFindObjectName)))
    (Variables|Default|Settemp _point_2))
  (AI|Components|Blackboard|SetValueasObject _returnvalue (Variables|Default|GetActualObject) _point)
  (AI|BehaviorTree|FinishExecute true))