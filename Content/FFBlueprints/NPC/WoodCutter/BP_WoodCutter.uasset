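; BP_WoodCutter is a woodcutter NPC Blueprint that can be switched into a wood-cutting animation.
; Its Cutting event hides the LogWood component, then sets the IsCutting flag and UseBabushkaCustom value on its BPA_WoodCutter animation instance.
; The animation instance reference is fetched from the mesh and cached on demand when not yet valid.
; BeginPlay, Tick and overlap events are unused.
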(event Custom|Cutting
  (Rendering|SetVisibility (Variables|Default|GetLogWood) false false)
  (Utilities|IsValid (Variables|Default|GetAnimator)
    (:Is%20Valid
      _)
    (:Is%20Not%20Valid
      (bind _asbpa_wood_cutter (Utilities|Casting|CastToBPA_WoodCutter (Components|SkeletalMesh|GetAnimInstance (Variables|Character|GetMesh))))
      (Variables|Default|SetAnimator _asbpa_wood_cutter)))
  (Variables|/Game/FFBlueprints/NPC/WoodCutter/BPA_WoodCutter.BPA_WoodCutter_C|SetUseBabushkaCustom (Variables|Default|GetAnimator) 1.0)
  (Variables|/Game/FFBlueprints/NPC/WoodCutter/BPA_WoodCutter.BPA_WoodCutter_C|SetIsCutting (Variables|Default|GetAnimator) true))

(event EventBeginPlay
  (|CallParentFunction) ; This node is disabled and will not be called.\nDrag off pins to build functionality.
)

(event Collision|EventActorBeginOverlap
  (params (OtherActor :type Actor%20Object%20Reference))
  (|CallParentFunction OtherActor) ; This node is disabled and will not be called.\nDrag off pins to build functionality.
)

(event EventTick
  (params (DeltaSeconds :type Float%20%28single-precision%29))
  (|CallParentFunction DeltaSeconds) ; This node is disabled and will not be called.\nDrag off pins to build functionality.
)

(fn ConstructionScript
  (|CallParentFunction))