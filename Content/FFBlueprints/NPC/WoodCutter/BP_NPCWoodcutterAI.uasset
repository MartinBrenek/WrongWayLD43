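; AI controller for the woodcutter NPC that initializes its blackboard when play begins.
; It casts the controlled pawn to BP_WoodCutter, activates BB_Woodcutter, and copies in the pawn itself plus its WoodCutter, Storage and House references.
; It also sets the InQuest flag to true, then calls the parent BeginPlay, which is skipped if the cast fails.
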(event EventBeginPlay
  (bind _asbp_wood_cutter (Utilities|Casting|CastToBP_WoodCutter (Pawn|GetControlledPawn)))
  (bind _blackboardcomponent (Class|AIController|UseBlackboard "/Game/FFBlueprints/NPC/WoodCutter/BB_Woodcutter.BB_Woodcutter"))
  (AI|Components|Blackboard|SetValueasObject _blackboardcomponent (Variables|Default|GetOwnerKey) _asbp_wood_cutter)
  (AI|Components|Blackboard|SetValueasObject _blackboardcomponent (Variables|Default|GetWoodCutter) (Variables|/Game/FFBlueprints/NPC/WoodCutter/BP_WoodCutter.BP_WoodCutter_C|GetWoodCutter _asbp_wood_cutter))
  (AI|Components|Blackboard|SetValueasObject _blackboardcomponent (Variables|Default|GetStorage) (Variables|/Game/FFBlueprints/NPC/WoodCutter/BP_WoodCutter.BP_WoodCutter_C|GetStorage _asbp_wood_cutter))
  (AI|Components|Blackboard|SetValueasObject _blackboardcomponent (Variables|Default|GetHouse) (Variables|/Game/FFBlueprints/NPC/WoodCutter/BP_WoodCutter.BP_WoodCutter_C|GetHouse _asbp_wood_cutter))
  (AI|Components|Blackboard|SetValueasBool _blackboardcomponent (Variables|Default|GetInQuest) true)
  (|CallParentFunction))

(event EventTick
  (params (DeltaSeconds :type Float%20%28single-precision%29)))

(fn ConstructionScript
  (|CallParentFunction))