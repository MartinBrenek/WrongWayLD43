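; BP_CutWoodTask is a behavior tree task that has a woodcutter NPC perform its wood-cutting action.
; On execute it sets the AnimationRunning blackboard flag, gets the BP_WoodCutter pawn from its AI controller and calls Cutting on it.
; Tick polls that flag and, once it is false, clears the animator's IsCutting state and finishes the task successfully.
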(event EventReceiveExecute
  (params (OwnerActor :type Actor%20Object%20Reference))
  (AI|Components|Blackboard|SetValueasBool (AI|GetBlackboard OwnerActor) (Variables|Default|GetAnimationRunning) true)
  (bind _asbp_npcbase_aicontroller (Utilities|Casting|CastToBP_NPCBaseAIController OwnerActor))
  (bind _asbp_wood_cutter (Utilities|Casting|CastToBP_WoodCutter (Pawn|GetControlledPawn _asbp_npcbase_aicontroller)))
  (bind _output_get (Variables|Default|SetWoodCutter _asbp_wood_cutter))
  (Default|Cutting _asbp_wood_cutter))

(event EventTick
  (params (OwnerActor :type Actor%20Object%20Reference) (DeltaSeconds :type Float%20%28single-precision%29))
  (if (not (ScalableFloat|GetValueasBool (AI|GetBlackboard OwnerActor) (Variables|Default|GetAnimationRunning)))
    (Variables|/Game/FFBlueprints/NPC/WoodCutter/BPA_WoodCutter.BPA_WoodCutter_C|SetIsCutting (Variables|/Game/FFBlueprints/NPC/WoodCutter/BP_WoodCutter.BP_WoodCutter_C|GetAnimator (Variables|Default|GetWoodCutter)) false)
    (AI|BehaviorTree|FinishExecute true)))