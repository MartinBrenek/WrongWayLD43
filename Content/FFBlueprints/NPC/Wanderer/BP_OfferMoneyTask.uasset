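; Behavior tree task that has a Wanderer NPC make a money offer in response to a BaldKing character.
; On execute it sets the offering and animation-running blackboard flags, calls StopOffering on the BaldKing and MakeOffer on the owning Wanderer, both read from blackboard objects.
; Tick polls the animation-running flag and, once it is false, clears the offering flag and finishes successfully.
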(event EventReceiveExecute
  (params (OwnerActor :type Actor%20Object%20Reference))
  (bind _returnvalue (AI|GetBlackboard OwnerActor))
  (AI|Components|Blackboard|SetValueasBool _returnvalue (Variables|Default|GetIsOffering) true)
  (AI|Components|Blackboard|SetValueasBool _returnvalue (Variables|Default|GetAnimationRunning) true)
  (bind _asbp_bald_king (Utilities|Casting|CastToBP_BaldKing (AI|Components|Blackboard|GetValueasObject _returnvalue (Variables|Default|GetWhore))))
  (Default|StopOffering _asbp_bald_king)
  (bind _asbp_wanderer (Utilities|Casting|CastToBP_Wanderer (AI|Components|Blackboard|GetValueasObject _returnvalue (Variables|Default|GetOwner))))
  (Default|MakeOffer _asbp_wanderer))

(event EventTick
  (params (OwnerActor :type Actor%20Object%20Reference) (DeltaSeconds :type Float%20%28single-precision%29))
  (bind _returnvalue (AI|GetBlackboard OwnerActor))
  (if (not (ScalableFloat|GetValueasBool _returnvalue (Variables|Default|GetAnimationRunning)))
    (AI|Components|Blackboard|SetValueasBool _returnvalue (Variables|Default|GetIsOffering) false)
    (AI|BehaviorTree|FinishExecute true)))