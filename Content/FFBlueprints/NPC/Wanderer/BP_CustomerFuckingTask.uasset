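; Behavior tree task that plays out a timed sex act for a Wanderer NPC, named as a customer task.
; It gets the Wanderer from the blackboard's Owner key, disables its capsule collision, calls MakeFuck and sets IsFucking.
; After a fixed delay it clears IsFucking and CanFuck, restores collision, calls EndFuck and finishes successfully.
; A failed cast stops execution without finishing the task.
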(event EventReceiveExecute
  (params (OwnerActor :type Actor%20Object%20Reference))
  (bind _returnvalue (AI|GetBlackboard OwnerActor))
  (bind _asbp_wanderer (Utilities|Casting|CastToBP_Wanderer (AI|Components|Blackboard|GetValueasObject _returnvalue (Variables|Default|GetOwner))))
  (Collision|SetCollisionEnabled (Variables|/Script/Engine.Character|GetCapsuleComponent _asbp_wanderer) "NoCollision")
  (Default|MakeFuck _asbp_wanderer)
  (AI|Components|Blackboard|SetValueasBool _returnvalue (Variables|Default|GetIsFucking) true)
  (Utilities|FlowControl|Delay 5.0)
  (AI|Components|Blackboard|SetValueasBool _returnvalue (Variables|Default|GetIsFucking) false)
  (AI|Components|Blackboard|SetValueasBool _returnvalue (Variables|Default|GetCanFuck) false)
  (Collision|SetCollisionEnabled (Variables|/Script/Engine.Character|GetCapsuleComponent _asbp_wanderer) "QueryAndPhysics")
  (Default|EndFuck _asbp_wanderer)
  (AI|BehaviorTree|FinishExecute true))