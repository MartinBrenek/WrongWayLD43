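; Wanderer NPC Blueprint that acts as a client in an adult transaction quest with a prostitute NPC.
; Events for the offer, act, end and theft toggle a cached animator's base pose, money visibility and Blackboard target/quest state.
; It can spawn a condom on the hand socket and bind its pickup event.
; Pickup during the player's SlowTime releases the item, clears quest flags and notifies the linked BP_BaldKing of the theft.
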(event Custom|MakeFuck
  (Utilities|CheckAnimator
    (:out
      (Variables|/Game/FFBlueprints/NPC/Wanderer/BP_WandererAnimator.BP_WandererAnimator_C|SetUseWandererBase (Variables|Default|GetAnimator_0) 1.0))))

(event Custom|EndFuck
  (Utilities|CheckAnimator
    (:out
      (CallFunction|SetupWhoreTarget)
      (Variables|/Game/FFBlueprints/NPC/Wanderer/BP_WandererAnimator.BP_WandererAnimator_C|SetUseWandererBase (Variables|Default|GetAnimator_0) 0.0))))

(event Custom|MakeOffer
  (Utilities|CheckAnimator
    (:out
      (Variables|/Game/FFBlueprints/NPC/Wanderer/BP_WandererAnimator.BP_WandererAnimator_C|SetUseWandererBase (Variables|Default|GetAnimator_0) 1.0)
      (CallFunction|ShowMoney true))))

(event Custom|CondomStolen
  (Utilities|CheckAnimator
    (:out
      (CallFunction|SetupWhoreTarget)
      (Variables|/Game/FFBlueprints/NPC/Wanderer/BP_WandererAnimator.BP_WandererAnimator_C|SetUseWandererBase (Variables|Default|GetAnimator_0) 0.0))))

(event Custom|CondomPickUp
  (bind _returnvalue (AI|GetBlackboard 0))
  (bind _asfirst_person_character (Utilities|Casting|CastToFirstPersonCharacter (Game|Player|GetPlayerPawn 0)))
  (if (Variables|/Game/FirstPersonBP/Blueprints/FirstPersonCharacter.FirstPersonCharacter_C|GetSlowTime _asfirst_person_character)
    (AI|Components|Blackboard|SetValueasBool _returnvalue (Variables|Default|GetInQuestKey) false)
    (Utilities|IsValid (Variables|Default|GetActiveItem)
      (:Is%20Valid
        (bind _asbp_condom (Utilities|Casting|CastToBP_Condom (Variables|Default|GetActiveItem)))
        (Physics|SetSimulatePhysics (Variables|/Game/FFBlueprints/PickableItem.PickableItem_C|GetCube _asbp_condom) true)
        (Variables|Default|SetActiveItem 0)
        (bind _asbp_bald_king (Utilities|Casting|CastToBP_BaldKing (AI|Components|Blackboard|GetValueasObject _returnvalue (Variables|Default|GetWhore))))
        (AI|Components|Blackboard|SetValueasBool (AI|GetBlackboard _asbp_bald_king) (Variables|Default|GetInQuestKey) false)
        (Default|CondomStolen _asbp_bald_king)))))

(event EventBeginPlay
  (|CallParentFunction))

(event Collision|EventActorBeginOverlap
  (params (OtherActor :type Actor%20Object%20Reference))
  (|CallParentFunction OtherActor) ; This node is disabled and will not be called.\nDrag off pins to build functionality.
)

(event EventTick
  (params (DeltaSeconds :type Float%20%28single-precision%29))
  (|CallParentFunction DeltaSeconds) ; This node is disabled and will not be called.\nDrag off pins to build functionality.
)

(fn ConstructionScript
  (|CallParentFunction))

(fn SetupWhoreTarget
  (params (Whore :type BP%20Bald%20King%20Object%20Reference))
  (bind _returnvalue (AI|GetBlackboard 0))
  (AI|Components|Blackboard|SetValueasObject _returnvalue (LocalVariables|GetWhoreKey) Whore)
  (AI|Components|Blackboard|SetValueasBool _returnvalue (LocalVariables|GetInQuest) (not (== Whore 0))))

(fn ShowMoney
  (params (Show :type Boolean))
  (Rendering|SetVisibility (Variables|Default|GetMoney) Show false))

(fn ShowCondom
  (params (Show :type Boolean))
  (if Show
    (bind _returnvalue (Game|SpawnActorfromClass "/Game/FFBlueprints/FastFoodOutDoor/BP_Condom.BP_Condom_C" (Transformation|GetSocketTransform (Variables|Character|GetMesh) "RH_socket" "RTS_World") "AdjustIfPossibleButAlwaysSpawn" 0 true 0))
    (Physics|SetSimulatePhysics (Variables|/Game/FFBlueprints/PickableItem.PickableItem_C|GetCube _returnvalue) false)
    (Transformation|AttachComponentToComponent _returnvalue (Variables|Default|GetCondom) "" "SnapToTarget" "SnapToTarget" "KeepWorld" false)
    (EventDispatchers|BindEventtoPickUpEvent _returnvalue (EventDispatchers|CreateEvent :!event Custom|CondomPickUp))
    (Variables|Default|SetActiveItem _returnvalue)
    (else
      (Utilities|IsValid (Variables|Default|GetActiveItem)
        (:Is%20Valid
          (Actor|DestroyActor (Variables|Default|GetActiveItem)))))))