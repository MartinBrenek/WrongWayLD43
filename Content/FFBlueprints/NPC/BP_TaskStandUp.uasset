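; Behavior Tree task that makes an NPC stand up from sitting.
; On execute it clears the IsSitting blackboard flag and sets AnimationRunning.
; Each tick it checks AnimationRunning and finishes successfully once that flag is false, so clearing the flag is left to logic outside this task.
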(event EventReceiveExecute
  (params (OwnerActor :type Actor%20Object%20Reference))
  (bind _returnvalue (AI|GetBlackboard OwnerActor))
  (AI|Components|Blackboard|SetValueasBool _returnvalue (Variables|Default|GetIsSitting) false)
  (AI|Components|Blackboard|SetValueasBool _returnvalue (Variables|Default|GetAnimationRunning) true))

(event EventTick
  (params (OwnerActor :type Actor%20Object%20Reference) (DeltaSeconds :type Float%20%28single-precision%29))
  (if (not (ScalableFloat|GetValueasBool (AI|GetBlackboard OwnerActor) (Variables|Default|GetAnimationRunning)))
    (AI|BehaviorTree|FinishExecute true)))