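; NPC manager for the fast food game that spawns and tracks customers and crowd characters, registering itself on the game state.
; A looping timer picks a random available spawner, favoring customers when the queue has room during FastFoodPhase, otherwise crowd NPCs up to a cap.
; Spawners also serve as despawn points.
; Points of interest are grouped by type, claimed from shuffled lists, and chained through weighted-random DataTable transitions.
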(event Custom|RegisterNPC
  (params (Character :type Crowd%20Character%20Object%20Reference))
  (bind _asbp_customer_character (Utilities|Casting|CastToBP_CustomerCharacter Character)
    (:then
      (Utilities|Array|Add (Variables|Default|GetCustemersCharacters) _asbp_customer_character))
    (:CastFailed
      (Utilities|Array|Add (Variables|Default|GetCrowdsCharacters) Character))))

(event Custom|UnregisterNPC
  (params (Character :type Crowd%20Character%20Object%20Reference))
  (bind _asbp_customer_character (Utilities|Casting|CastToBP_CustomerCharacter Character)
    (:then
      (Utilities|Array|RemoveItem (Variables|Default|GetCustemersCharacters) _asbp_customer_character))
    (:CastFailed
      (Utilities|Array|RemoveItem (Variables|Default|GetCrowdsCharacters) Character))))

(event EventBeginPlay
  (Utilities|FlowControl|Sequence
    (:then_0
      (Variables|/Game/FFBlueprints/GameMode/FastFoodGameState.FastFoodGameState_C|SetNPCManager (CallFunction|GetFastFoodGameState) self)
      (POI|Initialize))
    (:then_1
      (bind _returnvalue (Utilities|Time|SetTimerbyFunctionName self "CheckIsEmptyNPCSpawner" (Variables|Spawn|GetNormalSpawnDelay) true (Variables|Spawn|GetFisrtSpawnDelay)))
      (Variables|Spawn|SetSpawnTimer _returnvalue))))

(event Collision|EventActorBeginOverlap
  (params (OtherActor :type Actor%20Object%20Reference)))

(event EventTick
  (params (DeltaSeconds :type Float%20%28single-precision%29)))

(fn ConstructionScript)

(fn GetSpecificPoi
  (params (Name :type Name))
  (bind _specialpoidefs (Variables|POI|GetSpecialPOIDefs))
  (bind _value (Utilities|Map|Find _specialpoidefs Name))
  (bind _pois (Utilities|Struct|BreakNPCPOIGroups _value))
  (LocalVariables|SetCount (Utilities|Array|Length _pois))
  (if (== 1 (LocalVariables|GetCount))
    (return (Utilities|Array|Get(acopy) _pois) (LocalVariables|GetCount))
    (else
      (return (Utilities|Array|Get(acopy) _pois (Math|Random|RandomIntegerinRange 0 (- (LocalVariables|GetCount) 1))) (LocalVariables|GetCount)))))

(fn Initialize
  (bind _cyclespoidefs (Variables|POI|GetCyclesPOIDefs))
  (bind _outactors (Actor|GetAllActorsOfClass "/Game/FFBlueprints/NPC/BP_NPCPOI.BP_NPCPOI_C"))
  (for _array_element _outactors
    (for (_array_element_2 _array_index) _cyclespoidefs
      (if (== (.type _array_element_2) (Variables|/Game/FFBlueprints/NPC/BP_NPCPOI.BP_NPCPOI_C|GetPOItype _array_element))
        (Utilities|Array|Add (.Places (Utilities|Struct|BreakPOIItemsList (Utilities|Array|Get(acopy) _cyclespoidefs _array_index))) _array_element)))))

(fn FindandOccupyPOI
  (params (RandomType :type Boolean) (PredefinedType :type POIType%20Enum :default "NewEnumerator0"))
  (if RandomType
    (LocalVariables|SetPOITypeEnum (Utilities|GetRandomPoiType))
    (else
      (LocalVariables|SetPOITypeEnum PredefinedType)))
  (bind _poiitem (Utilities|FindPOICycleDef (LocalVariables|GetPOITypeEnum))
    (:Output
      (if true
        (Utilities|Array|Shuffle (.places _poiitem)))
      (for _array_element (.places _poiitem)
        (if (not (Variables|/Game/FFBlueprints/NPC/BP_NPCPOI.BP_NPCPOI_C|GetOccupied _array_element))
          (Variables|/Game/FFBlueprints/NPC/BP_NPCPOI.BP_NPCPOI_C|SetOccupied _array_element true)
          (return _array_element (.cycleconfig _poiitem) true)))
      (return 0 0 false))))

(fn GetNextPOI
  (params (CurrentState :type POIType%20Enum :default "NewEnumerator0") (CycleConfig :type Data%20Table%20Object%20Reference))
  (bind _outrownames (DataTable|GetDataTableRowNames CycleConfig))
  (for _array_element _outrownames
    (bind _returnvalue (Utilities|GetDataTableRow CycleConfig _array_element)
      (:then
        (bind _structout (Utilities|Struct|SetmembersinPOIItem _returnvalue))
        (if (== CurrentState (.Current (Utilities|Struct|BreakPOIItem _structout)))
          (bind _output (POI|GetPoiTypebyProbability (.Next (Utilities|Struct|BreakPOIItem _structout))))
          (return _output))))))

(fn GetPoiTypebyProbability
  (params (Input :type Array%20of%20POI%20State%20Structures))
  (for _array_element Input
    (LocalVariables|SetProbabilitySum (+ (.probability _array_element) (LocalVariables|GetProbabilitySum))))
  (LocalVariables|SetCurrentRandom (Math|Random|RandomFloatinRange 0.0 1.0))
  (for (_array_element_2 _array_index) Input
    (if (Math|Float|InRange(Float) (LocalVariables|GetCurrentRandom) (LocalVariables|GetCurrentMin) (+ (/ (.probability _array_element_2) (LocalVariables|GetProbabilitySum)) (LocalVariables|GetCurrentMin)))
      (return (.POI (Utilities|Struct|BreakPOIState (Utilities|Array|Get(acopy) Input _array_index))))
      (else
        (LocalVariables|SetCurrentMin (/ (.probability _array_element_2) (LocalVariables|GetProbabilitySum))))))
  (return (.POI (Utilities|Struct|BreakPOIState (Utilities|Array|Get(acopy) Input)))))

(fn GetCountAllNPC
  (return (+ (Utilities|Array|Length (Variables|Default|GetCrowdsCharacters)) (Utilities|Array|Length (Variables|Default|GetCustemersCharacters)))))

(fn CheckIsEmptyNPCSpawner
  (Utilities|FlowControl|Sequence
    (:then_0
      (for _array_element (Variables|Default|GetSpawners)
        (if (Default|IsAviablePoint _array_element)
          (Utilities|Array|Add (LocalVariables|GetAviableSpawners) _array_element))))
    (:then_1
      (if (> (Utilities|Array|Length (LocalVariables|GetAviableSpawners)) 0)
        (Variables|Default|SetSelected (Utilities|Array|Get(acopy) (LocalVariables|GetAviableSpawners) (Math|Random|RandomInteger (Utilities|Array|Length (LocalVariables|GetAviableSpawners)))))
        (if (and (Default|IsFreeSlot (Variables|Default|GetQueue)) (Variables|/Game/FFBlueprints/GameMode/FastFoodGameState.FastFoodGameState_C|GetFastFoodPhase (CallFunction|GetFastFoodGameState)))
          (Default|SpawnCrowd (Variables|Default|GetSelected) "/Game/FFBlueprints/Crowd/BP_CustomerCharacter.BP_CustomerCharacter_C")
          (elif (< (CallFunction|GetCountAllNPC) (Variables|Default|GetMaxAiChars))
            (Default|SpawnCrowd (Variables|Default|GetSelected) "/Game/FFBlueprints/Crowd/CrowdCharacter.CrowdCharacter_C")
            (else
              (return))))
        (else
          (return))))))

(fn RegisterSpawner
  (params (Spawner :type Crowd%20Spawner%20and%20Despawner%20Object%20Reference))
  (Utilities|Array|Add (Variables|Default|GetSpawners) Spawner))

(fn GetAviableDespawner
  (for _array_element (Variables|Default|GetSpawners)
    (if (Default|IsAviablePoint _array_element)
      (Utilities|Array|Add (LocalVariables|GetAviable) _array_element)))
  (if (> (Utilities|Array|Length (LocalVariables|GetAviable)) 0)
    (return (Utilities|Array|Get(acopy) (LocalVariables|GetAviable) (Math|Random|RandomInteger (Utilities|Array|Length (LocalVariables|GetAviable)))))
    (else
      (return 0))))