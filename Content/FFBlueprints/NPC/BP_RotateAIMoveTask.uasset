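; Behavior tree task that turns an NPC's controlled pawn to face the actor stored in a blackboard key.
; On execute it caches start and look-at rotations, keeping current pitch, and sets IsRotating plus a RotateLeft flag derived from comparing roll values.
; Tick lerps along the shortest path by a fixed alpha step per tick, so speed depends on frame rate, then clears IsRotating and finishes successfully.
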(event EventReceiveExecute
  (params (OwnerActor :type Actor%20Object%20Reference))
  (bind _asbp_npcbase_aicontroller (Utilities|Casting|CastToBP_NPCBaseAIController OwnerActor))
  (bind _asactor (Utilities|Casting|CastToActor (AI|Components|Blackboard|GetValueasObject (AI|GetBlackboard _asbp_npcbase_aicontroller) (Variables|Default|GetActualObject))))
  (Variables|Default|SetStartRot (Transformation|GetActorRotation (Pawn|GetControlledPawn _asbp_npcbase_aicontroller)))
  (Variables|Default|SetEndRot (Math|Rotator|MakeRotator (.Roll (Math|Rotator|BreakRotator (Math|Rotator|FindLookatRotation (Transformation|GetActorLocation (Pawn|GetControlledPawn _asbp_npcbase_aicontroller)) (Transformation|GetActorLocation _asactor)))) (.Pitch (Math|Rotator|BreakRotator (Transformation|GetActorRotation (Pawn|GetControlledPawn _asbp_npcbase_aicontroller)))) (.Yaw (Math|Rotator|BreakRotator (Math|Rotator|FindLookatRotation (Transformation|GetActorLocation (Pawn|GetControlledPawn _asbp_npcbase_aicontroller)) (Transformation|GetActorLocation _asactor))))))
  (AI|Components|Blackboard|SetValueasBool (AI|GetBlackboard _asbp_npcbase_aicontroller) (Variables|Default|GetRotateLeft) (> (.Roll (Math|Rotator|BreakRotator (Variables|Default|GetStartRot))) (.Roll (Math|Rotator|BreakRotator (Variables|Default|GetEndRot)))))
  (AI|Components|Blackboard|SetValueasBool (AI|GetBlackboard _asbp_npcbase_aicontroller) (Variables|Default|GetIsRotating) true)
  (Variables|Default|SetReady true))

(event EventTick
  (params (OwnerActor :type Actor%20Object%20Reference) (DeltaSeconds :type Float%20%28single-precision%29))
  (if (Variables|Default|GetReady)
    (Transformation|SetActorRotation (Pawn|GetControlledPawn (stale _asbp_npcbase_aicontroller)) (Math|Rotator|Lerp(Rotator) (Variables|Default|GetStartRot) (Variables|Default|GetEndRot) (Variables|Default|GetAlpha) true))
    (if (>= (Variables|Default|GetAlpha) 1.0)
      (Variables|Default|SetAlpha 0.0)
      (Variables|Default|SetReady false)
      (AI|Components|Blackboard|SetValueasBool (AI|GetBlackboard OwnerActor) (Variables|Default|GetIsRotating) false)
      (AI|BehaviorTree|FinishExecute true)
      (else
        (bind _output_get (Variables|Default|SetAlpha (+ (stale _output_get) 0.05)))))
    (else
      (bind _asbp_npcbase_aicontroller (Utilities|Casting|CastToBP_NPCBaseAIController (stale EventReceiveExecute OwnerActor)))
      (bind _asactor (Utilities|Casting|CastToActor (AI|Components|Blackboard|GetValueasObject (AI|GetBlackboard _asbp_npcbase_aicontroller) (Variables|Default|GetActualObject))))
      (Variables|Default|SetStartRot (Transformation|GetActorRotation (Pawn|GetControlledPawn _asbp_npcbase_aicontroller)))
      (Variables|Default|SetEndRot (Math|Rotator|MakeRotator (.Roll (Math|Rotator|BreakRotator (Math|Rotator|FindLookatRotation (Transformation|GetActorLocation (Pawn|GetControlledPawn _asbp_npcbase_aicontroller)) (Transformation|GetActorLocation _asactor)))) (.Pitch (Math|Rotator|BreakRotator (Transformation|GetActorRotation (Pawn|GetControlledPawn _asbp_npcbase_aicontroller)))) (.Yaw (Math|Rotator|BreakRotator (Math|Rotator|FindLookatRotation (Transformation|GetActorLocation (Pawn|GetControlledPawn _asbp_npcbase_aicontroller)) (Transformation|GetActorLocation _asactor))))))
      (AI|Components|Blackboard|SetValueasBool (AI|GetBlackboard _asbp_npcbase_aicontroller) (Variables|Default|GetRotateLeft) (> (.Roll (Math|Rotator|BreakRotator (Variables|Default|GetStartRot))) (.Roll (Math|Rotator|BreakRotator (Variables|Default|GetEndRot)))))
      (AI|Components|Blackboard|SetValueasBool (AI|GetBlackboard _asbp_npcbase_aicontroller) (Variables|Default|GetIsRotating) true)
      (Variables|Default|SetReady true))))