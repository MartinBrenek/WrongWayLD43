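; BP_NPCDoBPTask is a behavior tree task that runs a task, identified by TaskID, on an NPC's CrowdCharacter pawn.
; On execute, it gets the pawn from the BP_NPCBaseAIController, stores it as Target and starts the task.
; Tick polls the task state, finishing successfully on None or Succes and failing on Fail.
; A pawn that is not a CrowdCharacter also fails the task.
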(event EventReceiveExecute
  (params (OwnerActor :type Actor%20Object%20Reference))
  (bind _asbp_npcbase_aicontroller (Utilities|Casting|CastToBP_NPCBaseAIController OwnerActor))
  (bind _ascrowd_character (Utilities|Casting|CastToCrowdCharacter (Pawn|GetControlledPawn _asbp_npcbase_aicontroller))
    (:then
      (bind _output_get (Variables|Default|SetTarget _ascrowd_character))
      (Default|StartTask _output_get (Variables|Default|GetTaskID)))
    (:CastFailed
      (AI|BehaviorTree|FinishExecute false))))

(event EventTick
  (params (OwnerActor :type Actor%20Object%20Reference) (DeltaSeconds :type Float%20%28single-precision%29))
  (switch Utilities|FlowControl|Switch|SwitchonTaskState (Default|GetTaskState (Variables|Default|GetTarget) (Variables|Default|GetTaskID))
    (:NewEnumerator3
      (AI|BehaviorTree|FinishExecute true))
    (:NewEnumerator1
      (AI|BehaviorTree|FinishExecute true))
    (:NewEnumerator2
      (AI|BehaviorTree|FinishExecute false))))