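; Behavior tree task that runs the Bald King NPC's trade and reports its result to the tree.
; On execute it gets the controlled BaldKing pawn through the base NPC AI controller and calls StartTrade on it.
; Tick then polls the king's TradeRunning state and finishes the task as succeeded or failed to match.
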(event EventReceiveExecute
  (params (OwnerActor :type Actor%20Object%20Reference))
  (bind _asbp_npcbase_aicontroller (Utilities|Casting|CastToBP_NPCBaseAIController OwnerActor))
  (bind _asbald_king (Utilities|Casting|CastToBaldKing (Pawn|GetControlledPawn _asbp_npcbase_aicontroller)))
  (bind _output_get (Variables|Default|SetKing _asbald_king))
  (Default|StartTrade _output_get))

(event EventTick
  (params (OwnerActor :type Actor%20Object%20Reference) (DeltaSeconds :type Float%20%28single-precision%29))
  (switch Utilities|FlowControl|Switch|SwitchonTaskState (Variables|/Game/FFBlueprints/NPC/BaldKing/BaldKing.BaldKing_C|GetTradeRunning (Variables|Default|GetKing))
    (:NewEnumerator1
      (AI|BehaviorTree|FinishExecute true))
    (:NewEnumerator2
      (AI|BehaviorTree|FinishExecute false))))