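; BP_OfferingServicesTask is a behavior tree task for the BaldKing NPC's offering-services state in its Whore role.
; On execute it sets the AnimationRunning and IsOffering blackboard flags to true.
; Tick polls AnimationRunning, which is cleared outside this task, then resets IsOffering and finishes successfully once the Owner key casts to BP_BaldKing.
; The task plays no animation itself and only signals through the blackboard.
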(event EventReceiveExecute
  (params (OwnerActor :type Actor%20Object%20Reference))
  (bind _returnvalue (AI|GetBlackboard OwnerActor))
  (AI|Components|Blackboard|SetValueasBool _returnvalue (Variables|Default|GetAnimationRunning) true)
  (AI|Components|Blackboard|SetValueasBool _returnvalue (Variables|Default|GetIsOffering) true)
  (Utilities|Casting|CastToBP_BaldKing (AI|Components|Blackboard|GetValueasObject _returnvalue (Variables|Default|GetOwner))))

(event EventTick
  (params (OwnerActor :type Actor%20Object%20Reference) (DeltaSeconds :type Float%20%28single-precision%29))
  (bind _returnvalue (AI|GetBlackboard OwnerActor))
  (if (not (ScalableFloat|GetValueasBool _returnvalue (Variables|Default|GetAnimationRunning)))
    (AI|Components|Blackboard|SetValueasBool _returnvalue (Variables|Default|GetIsOffering) false)
    (Utilities|Casting|CastToBP_BaldKing (AI|Components|Blackboard|GetValueasObject _returnvalue (Variables|Default|GetOwner)))
    (AI|BehaviorTree|FinishExecute true)))