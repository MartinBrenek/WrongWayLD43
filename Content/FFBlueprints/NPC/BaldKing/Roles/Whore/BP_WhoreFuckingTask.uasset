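; Behavior tree task that runs a timed sex interaction for a BaldKing NPC, filed under its Whore role.
; It fetches the NPC from the blackboard, offsets it along world X, disables capsule collision, calls WaitForFuck and sets IsFucking.
; After a fixed delay it clears IsFucking and CanFuck, reverses the offset, calls EndFuck, restores collision and finishes successfully.
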(event EventReceiveExecute
  (params (OwnerActor :type Actor%20Object%20Reference))
  (bind _returnvalue (AI|GetBlackboard OwnerActor))
  (bind _asbp_bald_king (Utilities|Casting|CastToBP_BaldKing (AI|Components|Blackboard|GetValueasObject _returnvalue (Variables|Default|GetOwner))))
  (Transformation|SetActorLocation _asbp_bald_king (+ (Transformation|GetActorLocation _asbp_bald_king) "50.000000, 0, 0") false false)
  (Collision|SetCollisionEnabled (Variables|/Script/Engine.Character|GetCapsuleComponent _asbp_bald_king) "NoCollision")
  (Default|WaitforFuck _asbp_bald_king)
  (AI|Components|Blackboard|SetValueasBool _returnvalue (Variables|Default|GetIsFucking) true)
  (Utilities|FlowControl|Delay 5.0)
  (AI|Components|Blackboard|SetValueasBool _returnvalue (Variables|Default|GetIsFucking) false)
  (AI|Components|Blackboard|SetValueasBool _returnvalue (Variables|Default|GetCanFuck) false)
  (Transformation|SetActorLocation _asbp_bald_king (+ (Transformation|GetActorLocation _asbp_bald_king) "-50.000000, 0, 0") false false)
  (Default|EndFuck _asbp_bald_king)
  (Collision|SetCollisionEnabled (Variables|/Script/Engine.Character|GetCapsuleComponent _asbp_bald_king) "QueryAndPhysics")
  (AI|BehaviorTree|FinishExecute true))