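; BP_CanFuckTask is a behavior tree task for a BaldKing NPC role that acts as a readiness handshake for sex between two actors.
; On execute it sets the owner's CanFuck blackboard flag and caches the actor stored under the Target key.
; Tick polls that actor's blackboard and finishes successfully once its CanFuck flag is also true.
; It has no timeout or failure finish, including when the Target cast fails.
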(event EventTick
  (params (OwnerActor :type Actor%20Object%20Reference) (DeltaSeconds :type Float%20%28single-precision%29))
  (if (ScalableFloat|GetValueasBool (AI|GetBlackboard (Variables|Default|GetTargetActor)) (Variables|Default|GetCanFuck))
    (AI|BehaviorTree|FinishExecute true)))

(event EventReceiveExecute
  (params (OwnerActor :type Actor%20Object%20Reference))
  (bind _returnvalue (AI|GetBlackboard OwnerActor))
  (AI|Components|Blackboard|SetValueasBool _returnvalue (Variables|Default|GetCanFuck) true)
  (bind _asactor (Utilities|Casting|CastToActor (AI|Components|Blackboard|GetValueasObject _returnvalue (Variables|Default|GetTarget))))
  (Variables|Default|SetTargetActor _asactor))