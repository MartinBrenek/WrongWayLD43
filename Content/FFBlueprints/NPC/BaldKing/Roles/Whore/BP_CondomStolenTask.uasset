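; Behavior tree task for the BaldKing NPC that handles the condom-stolen quest step.
; On execute it sets the QuestCompleted blackboard flag to true.
; Its tick calls CondomStolen on the BP_BaldKing stored in the Owner blackboard key, but only while that flag is false.
; The graph contains no Finish Execute call.
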(event EventReceiveExecute
  (params (OwnerActor :type Actor%20Object%20Reference))
  (AI|Components|Blackboard|SetValueasBool (AI|GetBlackboard OwnerActor) (Variables|Default|GetQuestCompleted) true))

(event EventTick
  (params (OwnerActor :type Actor%20Object%20Reference) (DeltaSeconds :type Float%20%28single-precision%29))
  (bind _returnvalue (AI|GetBlackboard OwnerActor))
  (if (not (ScalableFloat|GetValueasBool _returnvalue (Variables|Default|GetQuestCompleted)))
    (bind _asbp_bald_king (Utilities|Casting|CastToBP_BaldKing (AI|Components|Blackboard|GetValueasObject _returnvalue (Variables|Default|GetOwner))))
    (Default|CondomStolen _asbp_bald_king)))