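; BP_BaldkingState is the state machine for the Bald King NPC, specializing a parent state class with Bald King state and transition enums.
; It sets an initial state on BeginPlay, wraps the parent's set, get and next-state calls with enum conversions, and raises a typed event on state changes.
; Helper functions count transitions, map state names to indices, and convert data table rows into transition-indexed arrays of target states.
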(event EventBeginPlay
  (|CallParentFunction)
  (CallFunction|SetStateBaldKing "NewEnumerator0"))

(event EventTick
  (params (DeltaSeconds :type Float%20%28single-precision%29))
  (|CallParentFunction DeltaSeconds) ; This node is disabled and will not be called.\nDrag off pins to build functionality.
)

(event EventSetState
  (params (State :type Byte :default 0))
  (|CallParentFunction State)
  (Default|CallNewStateBaldKing (Utilities|Enum|ByteToEnumStateBaldKing State)))

(fn NextStateBaldKing
  (params (Transition :type TransitionStateBaldKing%20Enum :default "NewEnumerator5"))
  (bind (_nextstatefound _newstate) (CallFunction|NextState Transition))
  (return _nextstatefound (Utilities|Enum|ByteToEnumStateBaldKing _newstate)))

(fn GetActualStateBaldKing
  (bind _state (CallFunction|GetActualState))
  (return (Utilities|Enum|ByteToEnumStateBaldKing _state)))

(fn SetStateBaldKing
  (params (State :type StateBaldKing%20Enum :default "NewEnumerator5"))
  (CallFunction|SetState State))

(fn GetNumOfTransition
  (|ForEachTransitionStateBaldKing
    (:LoopBody
      (Math|Integer|IncrementInt (LocalVariables|GetNumTransition)))
    (:then
      (return (LocalVariables|GetNumTransition)))))

(fn GetStringtoState
  (bind _enumvalue (|ForEachStateBaldKing)
    (:LoopBody
      (Utilities|Map|Add (LocalVariables|GetStateFromString) (Utilities|String|EnumtoString _enumvalue) (Math|Conversions|ToInteger(Byte) _enumvalue)))
    (:then
      (return (LocalVariables|GetStateFromString)))))

(fn GetRowArrayfromTable
  (params (Row :type Name :default "None") (Table :type Data%20Table%20Object%20Reference) (NumTransition :type Integer))
  (bind _returnvalue (Utilities|GetDataTableRow Table Row)
    (:then
      (Utilities|FlowControl|Sequence
        (:then_0
          (Utilities|Array|SetArrayElem (LocalVariables|GetTempArray) (- NumTransition 1) 0 true))
        (:then_1
          (bind _output_get (LocalVariables|SetRowStruct _returnvalue))
          (for _array_element (Utilities|Struct|BreakTableTranstionStructBaldKing _output_get)
            (Utilities|Array|SetArrayElem (LocalVariables|GetTempArray) (Math|Conversions|ToInteger(Byte) (.Transition (Utilities|Struct|BreakTransPairBaldking _array_element))) (Math|Conversions|ToInteger(Byte) (.State (Utilities|Struct|BreakTransPairBaldking _array_element)))))
          (return (LocalVariables|GetTempArray)))))))