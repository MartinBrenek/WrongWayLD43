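; Behavior tree task that makes the Bald King NPC perform its trash bin search.
; On execute it caches the controlled BP_BaldKing, sets the AnimationRunning blackboard flag and starts the search.
; Tick polls that flag until it is false, then stops the search and finishes successfully, or fails if the King reference is invalid.
; The task never clears the flag itself.
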(event EventReceiveExecute
  (params (OwnerActor :type Actor%20Object%20Reference))
  (bind _asbp_npcbase_aicontroller (Utilities|Casting|CastToBP_NPCBaseAIController OwnerActor))
  (bind _asbp_bald_king (Utilities|Casting|CastToBP_BaldKing (Pawn|GetControlledPawn _asbp_npcbase_aicontroller)))
  (bind _output_get (Variables|Default|SetKing _asbp_bald_king))
  (AI|Components|Blackboard|SetValueasBool (AI|GetBlackboard OwnerActor) (Variables|Default|GetAnimationRunning) true)
  (Default|SearchTrashBin _output_get true))

(event EventTick
  (params (OwnerActor :type Actor%20Object%20Reference) (DeltaSeconds :type Float%20%28single-precision%29))
  (bind _king (Variables|Default|GetKing))
  (if (not (ScalableFloat|GetValueasBool (AI|GetBlackboard OwnerActor) (Variables|Default|GetAnimationRunning)))
    (Utilities|IsValid _king
      (:Is%20Valid
        (Default|SearchTrashBin _king false)
        (AI|BehaviorTree|FinishExecute true))
      (:Is%20Not%20Valid
        (AI|BehaviorTree|FinishExecute false)))))