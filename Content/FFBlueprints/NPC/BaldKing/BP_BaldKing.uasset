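; BaldKing quest NPC whose roles include businessman (King), junkie and prostitute, each with a stealable item: suitcase, weed or condom.
; BPBaldkingState holds the saved role, which routes shared events and selects mesh and props.
; Behavior tree actions drive role-specific item display, offering and customer pairing with BP_Wanderer.
; Thefts toggle player bullet time and end quests; businessman and junkie theft endings advance state and target the DrugDen.
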(event Custom|NewStateSet
  (params (NewState :type BaldKingState%20Enum :default "NewEnumerator5"))
  ;[1 1 1] Startup setup
  (CallFunction|ChangeRole NewState))

(event Custom|StolenEnd
  ;[1 1 1] SharedActions
  (switch Utilities|FlowControl|Switch|SwitchonBaldKingState (Default|GetActualStateBaldKing (Variables|Default|GetBP_BaldkingState))
    (:NewEnumerator1
      (CallFunction|BusinessmanStolenEnd))
    (:NewEnumerator3
      (CallFunction|JunkieStolenEnd))))

(event EventBeginPlay
  ;[1 1 1] Startup setup
  (|CallParentFunction)
  (EventDispatchers|BindEventtoNewStateBaldKing (Variables|Default|GetBP_BaldkingState) (delegate Custom|NewStateSet)))

(event Collision|EventActorBeginOverlap
  (params (OtherActor :type Actor%20Object%20Reference)))

(event EventInitializePawn
  (params (State :type Byte :default 0))
  ;[1 1 1] NPC visual update
  (switch Utilities|FlowControl|Switch|SwitchonBaldKingState (Utilities|Enum|ByteToEnumBaldKingState State)
    (:NewEnumerator1
      (CallFunction|ShowItem "/Game/FFBlueprints/Ingredients/BP_MoneyCase.BP_MoneyCase_C" "None" "NewEnumerator0")
      (Rendering|SetVisibility (Variables|Default|Getjoint) false false)
      (Components|Activation|SetActive (Variables|Default|GetParticleSystem) false false)
      (Rendering|SetVisibility (Variables|Default|GetPurse) false false)
      (Rendering|SetVisibility (Variables|Default|Getskirt) false true))
    (:NewEnumerator2
      (Rendering|SetVisibility (Variables|Default|Getjoint) false false)
      (Components|Activation|SetActive (Variables|Default|GetParticleSystem) false false))
    (:NewEnumerator3
      (Rendering|SetVisibility (Variables|Default|GetPurse) false true)
      (Rendering|SetVisibility (Variables|Default|Getskirt) false false)
      (Class|SkinnedMeshComponent|SetSkeletalMesh (Variables|Character|GetMesh) "/Game/assets/characters/plesoun/plesoun_homeless.plesoun_homeless" true)
      (Rendering|SetVisibility (Variables|Default|Getjoint) false false :!label _label)
      (Components|Activation|SetActive (Variables|Default|GetParticleSystem) false false))
    (:NewEnumerator4
      (Rendering|SetVisibility (Variables|Default|GetPurse) true false)
      (Rendering|SetVisibility (Variables|Default|Getskirt) false false)
      (Class|SkinnedMeshComponent|SetSkeletalMesh (Variables|Character|GetMesh) "/Game/assets/characters/plesoun/plesoun_hooker.plesoun_hooker" true)
      (goto _label))))

(event EventTick
  (params (DeltaSeconds :type Float%20%28single-precision%29)))

(event EventUseItem
  ;[1 1 1] SharedActions
  (switch Utilities|FlowControl|Switch|SwitchonBaldKingState (Default|GetActualStateBaldKing (Variables|Default|GetBP_BaldkingState))
    (:NewEnumerator3
      (CallFunction|UseJunkie))))

(event EventCAlltoStartQuest
  (params (QuestType :type Ingredients%20Enum :default "NewEnumerator9"))
  (bind _bp_baldkingstate (Variables|Default|GetBP_BaldkingState))
  ;[1 1 1] Quest start/end
  (|CallParentFunction QuestType)
  (switch Utilities|FlowControl|Switch|SwitchonBaldKingState (Default|GetActualStateBaldKing _bp_baldkingstate)
    (:NewEnumerator0
      (Default|NextState _bp_baldkingstate "NewEnumerator2"))
    (:NewEnumerator2
      (Default|NextState _bp_baldkingstate "NewEnumerator2"))))

(event EventCalltoEndQuest
  ;[1 1 1] Quest start/end
  (switch Utilities|FlowControl|Switch|SwitchonBaldKingState (Default|GetActualStateBaldKing (Variables|Default|GetBP_BaldkingState))
    (:NewEnumerator1
      _)
    (:NewEnumerator3
      _)
    (:NewEnumerator4
      _))
  (AI|Components|Blackboard|SetValueasBool (AI|GetBlackboard 0) (Utilities|Name|MakeLiteralName "InQuest") false))

(event EventUpdatePawnState
  (params (Key :type Byte :default 0))
  ;[1 1 1] BT action update
  (bind _output_get (Variables|Default|SetCurrentAction (Utilities|Enum|ByteToEnumE_BaldKingAction Key)))
  (switch Utilities|FlowControl|Switch|SwitchonE_BaldKingAction _output_get
    (:NewEnumerator0
      (Variables|Default|SetCanInteract true)
      (Utilities|FlowControl|Delay 3.0)
      (Variables|Default|SetCanInteract false)
      (Default|CallOnJobEnded true))
    (:NewEnumerator2
      (if (ScalableFloat|GetValueasBool (AI|GetBlackboard 0) (Variables|Default|GetIsInQuest))
        _))
    (:NewEnumerator5
      (CallFunction|ShowItem "/Game/FFBlueprints/Ingredients/BP_MoneyCase.BP_MoneyCase_C" "None" "NewEnumerator0"))
    (:NewEnumerator8
      (CallFunction|UseDrugs))
    (:NewEnumerator11
      (CallFunction|WaitforCustomer))
    (:NewEnumerator12
      (CallFunction|StartFuck))))

(event EventLoadedData
  (params (Data :type Save%20Object%20Data%20Structure))
  ;[1 1 1] Startup setup
  (Default|SetState (Variables|Default|GetBP_BaldkingState) (.State (Utilities|Struct|BreakSaveObjectData Data))))

(event EventShouldChangeVisual
  ;[1 0.1603 0] Deprecated - MESS
)

(event EventItemPickedAction
  (params (Item :type Pickable%20Item%20Object%20Reference) (Picked :type Boolean))
  ;[1 1 1] SharedActions
  (switch Utilities|FlowControl|Switch|SwitchonBaldKingState (Default|GetActualStateBaldKing (Variables|Default|GetBP_BaldkingState))
    (:NewEnumerator1
      (CallFunction|TrytoStoleSuitCase Picked))
    (:NewEnumerator3
      (CallFunction|TrytoPickupWeed Picked))
    (:NewEnumerator4
      (CallFunction|TrytoPickUpCondom Picked))))

(event Custom|TryToStoleSuitCase
  (params (Picked :type Boolean))
  ;[1 1 1] Used events
  (if Picked
    (Default|BulletTimePressed (CallFunction|GetPlayer))
    (AI|Components|Blackboard|SetValueasBool (AI|GetBlackboard 0) (Variables|Default|GetStolen_key) true)
    (CallFunction|CalltoEndQuest)
    (bind _actor (CallFunction|GetActorReference "GreenGrocer"))
    (bind _asbp_green_grocer (Utilities|Casting|CastToBP_GreenGrocer _actor))
    (Default|CalltoEndQuest _asbp_green_grocer)))

(event Custom|LeaveOnTable
  ;[1 1 1] Used events
  (Variables|Default|SetReadyToUse true))

(event Custom|TakeFromTable
  ;[1 1 1] Used events
  (Variables|Default|SetReadyToUse false))

(event Custom|BusinessmanStolenEnd
  (AI|Components|Blackboard|SetValueasBool (AI|GetBlackboard 0) (Utilities|Name|MakeLiteralName "InQuest") false)
  (bind _newstate (Default|NextState (Variables|Default|GetBP_BaldkingState) "NewEnumerator8"))
  (bind _asbp_npcbald_king_ai (Utilities|Casting|CastToBP_NPCBaldKingAI (Pawn|GetController)))
  (bind _point (Default|GetSpecificPoi _asbp_npcbald_king_ai "DrugDen"))
  (AI|Components|Blackboard|SetValueasObject (AI|GetBlackboard 0) (Utilities|Name|MakeLiteralName "ActualObject") _point)
  (CallFunction|ChangeRole _newstate))

(event Custom|StartSmokeWeed
  (bind _joint (Variables|Default|Getjoint))
  (Rendering|SetVisibility (Variables|Default|Getjoint) true true)
  (Components|Activation|SetActive (Variables|Default|GetParticleSystem) true true)
  (Utilities|EnableCollision (Variables|Default|Getjoint) true
    (:NewParam
      (bind (_direction _scale _position) (Timeline|Timeline_1 PlayFromStart)
        (:Update
          (Transformation|SetRelativeScale3D _joint _scale)
          (Transformation|SetRelativeLocation _joint _position false true))
        (:Finished
          (Rendering|SetVisibility (Variables|Default|Getjoint) false true)
          (Components|Activation|SetActive (Variables|Default|GetParticleSystem) false false)
          (Utilities|EnableCollision (Variables|Default|Getjoint) false))))))

(event Custom|UseDrugs
  (bind _item (CallFunction|ShowItem "/Game/FFBlueprints/NPC/BaldKing/BaldKingItems/BP_Weed.BP_Weed_C" "None" "NewEnumerator1"))
  (Physics|SetSimulatePhysics (Variables|/Game/FFBlueprints/PickableItem.PickableItem_C|GetCube _item) true))

(event Custom|PickUpWeed
  (CallFunction|HideItem "/Game/FFBlueprints/NPC/BaldKing/BaldKingItems/BP_Weed.BP_Weed_C" "None"))

(event Custom|UseJunkie
  (bind _joint (Variables|Default|Getjoint))
  (Utilities|FlowControl|Sequence
    (:then_1
      (bind (_direction _scale _position) (Timeline|Timeline_1 Stop)
        (:Update
          (Transformation|SetRelativeScale3D _joint _scale)
          (Transformation|SetRelativeLocation _joint _position false true))
        (:Finished
          (Rendering|SetVisibility (Variables|Default|Getjoint) false true :!label _label)
          (Components|Activation|SetActive (Variables|Default|GetParticleSystem) false false)
          (Utilities|EnableCollision (Variables|Default|Getjoint) false))))
    (:then_2
      (goto _label))))

(event Custom|JunkieStolenEnd
  (Default|NextState (Variables|Default|GetBP_BaldkingState) "NewEnumerator8")
  (bind _asbp_npcbald_king_ai (Utilities|Casting|CastToBP_NPCBaldKingAI (Pawn|GetController)))
  (AI|Components|Blackboard|SetValueasBool (AI|GetBlackboard _asbp_npcbald_king_ai) (Utilities|Name|MakeLiteralName "InQuest") false)
  (bind _point (Default|GetSpecificPoi _asbp_npcbald_king_ai "DrugDen"))
  (AI|Components|Blackboard|SetValueasObject (AI|GetBlackboard _asbp_npcbald_king_ai) (Utilities|Name|MakeLiteralName "ActualObject") _point)
  (Default|SetupData _asbp_npcbald_king_ai (Utilities|Enum|LiteralenumBaldKingState "NewEnumerator2")))

(event Custom|TryToPickupWeed
  (params (Picked :type Boolean))
  (if Picked
    (Default|BulletTimePressed (CallFunction|GetPlayer))
    (AI|Components|Blackboard|SetValueasBool (AI|GetBlackboard self) (Variables|Default|GetIsStolenKey) true)
    (CallFunction|CalltoEndQuest)))

(event Custom|StartJunkieQuest
  (bind _asbp_npcbase_aicontroller (Utilities|Casting|CastToBP_NPCBaseAIController (Pawn|GetController)))
  (Default|SetupData _asbp_npcbase_aicontroller (Utilities|Enum|LiteralenumBaldKingState "NewEnumerator2")))

(event Custom|WaitForCustomer
  (bind _asfast_food_game_state (Utilities|Casting|CastToFastFoodGameState (Game|GetGameState)))
  (bind (_value _found) (Default|GetActorReference (Variables|/Game/FFBlueprints/GameMode/FastFoodGameState.FastFoodGameState_C|GetQuestManager _asfast_food_game_state) (Variables|Default|GetWanderer)))
  (if _found
    (bind _asbp_wanderer (Utilities|Casting|CastToBP_Wanderer _value))
    (Default|SetupWhoreTarget _asbp_wanderer self)
    (CallFunction|SetupWandererTarget _asbp_wanderer)))

(event Custom|StartFuck
  (Transformation|SetActorLocation (+ (Transformation|GetActorLocation) "50.000000, 0, 0") false false)
  (Collision|SetCollisionEnabled (Variables|Default|GetCapsuleComponent) "NoCollision"))

(event Custom|TryToPickUpCondom
  (params (Picked :type Boolean))
  (if Picked
    (Default|BulletTimePressed (CallFunction|GetPlayer))
    (Variables|Default|SetActiveItem 0)
    (bind _asbp_wanderer (Utilities|Casting|CastToBP_Wanderer (AI|Components|Blackboard|GetValueasObject (AI|GetBlackboard 0) (Variables|Default|GetWanderer))))
    (AI|Components|Blackboard|SetValueasBool (AI|GetBlackboard _asbp_wanderer) (Variables|Default|GetInQuestKey) false)
    (Default|CondomStolen _asbp_wanderer)
    (CallFunction|CalltoEndQuest)))

(event Custom|StopOffering
  (Default|CallOnJobEnded true))

(event Custom|EndFuck
  (Transformation|SetActorLocation (+ (Transformation|GetActorLocation) "-50.000000, 0, 0") false false)
  (Collision|SetCollisionEnabled (Variables|Default|GetCapsuleComponent) "QueryAndPhysics")
  (CallFunction|SetupWandererTarget))

(event Custom|CondomStolen
  (CallFunction|CalltoEndQuest))

(fn ConstructionScript)

(fn SetState
  (bind _asfast_food_game_state (Utilities|Casting|CastToFastFoodGameState (Game|GetGameState)))
  (bind (_value _found) (Default|GetQuestData (Variables|/Game/FFBlueprints/GameMode/FastFoodGameState.FastFoodGameState_C|GetQuestManager _asfast_food_game_state) (Variables|Default|GetQuestDataKey)))
  (if _found
    (Variables|Default|SetState _value)
    (else
      (Variables|Default|SetState 0)))
  (CallFunction|InitializePawn (Utilities|Enum|LiteralenumBaldKingState "NewEnumerator5")))

(fn SetupWandererTarget
  (params (Wanderer :type Actor%20Object%20Reference))
  (AI|Components|Blackboard|SetValueasObject (AI|GetBlackboard 0) (Variables|Default|GetWanderer) Wanderer))

(fn SetupWeed
  (params (ShouldSpawn :type Boolean))
  (bind _weedspawn (Variables|Default|GetWeedSpawn))
  (bind _returnvalue (Transformation|GetWorldTransform _weedspawn))
  (if ShouldSpawn
    (bind _returnvalue_2 (Game|SpawnActorfromClass "/Game/FFBlueprints/NPC/BaldKing/BaldKingItems/BP_Weed.BP_Weed_C" (Math|Transform|MakeTransform (.location _returnvalue) (.rotation _returnvalue) "1,1,1") "AdjustIfPossibleButAlwaysSpawn" 0 0))
    (bind _output_get (Variables|Default|SetSpawnedWeed _returnvalue_2))
    (Physics|SetSimulatePhysics (Variables|/Game/FFBlueprints/PickableItem.PickableItem_C|GetCube _output_get) true)
    (else
      (Utilities|IsValid (Variables|Default|GetSpawnedWeed)
        (:Is%20Valid
          (EventDispatchers|UnbindallEventsfromItemPickedbyPlayer (Variables|Default|GetSpawnedWeed))
          (Actor|DestroyActor (Variables|Default|GetSpawnedWeed)))))))

(fn IsReadytoUse
  (return (Variables|Default|GetReadyToUse)))

(fn CombinewithItem
  (params (ItemToCombine :type Actor%20Object%20Reference))
  (return false false false false))

(fn GetSaveData
  (bind _state (Default|GetActualState (Variables|Default|GetBP_BaldkingState)))
  (return (Utilities|Struct|MakeSaveObjectData (Utilities|GetClass self) (Transformation|GetWorldTransform (Variables|Default|GetCapsuleComponent)) "0.000000,0.000000,0.000000|0.000000,0.000000,0.000000|1.000000,1.000000,1.000000" _state)))