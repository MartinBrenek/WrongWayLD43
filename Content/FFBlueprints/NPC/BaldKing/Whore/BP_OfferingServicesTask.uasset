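; Behavior tree task that runs the BaldKing NPC's offering-services action.
; On execute it sets the AnimationRunning and IsOffering blackboard flags, then calls OfferServices on the BaldKing stored under the Owner key.
; Tick polls AnimationRunning, which this task never clears itself.
; Once that flag is false, it clears IsOffering, calls OfferingFinnished on the BaldKing and finishes with success.
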(event EventReceiveExecute
  (params (OwnerActor :type Actor%20Object%20Reference))
  (bind _returnvalue (AI|GetBlackboard OwnerActor))
  (AI|Components|Blackboard|SetValueasBool _returnvalue (Variables|Default|GetAnimationRunning) true)
  (AI|Components|Blackboard|SetValueasBool _returnvalue (Variables|Default|GetIsOffering) true)
  (bind _asbald_king (Utilities|Casting|CastToBaldKing (AI|Components|Blackboard|GetValueasObject _returnvalue (Variables|Default|GetOwner))))
  (Default|OfferServices _asbald_king))

(event EventTick
  (params (OwnerActor :type Actor%20Object%20Reference) (DeltaSeconds :type Float%20%28single-precision%29))
  (bind _returnvalue (AI|GetBlackboard OwnerActor))
  (if (not (ScalableFloat|GetValueasBool _returnvalue (Variables|Default|GetAnimationRunning)))
    (AI|Components|Blackboard|SetValueasBool _returnvalue (Variables|Default|GetIsOffering) false)
    (bind _asbald_king (Utilities|Casting|CastToBaldKing (AI|Components|Blackboard|GetValueasObject _returnvalue (Variables|Default|GetOwner))))
    (Default|OfferingFinnished _asbald_king)
    (AI|BehaviorTree|FinishExecute true)))