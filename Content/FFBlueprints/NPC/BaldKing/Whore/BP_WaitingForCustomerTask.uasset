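; Behavior tree task that puts a BaldKing NPC into a waiting-for-customer state.
; On execute it casts the blackboard Owner to BaldKing, calls WaitForCustomer and sets the IsWaiting and AnimationRunning flags.
; Tick polls IsWaiting and finishes the task successfully once another source clears it.
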(event EventReceiveExecute
  (params (OwnerActor :type Actor%20Object%20Reference))
  (bind _returnvalue (AI|GetBlackboard OwnerActor))
  (bind _asbald_king (Utilities|Casting|CastToBaldKing (AI|Components|Blackboard|GetValueasObject _returnvalue (Variables|Default|GetOwner))))
  (Default|WaitforCustomer _asbald_king)
  (AI|Components|Blackboard|SetValueasBool _returnvalue (Variables|Default|GetIsWaiting) true)
  (AI|Components|Blackboard|SetValueasBool _returnvalue (Variables|Default|GetAnimationRunning) true))

(event EventTick
  (params (OwnerActor :type Actor%20Object%20Reference) (DeltaSeconds :type Float%20%28single-precision%29))
  (if (not (ScalableFloat|GetValueasBool (AI|GetBlackboard OwnerActor) (Variables|Default|GetIsWaiting)))
    (AI|BehaviorTree|FinishExecute true)))