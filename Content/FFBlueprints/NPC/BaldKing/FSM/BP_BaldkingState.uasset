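; Bald King NPC state machine, specializing a parent FSM with the Bald King's own state enum.
; State changes run the parent logic, then fire a Bald King-typed new-state call.
; Overrides convert data table rows into transition-indexed state arrays, map state names to values, and supply state and action names as text.
; NextStateBaldKing is a deprecated stub that logs a notice to use NextState.
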(event EventBeginPlay
  (|CallParentFunction))

(event EventTick
  (params (DeltaSeconds :type Float%20%28single-precision%29))
  (|CallParentFunction DeltaSeconds) ; This node is disabled and will not be called.\nDrag off pins to build functionality.
)

(event EventSetState
  (params (State :type Byte :default 0))
  (|CallParentFunction State)
  (Default|CallNewStateBaldKing (Utilities|Enum|ByteToEnumBaldKingState State))
  (CallFunction|DebugLog "-----------CALL NEW STATE" "NewEnumerator0"))

(fn NextStateBaldKing
  (params (Transition :type TransitionStateBaldKing%20Enum :default "NewEnumerator5"))
  (CallFunction|DebugLog "Called Old Next State BaldKing (use only NextState)" "NewEnumerator1")
  (return false "NewEnumerator5"))

(fn GetActualStateBaldKing
  (bind _state (CallFunction|GetActualState))
  (return (Utilities|Enum|ByteToEnumBaldKingState _state)))

(fn SetStateBaldKing
  (params (State :type BaldKingState%20Enum :default "NewEnumerator5"))
  (CallFunction|SetState State))

(fn GetStringtoState
  (bind _enumvalue (|ForEachBaldKingState)
    (:LoopBody
      (Utilities|Map|Add (LocalVariables|GetStateFromString) (Utilities|String|EnumtoString _enumvalue) (Math|Conversions|ToInteger(Byte) _enumvalue)))
    (:then
      (return (LocalVariables|GetStateFromString)))))

(fn GetRowArrayfromTable
  (params (Row :type Name :default "None") (Table :type Data%20Table%20Object%20Reference) (NumTransition :type Integer))
  (bind _returnvalue (Utilities|GetDataTableRow Table Row)
    (:then
      (Utilities|FlowControl|Sequence
        (:then_0
          (Utilities|Array|SetArrayElem (LocalVariables|GetTempArray) (- NumTransition 1) 0 true))
        (:then_1
          (bind _output_get (LocalVariables|SetRowStruct _returnvalue))
          (for _array_element (Utilities|Struct|BreakTableTranstionStructBaldKing _output_get)
            (Utilities|Array|SetArrayElem (LocalVariables|GetTempArray) (Math|Conversions|ToInteger(Byte) (.Transition (Utilities|Struct|BreakTransPairBaldking _array_element))) (Math|Conversions|ToInteger(Byte) (.State (Utilities|Struct|BreakTransPairBaldking _array_element)))))
          (return (LocalVariables|GetTempArray)))))))

(fn GetEnumStatetoText
  (params (EnumByte :type Byte :default 0))
  (return (Utilities|String|EnumtoString (Utilities|Enum|ByteToEnumBaldKingState EnumByte))))

(fn GetEnumActiontoText
  (bind _asbp_bald_king (Utilities|Casting|CastToBP_BaldKing (Variables|Default|GetOwner)))
  (Utilities|IsValid _asbp_bald_king
    (:Is%20Valid
      (return (Utilities|String|EnumtoString (Variables|/Game/FFBlueprints/NPC/BaldKing/BP_BaldKing.BP_BaldKing_C|GetCurrentAction _asbp_bald_king))))))