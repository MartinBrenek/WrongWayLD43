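; AI setup Blueprint for the Bald King NPC group, choosing NPC behavior from an AI state.
; SetupAI switches on that state to initialize a behavior tree and blackboard for crowd wandering, King, Junkie, Junkie Idle or Whore roles.
; King, Junkie and Whore are flagged as quest roles.
; Junkie Idle defers running its single-task tree, stores the DrugDen point of interest in the blackboard, then calls TryChangeBT.
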(event Custom|SetupAI
  (params (AIState :type StateBaldKing%20Enum :default "NewEnumerator5"))
  (switch Utilities|FlowControl|Switch|SwitchonStateBaldKing AIState
    (:NewEnumerator0
      (CallFunction|Initialize "/Game/FFBlueprints/Crowd/BTCrowd.BTCrowd" "/Game/FFBlueprints/Crowd/BBCrowd.BBCrowd" false true))
    (:NewEnumerator1
      (CallFunction|Initialize "/Game/FFBlueprints/NPC/BaldKing/BT_BaldKing.BT_BaldKing" "/Game/FFBlueprints/NPC/BaldKing/BB_BaldKing.BB_BaldKing" true true))
    (:NewEnumerator2
      (CallFunction|Initialize "/Game/FFBlueprints/NPC/BT_NPCBaseActiveSingleTask.BT_NPCBaseActiveSingleTask" "/Game/FFBlueprints/Crowd/BBCrowd.BBCrowd" false false)
      (bind _point (CallFunction|GetSpecificPoi "DrugDen"))
      (AI|Components|Blackboard|SetValueasObject (AI|GetBlackboard 0) (Utilities|Name|MakeLiteralName "ActualObject") _point)
      (CallFunction|TryChangeBT))
    (:NewEnumerator3
      (CallFunction|Initialize "/Game/FFBlueprints/NPC/BaldKing/BT_JunkieQuest.BT_JunkieQuest" "/Game/FFBlueprints/Crowd/BBCrowd.BBCrowd" true true))
    (:NewEnumerator4
      (CallFunction|Initialize "/Game/FFBlueprints/NPC/BaldKing/Whore/BT_Whore.BT_Whore" "/Game/FFBlueprints/NPC/BaldKing/Whore/BB_Whore.BB_Whore" true true))))

(event EventBeginPlay)

(event EventTick
  (params (DeltaSeconds :type Float%20%28single-precision%29))
  (|CallParentFunction DeltaSeconds) ; This node is disabled and will not be called.\nDrag off pins to build functionality.
)

(fn ConstructionScript
  (|CallParentFunction))