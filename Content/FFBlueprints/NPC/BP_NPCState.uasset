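; Base NPC state machine component that tracks the actual state and changes it through transitions defined in a DataTable.
; On BeginPlay it converts the table into a state-to-transitions map, then fires transition 0 after a short delay; NextState looks up and sets nonzero targets.
; Table-parsing helpers are stubs that print an error, apparently meant for child overrides.
; With DebugState on, Tick shows the state on the owning CrowdCharacter's debug text.
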(event Custom|DebugPrintState
  (Variables|Default|SetWait%20on%20render false)
  (if (Variables|Default|GetDebugState)
    (if (Utilities|IsValid (Variables|Default|GetDebugText))
      (Rendering|Components|TextRender|SetText (Variables|Default|GetDebugText) (Utilities|Text|ToText(String) (CallFunction|GetEnumStatetoText (Variables|Default|GetActualState))) :!label _label)
      (else
        (bind _ascrowd_character (Utilities|Casting|CastToCrowdCharacter (Components|GetOwner)))
        (Utilities|IsValid (Variables|/Game/FFBlueprints/Crowd/CrowdCharacter.CrowdCharacter_C|GetDebugStateText _ascrowd_character)
          (:Is%20Valid
            (Variables|Default|SetDebugText (Variables|/Game/FFBlueprints/Crowd/CrowdCharacter.CrowdCharacter_C|GetDebugStateText _ascrowd_character))
            (goto _label))
          (:Is%20Not%20Valid
            (Default|AddDebugText _ascrowd_character)
            (Variables|Default|SetWait%20on%20render true)))))
    (elif (Utilities|IsValid (Variables|Default|GetDebugText))
      (Components|DestroyComponent (Variables|Default|GetDebugText))
      (Variables|Default|SetDebugText 0))))

(event EventBeginPlay
  (bind _converted (CallFunction|ConvertDataTable))
  (Variables|Default|SetConvertedDataTable _converted)
  (Utilities|FlowControl|Delay 0.2)
  (CallFunction|NextState))

(event EventTick
  (params (DeltaSeconds :type Float%20%28single-precision%29))
  (CallFunction|DebugPrintState))

(fn ConvertDataTable
  (Utilities|IsValid (Variables|Default|GetTransitionDataTable)
    (:Is%20Valid
      (Utilities|FlowControl|Sequence
        (:then_0
          (bind _stringtostate (CallFunction|GetStringtoState))
          (LocalVariables|SetStatefromString _stringtostate))
        (:then_1
          (bind _num (CallFunction|GetNumOfTransition))
          (LocalVariables|SetNumTransition _num))
        (:then_2
          (bind _outrownames (DataTable|GetDataTableRowNames (Variables|Default|GetTransitionDataTable)))
          (for _array_element _outrownames
            (if (.ReturnValue (Utilities|Map|Find (LocalVariables|GetStatefromString) (Utilities|String|ToString(Name) _array_element)))
              (bind _result (CallFunction|GetRowArrayfromTable _array_element (Variables|Default|GetTransitionDataTable) (LocalVariables|GetNumTransition)))
              (Utilities|Map|Add (LocalVariables|GetResult) (.Value (Utilities|Map|Find (LocalVariables|GetStatefromString) (Utilities|String|ToString(Name) _array_element))) (Utilities|Struct|MakeStructArray _result))
              (else
                (Development|PrintString (Utilities|String|Append "Not found pica " (Utilities|String|ToString(Name) _array_element))))))
          (return (LocalVariables|GetResult)))))
    (:Is%20Not%20Valid
      (Development|PrintString "Not Set Data Table" true true "(R=1.000000,G=0.000000,B=0.000000,A=1.000000)" 3e+02))))

(fn NextState
  (params (Transition :type Byte))
  (bind _returnvalue (Math|Conversions|ToInteger(Byte) Transition))
  (bind _converteddatatable (Variables|Default|GetConvertedDataTable))
  (bind _actualstate (Variables|Default|GetActualState))
  (bind _returnvalue_2 (Math|Conversions|ToInteger(Byte) _actualstate))
  (bind _value (Utilities|Map|Find _converteddatatable _returnvalue_2))
  (bind _array (Utilities|Struct|BreakStructArray _value))
  (bind _output (Utilities|Array|Get(acopy) _array _returnvalue))
  (bind _returnvalue_3 (!= _output 0))
  (bind _returnvalue_4 (Math|Conversions|ToByte(Integer) _output))
  (if _returnvalue_3
    (Utilities|FlowControl|Sequence
      (:then_0
        (|PrintResult Transition _returnvalue_4))
      (:then_1
        (CallFunction|SetState _returnvalue_4)
        (return _returnvalue_3 (Variables|Default|GetActualState))))
    (elif (Variables|Default|GetDebugState)
      (Development|PrintString (Utilities|String|Append "Not found state under translaiton: " (Utilities|String|ToString(Byte) Transition)) true true "(R=0.000000,G=0.660000,B=1.000000,A=1.000000)" 5.0))))

(fn GetActualState
  (return (Variables|Default|GetActualState)))

(fn SetState
  (params (State :type Byte))
  (Variables|Default|SetActualState State)
  (CallFunction|DebugPrintState))

(fn GetNumOfTransition
  (Development|PrintString "Pico posral si to" true true "(R=1.000000,G=0.000000,B=0.153147,A=1.000000)" 3e+01)
  (return 0))

(fn GetStringtoState
  (Development|PrintString "Pico posral si to" true true "(R=1.000000,G=0.000000,B=0.153147,A=1.000000)" 3e+01)
  (return 0))

(fn GetRowArrayfromTable
  (params (Row :type Name) (Table :type Data%20Table%20Object%20Reference) (NumTransition :type Integer))
  (Development|PrintString "Pico posral si to" true true "(R=1.000000,G=0.000000,B=0.153147,A=1.000000)" 3e+01)
  (return 0))

(fn GetEnumStatetoText
  (params (EnumByte :type Byte))
  (return (Utilities|String|ToString(Byte) EnumByte)))