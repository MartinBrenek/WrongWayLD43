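; Behavior tree task that sets an object from the NPC's blackboard as its point-of-interest target.
; It reads the actor from the selected object key and writes it to the ActualObject key.
; It also sets MoveToLocation to a point offset from that actor along its forward vector, then finishes successfully.
; If the cast to Actor fails, the task never calls FinishExecute.
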(event EventReceiveExecute
  (params (OwnerActor :type Actor%20Object%20Reference))
  (bind _returnvalue (AI|GetBlackboard OwnerActor))
  (bind _asactor (Utilities|Casting|CastToActor (AI|Components|Blackboard|GetValueasObject (AI|GetBlackboard OwnerActor) (.selectedkeyname (Variables|Default|GetObjectKey)))))
  (AI|Components|Blackboard|SetValueasObject _returnvalue (Variables|Default|GetActualObject) _asactor)
  (AI|Components|Blackboard|SetValueasVector _returnvalue (Variables|Default|GetMoveToLocation) (Math|Vector|MakeVector (.X (Math|Vector|BreakVector (+ (Transformation|GetActorLocation _asactor) (* (Transformation|GetActorForwardVector _asactor) (Variables|Default|GetOffset))))) (.Y (Math|Vector|BreakVector (+ (Transformation|GetActorLocation _asactor) (* (Transformation|GetActorForwardVector _asactor) (Variables|Default|GetOffset))))) (.Z (Math|Vector|BreakVector (+ (Transformation|GetActorLocation _asactor) (* (Transformation|GetActorForwardVector _asactor) (Variables|Default|GetOffset)))))))
  (AI|BehaviorTree|FinishExecute true))