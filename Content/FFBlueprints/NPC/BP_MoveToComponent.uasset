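; Behavior Tree task that moves an NPC to a scene component stored in a selected Blackboard key.
; On execute it caches the owning NPC AI controller, then each tick reads the component's current location and reissues SimpleMoveToLocation toward it.
; It finishes successfully once the pawn's horizontal (XY) distance is within DestionationRadius times ten; failed casts never finish the task.
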(event EventReceiveExecute
  (params (OwnerActor :type Actor%20Object%20Reference))
  (bind _asbp_npcbase_aicontroller (Utilities|Casting|CastToBP_NPCBaseAIController OwnerActor))
  (Variables|Default|SetTarget _asbp_npcbase_aicontroller))

(event EventTick
  (params (OwnerActor :type Actor%20Object%20Reference) (DeltaSeconds :type Float%20%28single-precision%29))
  (bind _asscene_component (Utilities|Casting|CastToSceneComponent (AI|Components|Blackboard|GetValueasObject (AI|GetBlackboard (Variables|Default|GetTarget)) (.SelectedKeyName (Utilities|Struct|BreakBlackboardKeySelector (Variables|Default|GetBlackBoard))))))
  (bind _is (CallFunction|IsinDestination (Transformation|GetWorldLocation _asscene_component)))
  (if _is
    (AI|BehaviorTree|FinishExecute true)
    (else
      (AI|Navigation|SimpleMovetoLocation (Variables|Default|GetTarget) (Transformation|GetWorldLocation _asscene_component)))))

(fn IsinDestination
  (params (TaergetLocation :type Vector))
  (return (<= (Math|Vector|VectorLengthXY (- TaergetLocation (Transformation|GetActorLocation (Pawn|GetControlledPawn (Variables|Default|GetTarget))))) (* (Variables|Default|GetDestionationRadius) 1e+01))))