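; Behavior tree task that injects a dynamic subtree into an NPC's behavior tree, then finishes successfully.
; Set New Task uses a supplied Task or, as when executed here without one, gets it from the ActualObject blackboard POI's info for the controlled CrowdCharacter.
; It sets that tree on the BTDynamicTask tag and records it in CurrentBT, logging if the POI or pawn cast fails.
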(event EventReceiveExecute
  (params (OwnerActor :type Actor%20Object%20Reference))
  (CallFunction|SetNewTask OwnerActor)
  (AI|BehaviorTree|FinishExecute true))

(fn SetNewTask
  (params (actor :type Actor%20Object%20Reference) (task :type Behavior%20Tree%20Object%20Reference))
  (bind _asbp_npcbase_aicontroller (Utilities|Casting|CastToBP_NPCBaseAIController actor))
  (Utilities|IsValid task
    (:Is%20Valid
      (bind _asbehavior_tree_component (Utilities|Casting|CastToBehaviorTreeComponent (Variables|/Script/AIModule.AIController|GetBrainComponent _asbp_npcbase_aicontroller)))
      (Class|BehaviorTreeComponent|SetDynamicSubtree _asbehavior_tree_component "(TagName=\"BTDynamicTask\")" task)
      (AI|Components|Blackboard|SetValueasObject (AI|GetBlackboard _asbp_npcbase_aicontroller) (Variables|Default|GetCurrentBT) task))
    (:Is%20Not%20Valid
      (bind _asbase_poiactor (Utilities|Casting|CastToBasePOIActor (AI|Components|Blackboard|GetValueasObject (AI|GetBlackboard _asbp_npcbase_aicontroller) (Variables|Default|GetActualObject)))
        (:then
          (bind _ascrowd_character (Utilities|Casting|CastToCrowdCharacter (Pawn|GetControlledPawn _asbp_npcbase_aicontroller))
            (:then
              (bind _task (Default|GetNPCInfobyPawn _asbase_poiactor _ascrowd_character))
              (bind _asbehavior_tree_component_2 (Utilities|Casting|CastToBehaviorTreeComponent (Variables|/Script/AIModule.AIController|GetBrainComponent _asbp_npcbase_aicontroller)))
              (Class|BehaviorTreeComponent|SetDynamicSubtree _asbehavior_tree_component_2 "(TagName=\"BTDynamicTask\")" _task)
              (AI|Components|Blackboard|SetValueasObject (AI|GetBlackboard _asbp_npcbase_aicontroller) (Variables|Default|GetCurrentBT) _task))
            (:CastFailed
              (CallFunction|DebugLog "" "NewEnumerator1")
              (return))))
        (:CastFailed
          (CallFunction|DebugLog "" "NewEnumerator1")
          (return))))))