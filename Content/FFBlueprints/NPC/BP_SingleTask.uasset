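; BP_SingleTask is a behavior tree task that runs a one-shot action on a CrowdCharacter NPC controlled by BP_NPCBaseAIController.
; On execute it sets the ActionKey blackboard bool to true and registers itself with the character for an animation-end callback.
; AnimEndCallBack clears the key, unregisters from the character and finishes successfully, so the task's length follows the animation.
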(event EventAnimEndCallBack
  (CallFunction|ExitState (AI|GetBlackboard (stale EventReceiveExecute OwnerActor)))
  (Default|UnregisterAnimEnd (stale EventReceiveExecute _ascrowd_character) (Variables|Default|GetActionKey))
  (AI|BehaviorTree|FinishExecute true))

(event EventReceiveExecute
  (params (OwnerActor :type Actor%20Object%20Reference))
  (bind _asbp_npcbase_aicontroller (Utilities|Casting|CastToBP_NPCBaseAIController OwnerActor))
  (bind _ascrowd_character (Utilities|Casting|CastToCrowdCharacter (Pawn|GetControlledPawn _asbp_npcbase_aicontroller)))
  (CallFunction|EnterState (AI|GetBlackboard OwnerActor))
  (Default|RegisterAnimEnd _ascrowd_character self (Variables|Default|GetActionKey)))

(fn EnterState
  (params (BlackBoard :type Blackboard%20Component%20Object%20Reference))
  (AI|Components|Blackboard|SetValueasBool BlackBoard (.SelectedKeyName (Utilities|Struct|BreakBlackboardKeySelector (Variables|Default|GetActionKey))) true)
  (return))

(fn ExitState
  (params (Blackboard :type Blackboard%20Component%20Object%20Reference))
  (AI|Components|Blackboard|SetValueasBool Blackboard (.SelectedKeyName (Utilities|Struct|BreakBlackboardKeySelector (Variables|Default|GetActionKey))) false))