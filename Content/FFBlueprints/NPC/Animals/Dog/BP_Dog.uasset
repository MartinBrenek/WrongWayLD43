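; Dog NPC that poops beside its kennel and can be plugged with a bottle cap, making it inflate via morph target as it poops.
; At full inflation it asks its green grocer owner for help, freezing if accepted or else exploding into a decal and physics poop projectiles.
; Using a capped dog pops the cap and, if inflated enough, swaps it for BP_FlockDog and starts AirPlane flights.
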(event Custom|StartShiting
  (Development|PrintString "start shitting")
  (if (Utilities|IsValid (Variables|Default|GetAnimator))
    _
    (else
      (bind _asdog_anim (Utilities|Casting|CastToDog_Anim (Components|SkeletalMesh|GetAnimInstance (Variables|Character|GetMesh))))
      (Variables|Default|SetAnimator _asdog_anim)))
  (Variables|/Game/FFBlueprints/NPC/Animals/Dog/Dog_Anim.Dog_Anim_C|SetShit (Variables|Default|GetAnimator) true)
  (Variables|Default|SetPoopInProgress true)
  (Variables|Default|SetStartValue (Variables|Default|GetValue))
  (if (not (Variables|Default|GetCaped))
    (bind _returnvalue (Game|SpawnActorfromClass "/Game/FFBlueprints/FastFoodOutDoor/Shit.Shit_C" (Transformation|GetWorldTransform (Variables|Default|GetArrow1)) "Undefined" 0 false 0))
    (Utilities|Array|Add (Variables|/Game/FFBlueprints/NPC/Animals/Dog/BP_Kennel.BP_Kennel_C|GetShitsOnPlace (Variables|Default|GetKennel)) _returnvalue)))

(event Custom|StopShit
  (Development|PrintString "stop shit")
  (if (not (Variables|Default|GetWaiting))
    (Variables|Default|SetPoopInProgress false)))

(event Custom|UpdateShitProgress
  (params (Progress :type Float%20%28single-precision%29))
  (bind _startvalue (Variables|Default|GetStartValue))
  (bind _returnvalue (Math|Float|Lerp _startvalue 0.0 Progress))
  (if (and (Variables|Default|GetPoopInProgress) (Variables|Default|GetCaped))
    (Variables|Default|SetValue (+ (Variables|Default|GetStartValue) (Math|Float|Lerp 0.0 0.4 Progress)))
    (if (< (Variables|Default|GetValue) 1.0)
      (CallFunction|UpdateInflation (Variables|Default|GetValue))
      (else
        (CallFunction|CallHelp)))
    (else
      (CallFunction|UpdateInflation _returnvalue)
      (Variables|Default|SetValue _returnvalue))))

(event Custom|DogExplosion
  (bind _capsulecomponent (Variables|Default|GetCapsuleComponent))
  (bind _mesh (Variables|Character|GetMesh))
  (bind _returnvalue (Transformation|GetWorldLocation _mesh))
  ;[1 1 1] WARNING ERROR
  (Development|PrintString "Hello")
  (Class|SaveObjectInterface|GetSaveData(Message) _capsulecomponent)
  (Effects|SpawnEmitteratLocation "/Game/assets/particles/PS_dogExplosion.PS_dogExplosion" (Transformation|GetWorldLocation _capsulecomponent))
  (bind (_outhit _returnvalue_2) (Collision|LineTraceByChannel _returnvalue (+ _returnvalue (* (Math|Vector|VectorDown) 1e+03)) "TraceTypeQuery1" false 0 "None"))
  (if _returnvalue_2
    (Rendering|Decal|SpawnDecalatLocation "/Game/assets/stall/base_mats/M_decal_Shit.M_decal_Shit" "16.000000,256.000000,256.000000" (.ImpactPoint (Collision|BreakHitResult _outhit)) "-90.000000,0.000000,0.000000" 0.0)
    (for _index (range 0 50)
      (bind _returnvalue_3 (Game|SpawnActorfromClass "/Game/FFBlueprints/NPC/Animals/Dog/ShitProjectile.ShitProjectile_C" (Math|Transform|MakeTransform (Transformation|GetWorldLocation (Variables|Default|GetCapsuleComponent)) (Math|Rotator|MakeRotfromZ (Math|Random|RandomUnitVectorinConeinDegrees "0, 0,1.000000" 9e+01))) "AlwaysSpawn" 0 0))
      (bind _output_get (Variables|Default|SetTemp (* (Math|Vector|GetUpVector (Variables|/Game/FFBlueprints/NPC/Animals/Dog/ShitProjectile.ShitProjectile_C|GetCollision _returnvalue_3)) 6e+02)))
      (Physics|SetPhysicsLinearVelocity (Variables|/Game/FFBlueprints/NPC/Animals/Dog/ShitProjectile.ShitProjectile_C|GetCollision _returnvalue_3) _output_get false "None")))
  (Actor|DestroyActor))

(event Custom|CallHelp
  (if (not (Variables|Default|GetWaiting))
    (bind _asbp_green_grocer (Utilities|Casting|CastToBP_GreenGrocer (Variables|Default|GetAnimalOwner))
      (:then
        (bind _reactonit (Default|DogCallforHelp _asbp_green_grocer self))
        (if _reactonit
          (Variables|/Game/FFBlueprints/NPC/Animals/Dog/Dog_Anim.Dog_Anim_C|SetFreeze (Variables|Default|GetAnimator) true)
          (Variables|Default|SetWaiting true)
          (else
            (CallFunction|DogExplosion :!label _label))))
      (:CastFailed
        (goto _label)))))

(event EventBeginPlay)

(event Collision|EventActorBeginOverlap
  (params (OtherActor :type Actor%20Object%20Reference)))

(event EventTick
  (params (DeltaSeconds :type Float%20%28single-precision%29)))

(event EventUseItem
  (if (Variables|Default|GetCaped)
    (Variables|Default|SetCaped false)
    (CallFunction|TakeCap)
    (if (> (Variables|Default|GetValue) 0.4)
      (Game|SpawnActorfromClass "/Game/FFBlueprints/NPC/Animals/Dog/BP_FlockDog.BP_FlockDog_C" (Transformation|GetWorldTransform (Variables|Default|GetCapsuleComponent)) "AlwaysSpawn" 0 (Variables|Default|GetValue) 0)
      (bind _outactors (Actor|GetAllActorsOfClass "/Game/FFBlueprints/NPC/Animals/Dog/AirPlane.AirPlane_C"))
      (for _array_element _outactors
        (Default|StarFlight _array_element))
      (Actor|DestroyActor))))

(fn ConstructionScript)

(fn TakeCap
  (bind _bottlecap (Variables|Default|GetBottleCap))
  (Rendering|SetVisibility _bottlecap false true)
  (bind _returnvalue (Game|SpawnActorfromClass "/Game/FFBlueprints/FastFoodOutDoor/BP_BottleCap.BP_BottleCap_C" (Math|Transform|MakeTransform (Transformation|GetWorldLocation _bottlecap)) "Undefined" 0 0))
  (Default|UseItem _returnvalue))

(fn UpdateInflation
  (params (Alpha :type Float%20%28single-precision%29))
  (if (Variables|Default|GetPoopInProgress)
    (Development|PrintString (Utilities|String|Append "Dog inflation" (Utilities|String|ToString(Float) Alpha)) true true "(R=1.000000,G=0.000000,B=0.068848,A=1.000000)" 1e+01)
    (Transformation|SetRelativeLocation (Variables|Default|GetBottleCap) (Math|Vector|Lerp(Vector) "-5.700000,-1.750000,-0.020000" "-12.400000,-2.900000,0.000000" Alpha) false false)
    (Components|SkeletalMesh|SetMorphTarget (Variables|Character|GetMesh) "dog_inflated" Alpha true)))

(fn CombinewithItem
  (params (ItemToCombine :type Actor%20Object%20Reference))
  (Utilities|Casting|CastToBP_BottleCap ItemToCombine)
  (Rendering|SetVisibility (Variables|Default|GetBottleCap) true false)
  (Variables|Default|SetCaped true)
  (return true false false false))

(fn IsReadytoPickUp
  (return false))

(fn IsReadytoUse
  (return (Math|Boolean|ANDBoolean (Variables|Default|GetAnalOpen) (not (Variables|Default|GetPoopInProgress)) (not (Variables|Default|GetCaped)))))