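; BP_Kennel is a kennel actor that spawns animals on behalf of an instigator.
; SpawnAnimal creates the given class at the Scene component's location and rotation with unit scale, always spawning regardless of collision.
; It stores the kennel and the instigator, as owner, on the new animal, sets the static mesh to ignore it when moving, and returns it.
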(event EventBeginPlay)

(event Collision|EventActorBeginOverlap
  (params (OtherActor :type Actor%20Object%20Reference)))

(event EventTick
  (params (DeltaSeconds :type Float%20%28single-precision%29)))

(fn ConstructionScript)

(fn SpawnAnimal
  (params (class :type BP%20Animal%20Class%20Reference) (Instigator :type Crowd%20Character%20Object%20Reference))
  (bind _scene (Variables|Default|GetScene))
  (bind _returnvalue (Transformation|GetWorldTransform _scene))
  (bind (_location _rotation) (Math|Transform|BreakTransform _returnvalue))
  (bind _returnvalue_2 (Game|SpawnActorfromClass class (Math|Transform|MakeTransform _location _rotation) "AlwaysSpawn" 0 Instigator))
  (Variables|/Game/FFBlueprints/NPC/Animals/BP_Animal.BP_Animal_C|SetKennel _returnvalue_2 self)
  (Variables|/Game/FFBlueprints/NPC/Animals/BP_Animal.BP_Animal_C|SetAnimalOwner _returnvalue_2 Instigator)
  (Collision|IgnoreActorwhenMoving (Variables|Default|GetStaticMesh) _returnvalue_2 true)
  (return _returnvalue_2))