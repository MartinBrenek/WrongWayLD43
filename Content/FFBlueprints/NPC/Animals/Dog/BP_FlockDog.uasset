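; Flock dog NPC that crashes an AirPlane it eats as prey, then destroys itself.
; On BeginPlay it sets the "dog_inflated" morph target from Inflation and calls DrawBorder, which draws a long-lived debug box derived from the UnderwaterMin and UnderwaterMax bounds.
; The graph has no movement or flocking logic, and its Tick is empty apart from a disconnected timer fragment.
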(event EventBeginPlay
  (Components|SkeletalMesh|SetMorphTarget (Variables|Default|GetSkeletalMesh) "dog_inflated" (Variables|Default|GetInflation) true)
  (Utilities|DrawBorder))

(event Collision|EventActorBeginOverlap
  (params (OtherActor :type Actor%20Object%20Reference)))

(event EventTick
  (params (DeltaSeconds :type Float%20%28single-precision%29)))

(event EventEatPrey
  (params (Prey :type Actor%20Object%20Reference))
  (bind _asair_plane (Utilities|Casting|CastToAirPlane Prey))
  (Default|Crash _asair_plane)
  (Actor|DestroyActor self))

(fn ConstructionScript)