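; Behavior tree task that turns an NPC to match the arrow component on its point of interest's action object.
; On execute, it reads the POI from the blackboard, captures start and target rotations, and sets RotateLeft and IsRotating.
; Tick lerps along the shortest path by a frame-rate-dependent fixed step, then clears IsRotating and finishes.
; Without an action object or arrow, the lerp still runs on existing rotation values.
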(event EventReceiveExecute
  (params (OwnerActor :type Actor%20Object%20Reference))
  (bind _asbp_npcbase_aicontroller (Utilities|Casting|CastToBP_NPCBaseAIController OwnerActor))
  (bind _asbp_npcpoi (Utilities|Casting|CastToBP_NPCPOI (AI|Components|Blackboard|GetValueasObject (AI|GetBlackboard _asbp_npcbase_aicontroller) (Variables|Default|GetActualObject))))
  (Utilities|IsValid (Variables|/Game/FFBlueprints/NPC/BP_NPCPOI.BP_NPCPOI_C|GetActionObject _asbp_npcpoi)
    (:Is%20Valid
      (Utilities|IsValid (Actor|GetComponentbyClass (Variables|/Game/FFBlueprints/NPC/BP_NPCPOI.BP_NPCPOI_C|GetActionObject _asbp_npcpoi) "/Script/Engine.ArrowComponent")
        (:Is%20Valid
          (bind _output_get (Variables|Default|SetStartRot (Transformation|GetActorRotation (Pawn|GetControlledPawn _asbp_npcbase_aicontroller))))
          (bind _output_get_2 (Variables|Default|SetEndRot (Transformation|GetWorldRotation (Actor|GetComponentbyClass (Variables|/Game/FFBlueprints/NPC/BP_NPCPOI.BP_NPCPOI_C|GetActionObject _asbp_npcpoi) "/Script/Engine.ArrowComponent"))))
          (AI|Components|Blackboard|SetValueasBool (AI|GetBlackboard _asbp_npcbase_aicontroller) (Variables|Default|GetRotateLeft) (> (.Yaw (Math|Rotator|BreakRotator _output_get)) (.Yaw (Math|Rotator|BreakRotator _output_get_2))))
          (AI|Components|Blackboard|SetValueasBool (AI|GetBlackboard _asbp_npcbase_aicontroller) (Variables|Default|GetIsRotating) true)
          (Variables|Default|SetReady true))
        (:Is%20Not%20Valid
          (Variables|Default|SetReady true))))
    (:Is%20Not%20Valid
      (Variables|Default|SetReady true))))

(event EventTick
  (params (OwnerActor :type Actor%20Object%20Reference) (DeltaSeconds :type Float%20%28single-precision%29))
  (if (Variables|Default|GetReady)
    (Transformation|SetActorRotation (Pawn|GetControlledPawn (stale EventReceiveExecute _asbp_npcbase_aicontroller)) (Math|Rotator|Lerp(Rotator) (Variables|Default|GetStartRot) (Variables|Default|GetEndRot) (Variables|Default|GetAlpha) true))
    (if (>= (Variables|Default|GetAlpha) 1.0)
      (Variables|Default|SetAlpha 0.0)
      (Variables|Default|SetReady false)
      (AI|Components|Blackboard|SetValueasBool (AI|GetBlackboard (stale EventReceiveExecute _asbp_npcbase_aicontroller)) (Variables|Default|GetIsRotating) false)
      (AI|BehaviorTree|FinishExecute true)
      (else
        (bind _output_get (Variables|Default|SetAlpha (+ (stale _output_get) 0.04)))))))