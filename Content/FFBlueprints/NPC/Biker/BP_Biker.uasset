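; BP_Biker is a usable NPC for the smoke quest that sends the player into the LSD world.
; It stays hidden until the quest starts; using it locks player turning while a timeline raises and grows the smoke collision.
; Player overlap with the smoke swaps streamed levels, starts the LSD effect with a sandbox-teleport callback and advances the quest state.
; If the smoke misses, the NPC becomes usable again.
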(event OnComponentBeginOverlap(Shoot)
  (params (OverlappedComponent :type Primitive%20Component%20Object%20Reference) (OtherActor :type Actor%20Object%20Reference) (OtherComp :type Primitive%20Component%20Object%20Reference) (OtherBodyIndex :type Integer) (bFromSweep :type Boolean) (SweepResult :type Hit%20Result%20Structure%20%28by%20ref%29))
  (bind _asfirst_person_character (Utilities|Casting|CastToFirstPersonCharacter OtherActor))
  (Variables|Default|SetPlayer _asfirst_person_character)
  (Utilities|FlowControl|Sequence
    (:then_0
      (Game|LoadStreamLevel(byName) "LSDWorld" true)
      (Game|UnloadStreamLevel(byName) "OutLSDSubLevel" false))
    (:then_1
      (Default|StartLSD _asfirst_person_character (delegate Custom|GoToSandBox))
      (Variables|Default|SetSmokeQuestState "NewEnumerator2"))))

(event Custom|GoToSandBox
  (bind _player (Variables|Default|GetPlayer))
  (Default|TeleporttoSandBox _player)
  (Default|LerpSize _player 0.0))

(event EventBeginPlay
  (Rendering|SetActorHiddenInGame true)
  (Variables|Default|SetStartPosParticle (Variables|/Script/Engine.SceneComponent|GetRelativeLocation (Variables|Default|GetShoot))))

(event Collision|EventActorBeginOverlap
  (params (OtherActor :type Actor%20Object%20Reference))
  (|CallParentFunction OtherActor) ; This node is disabled and will not be called.\nDrag off pins to build functionality.
)

(event EventUseItem
  (bind _shoot (Variables|Default|GetShoot))
  (bind _startposparticle (Variables|Default|GetStartPosParticle))
  (bind _particlesystem (Variables|Default|GetParticleSystem))
  (Variables|Default|SetSmokeQuestState "NewEnumerator1")
  (bind _asfirst_person_character (Utilities|Casting|CastToFirstPersonCharacter (Game|Player|GetPlayerPawn 0)))
  (Variables|Default|SetPlayer _asfirst_person_character)
  (Default|TurnInput _asfirst_person_character false)
  (Utilities|RestartParticleShoot)
  (bind _smoketime (Timeline|Smoke PlayFromStart)
    (:Update
      (Transformation|SetRelativeLocation _shoot (Math|Vector|Lerp(Vector) _startposparticle (+ _startposparticle "0, 0,50.000000") _smoketime) true false)
      (Transformation|SetRelativeScale3D _shoot (Math|Vector|Lerp(Vector) "0, 0, 0" "1.000000,1.000000,1.000000" _smoketime)))
    (:Finished
      (Default|TurnInput (Variables|Default|GetPlayer) true)
      (Rendering|SetVisibility _particlesystem false false)
      (Components|Activation|Deactivate _particlesystem)
      (Utilities|FlowControl|Delay 0.2)
      (Utilities|ResetCollision)
      (if (Utilities|Enum|Equal(Enum) (Variables|Default|GetSmokeQuestState) "NewEnumerator1")
        (Variables|Default|SetSmokeQuestState "NewEnumerator0")))))

(event EventCAlltoStartQuest
  (params (QuestType :type Ingredients%20Enum :default "NewEnumerator9"))
  (Variables|Default|SetSmokeQuestState "NewEnumerator0")
  (Rendering|SetActorHiddenInGame false))

(fn ConstructionScript
  (|CallParentFunction))

(fn CombinewithItem
  (params (ItemToCombine :type Actor%20Object%20Reference))
  (return false false false false))

(fn IsReadytoUse
  (return (Utilities|Enum|Equal(Enum) (Variables|Default|GetSmokeQuestState) "NewEnumerator0")))