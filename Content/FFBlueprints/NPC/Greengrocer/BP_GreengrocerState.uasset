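; BP_GreengrocerState is the Greengrocer NPC's state component, specializing a parent state machine with the Greengrocer's state and transition enums.
; Typed wrappers convert the parent's next-state and current-state results to StateGreengrocer, while SetStateGreengrocer is an empty stub.
; Helper functions count transitions, map state names to integers, and turn DataTable rows into transition-indexed arrays of next states.
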(event EventBeginPlay
  (|CallParentFunction))

(event EventTick
  (params (DeltaSeconds :type Float%20%28single-precision%29)))

(fn NextStateGreengrocer
  (params (Transition :type TransitionGreengrocer%20Enum :default "NewEnumerator0"))
  (bind (_nextstatefound _newstate) (CallFunction|NextState Transition))
  (return _nextstatefound (Utilities|Enum|ByteToEnumStateGreengrocer _newstate)))

(fn GetActualStateGreengrocer
  (bind _state (CallFunction|GetActualState))
  (return (Utilities|Enum|ByteToEnumStateGreengrocer _state)))

(fn SetStateGreengrocer)

(fn GetNumOfTransition
  (|ForEachTransitionGreengrocer
    (:LoopBody
      (Math|Integer|IncrementInt (LocalVariables|GetNumOfTransition)))
    (:then
      (return (LocalVariables|GetNumOfTransition)))))

(fn GetStringtoState
  (bind _enumvalue (|ForEachStateGreengrocer)
    (:LoopBody
      (Utilities|Map|Add (LocalVariables|GetStates) (Utilities|String|EnumtoString _enumvalue) (Math|Conversions|ToInteger(Byte) _enumvalue)))
    (:then
      (return (LocalVariables|GetStates)))))

(fn GetRowArrayfromTable
  (params (Row :type Name :default "None") (Table :type Data%20Table%20Object%20Reference) (NumTransition :type Integer))
  (bind _returnvalue (Utilities|GetDataTableRow Table Row)
    (:then
      (Utilities|FlowControl|Sequence
        (:then_0
          (Utilities|Array|SetArrayElem (LocalVariables|GetTempArray) (- NumTransition 1) 0 true))
        (:then_1
          (bind _output_get (LocalVariables|SetTempRow _returnvalue))
          (for _array_element (Utilities|Struct|BreakTableTransitionStructGreengrocer _output_get)
            (Utilities|Array|SetArrayElem (LocalVariables|GetTempArray) (Math|Conversions|ToInteger(Byte) (.Transition (Utilities|Struct|BreakTransPairGreengrocer _array_element))) (Math|Conversions|ToInteger(Byte) (.State (Utilities|Struct|BreakTransPairGreengrocer _array_element))) true))
          (return (LocalVariables|GetTempArray)))))))

(fn GetEnumStatetoText
  (params (EnumByte :type Byte :default 0))
  (return (Utilities|String|EnumtoString (Utilities|Enum|ByteToEnumStateGreengrocer EnumByte))))