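; Behavior Tree task for the dog walker NPC that searches for a target actor, by its name dog droppings, through an EQS query.
; It runs the query in single-result mode, optionally clearing the result blackboard key right after starting it.
; When the query finishes, it stores the found actor in that key and succeeds, or fails if none is found.
; An XY-distance IsInDestination helper is defined but not called here.
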(event Custom|OnFinished
  (params (QueryInstance :type Env%20Query%20Instance%20Blueprint%20Wrapper%20Object%20Reference) (QueryStatus :type EEnvQueryStatus%20Enum :default "Processing"))
  (bind (_resultactors _returnvalue) (AI|EQS|GetQueryResultsasActors QueryInstance))
  (if _returnvalue
    (AI|Components|Blackboard|SetValueasObject (AI|GetBlackboard (stale EventReceiveExecute OwnerActor)) (.SelectedKeyName (Utilities|Struct|BreakBlackboardKeySelector (Variables|Default|GetResult))) (Utilities|Array|Get(acopy) _resultactors))
    (AI|BehaviorTree|FinishExecute true)
    (else
      (AI|BehaviorTree|FinishExecute false))))

(event EventReceiveExecute
  (params (OwnerActor :type Actor%20Object%20Reference))
  (bind _returnvalue (AI|EQS|RunEQSQuery (Variables|Default|GetQueryTemplate) OwnerActor "SingleResult"))
  (EventDispatchers|BindEventtoOnQueryFinishedEvent _returnvalue (delegate Custom|OnFinished))
  (if (Variables|Default|GetClearProperty)
    (AI|Components|Blackboard|SetValueasObject (AI|GetBlackboard OwnerActor) (.SelectedKeyName (Utilities|Struct|BreakBlackboardKeySelector (Variables|Default|GetResult))) 0)))

(fn IsinDestination
  (params (TaergetLocation :type Vector))
  (return (<= (Math|Vector|VectorLengthXY (- TaergetLocation (Transformation|GetActorLocation (Pawn|GetControlledPawn (Variables|Default|GetTarget))))) (* (Variables|Default|GetDestionationRadius) 1e+01))))