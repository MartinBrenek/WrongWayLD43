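; Fishing rod item among the Greengrocer NPC's items, which starts with a magnet as its hook and swaps it for a visible hook when combined with a Hook item.
; Catch spawns a fish or coin on the magnet, depending on magnetic fishes, or always a fish on the hook, attached with physics off for GetCatched.
; UpdateHook moves the magnet with a debug line, and ResetHookPosition restores its starting transform.
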(event Custom|UpdateHook
  (params (Location :type Vector) (Rotation :type Rotator))
  (bind _magnet (Variables|Default|GetMagnet))
  (Transformation|SetWorldLocation _magnet Location false true)
  (Transformation|SetWorldRotation _magnet Rotation false false)
  (Rendering|Debug|DrawDebugLine Location (Transformation|GetActorLocation) "(R=1.000000,G=0.000000,B=0.452663,A=1.000000)" 6.0 1.0))

(event EventBeginPlay
  (|CallParentFunction)
  (Variables|Default|SetDefaultPosition (Transformation|GetRelativeTransform (Variables|Default|GetMagnet))))

(event Collision|EventActorBeginOverlap
  (params (OtherActor :type Actor%20Object%20Reference))
  (|CallParentFunction OtherActor) ; This node is disabled and will not be called.\nDrag off pins to build functionality.
)

(event EventTick
  (params (DeltaSeconds :type Float%20%28single-precision%29))
  (|CallParentFunction DeltaSeconds) ; This node is disabled and will not be called.\nDrag off pins to build functionality.
)

(fn ConstructionScript
  (|CallParentFunction))

(fn CombinewithItem
  (params (ItemToCombine :type Actor%20Object%20Reference))
  (Utilities|Casting|CastToHook ItemToCombine
    (:then
      (Rendering|SetVisibility (Variables|Default|GetHook) true false)
      (Rendering|SetVisibility (Variables|Default|GetMagnet) false false)
      (Variables|Default|SetMagnetAsHook false)
      (return true false false false))
    (:CastFailed
      (return false false false false))))

(fn IsReadytoUse
  (return (Variables|Default|GetReady)))

(fn Catch
  (params (MagneticFishes :type Boolean))
  (if (Variables|Default|GetMagnetAsHook)
    (if MagneticFishes
      (CallFunction|SpawnonHook (Variables|Default|GetMagnetedFish) "/Game/FFBlueprints/Ingredients/Fish.Fish_C" true)
      (else
        (CallFunction|SpawnonHook (Variables|Default|GetMagnetedFish) "/Game/FFBlueprints/NPC/Greengrocer/GreengrocerItems/BP_Coin.BP_Coin_C" false)))
    (else
      (CallFunction|SpawnonHook (Variables|Default|GetHookedFish) "/Game/FFBlueprints/Ingredients/Fish.Fish_C" true))))

(fn SpawnonHook
  (params (Parent :type Scene%20Component%20Object%20Reference) (Spawn :type Pickable%20Item%20Class%20Reference) (IsItFish :type Boolean))
  (Variables|Default|SetCatchedFish IsItFish)
  (bind _returnvalue (Game|SpawnActorfromClass Spawn (Math|Transform|MakeTransform "0, 0, 0") "AlwaysSpawn" 0 0))
  (Transformation|AttachComponentToComponent _returnvalue Parent "None" "SnapToTarget" "SnapToTarget" "KeepRelative" true)
  (bind _output_get (Variables|Default|SetCathedObject _returnvalue))
  (Physics|SetSimulatePhysics (Variables|/Game/FFBlueprints/PickableItem.PickableItem_C|GetCube _output_get) false))

(fn ResetHookPosition
  (Transformation|SetRelativeTransform (Variables|Default|GetMagnet) (Variables|Default|GetDefaultPosition) false true))

(fn SetReadytoCombine
  (params (Ready :type Boolean))
  (Variables|Default|SetReady Ready))

(fn GetCatched
  (params (ClearCatched :type Boolean))
  (LocalVariables|SetCatched (Variables|Default|GetCathedObject))
  (if ClearCatched
    (Variables|Default|SetCathedObject 0))
  (return (Variables|Default|GetCatchedFish) (LocalVariables|GetCatched)))