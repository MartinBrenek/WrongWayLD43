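; BP_NPCGreenGrocerAI is the AI Blueprint for the Greengrocer NPC, layered on parent logic that it mostly inherits.
; On BeginPlay it runs the parent logic, then copies InstantStartTransition into the blackboard bool named by InstantStartVar.
; InitBlackboard and the construction script only forward to the parent, and Tick is disabled.
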(event EventBeginPlay
  (|CallParentFunction)
  (AI|Components|Blackboard|SetValueasBool (AI|GetBlackboard self) (Variables|Default|GetInstantStartVar) (Variables|Default|GetInstantStartTransition)))

(event EventTick
  (params (DeltaSeconds :type Float%20%28single-precision%29))
  (|CallParentFunction DeltaSeconds) ; This node is disabled and will not be called.\nDrag off pins to build functionality.
)

(fn ConstructionScript
  (|CallParentFunction))

(fn InitBlackboard
  (bind _success (|CallParentFunction))
  (return _success))