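; BP_Offer is a behavior tree task that makes the greengrocer NPC perform its offering action.
; On execute it sets the OfferKey blackboard bool to true, then casts the AI controller's pawn to BP_GreenGrocer, stores it and calls Offering.
; Tick polls the greengrocer's OfferingRunning flag and finishes the task successfully once it is false.
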(event EventReceiveExecute
  (params (OwnerActor :type Actor%20Object%20Reference))
  (bind _asbp_npcbase_aicontroller (Utilities|Casting|CastToBP_NPCBaseAIController OwnerActor))
  (if (not (ScalableFloat|GetValueasBool (AI|GetBlackboard _asbp_npcbase_aicontroller) (Variables|Default|GetOfferKey)))
    (AI|Components|Blackboard|SetValueasBool (AI|GetBlackboard _asbp_npcbase_aicontroller) (Variables|Default|GetOfferKey) true))
  (bind _asbp_green_grocer (Utilities|Casting|CastToBP_GreenGrocer (Pawn|GetControlledPawn _asbp_npcbase_aicontroller)))
  (bind _output_get (Variables|Default|SetGreenGrocer _asbp_green_grocer))
  (Default|Offering _output_get))

(event EventTick
  (params (OwnerActor :type Actor%20Object%20Reference) (DeltaSeconds :type Float%20%28single-precision%29))
  (if (not (Variables|/Game/FFBlueprints/NPC/Greengrocer/BP_GreenGrocer.BP_GreenGrocer_C|GetOfferingRunning (Variables|Default|GetGreenGrocer)))
    (AI|BehaviorTree|FinishExecute true)))