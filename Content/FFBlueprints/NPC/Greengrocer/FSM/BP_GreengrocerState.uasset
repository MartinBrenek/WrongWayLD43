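; Greengrocer-specific state class for the NPC finite state machine, specializing a generic parent with the greengrocer state enum.
; SetState runs the parent logic, then notifies the new greengrocer state, while typed wrappers convert to and from that enum.
; Overrides map state names to values, flatten data table rows into transition-indexed next-state arrays, and expose state and owner action as text.
; NextStateGreengrocer is a deprecated stub that prints a warning pointing to NextState.
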(event EventBeginPlay
  (|CallParentFunction))

(event EventTick
  (params (DeltaSeconds :type Float%20%28single-precision%29)))

(event EventSetState
  (params (State :type Byte :default 0))
  (|CallParentFunction State)
  (Default|CallNewStateGreenGrocer (Utilities|Enum|ByteToEnumStateGreengrocer State)))

(fn NextStateGreengrocer
  (params (Transition :type TransitionGreengrocer%20Enum :default "NewEnumerator0"))
  (Development|PrintString "Called Old Next State Greengrocer (use only NextState)" true true "(R=1.000000,G=0.000000,B=0.000000,A=1.000000)" 6e+01)
  (return false "NewEnumerator5"))

(fn GetActualStateGreengrocer
  (bind _state (CallFunction|GetActualState))
  (return (Utilities|Enum|ByteToEnumStateGreengrocer _state)))

(fn SetStateGreengrocer
  (params (State :type StateGreengrocer%20Enum :default "NewEnumerator5"))
  (CallFunction|SetState State))

(fn GetStringtoState
  (bind _enumvalue (|ForEachStateGreengrocer)
    (:LoopBody
      (Utilities|Map|Add (LocalVariables|GetStates) (Utilities|String|EnumtoString _enumvalue) (Math|Conversions|ToInteger(Byte) _enumvalue)))
    (:then
      (return (LocalVariables|GetStates)))))

(fn GetRowArrayfromTable
  (params (Row :type Name :default "None") (Table :type Data%20Table%20Object%20Reference) (NumTransition :type Integer))
  (bind _returnvalue (Utilities|GetDataTableRow Table Row)
    (:then
      (Utilities|FlowControl|Sequence
        (:then_0
          (Utilities|Array|SetArrayElem (LocalVariables|GetTempArray) (- NumTransition 1) 0 true))
        (:then_1
          (bind _output_get (LocalVariables|SetTempRow _returnvalue))
          (for _array_element (Utilities|Struct|BreakTableTransitionStructGreengrocer _output_get)
            (Utilities|Array|SetArrayElem (LocalVariables|GetTempArray) (Math|Conversions|ToInteger(Byte) (.Transition (Utilities|Struct|BreakTransPairGreengrocer _array_element))) (Math|Conversions|ToInteger(Byte) (.State (Utilities|Struct|BreakTransPairGreengrocer _array_element))) true))
          (return (LocalVariables|GetTempArray)))))))

(fn GetEnumStatetoText
  (params (EnumByte :type Byte :default 0))
  (return (Utilities|String|EnumtoString (Utilities|Enum|ByteToEnumStateGreengrocer EnumByte))))

(fn GetEnumActiontoText
  (bind _asbp_green_grocer (Utilities|Casting|CastToBP_GreenGrocer (Variables|Default|GetOwner)))
  (Utilities|IsValid _asbp_green_grocer
    (:Is%20Valid
      (return (Utilities|String|EnumtoString (Variables|/Game/FFBlueprints/NPC/Greengrocer/BP_GreenGrocer.BP_GreenGrocer_C|GetCurrentAction _asbp_green_grocer))))))