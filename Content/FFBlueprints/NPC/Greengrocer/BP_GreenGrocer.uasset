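; Babushka quest NPC that works as a greengrocer, fisherman or dog walker, tracked by a saveable state component.
; Each quest starts its own behavior tree on a shared blackboard, with StartTask triggering animation flags and End events updating task states.
; The player can steal vegetables during slow time, buy with a rotten vegetable or swap the fishing magnet for a hook.
; Casts move the magnet along a spline, while dog problems queue through blackboard keys.
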(event EventBeginPlay
  (|CallParentFunction))

(event Collision|EventActorBeginOverlap
  (params (OtherActor :type Actor%20Object%20Reference))
  (|CallParentFunction OtherActor) ; This node is disabled and will not be called.\nDrag off pins to build functionality.
)

(event EventTick
  (params (DeltaSeconds :type Float%20%28single-precision%29))
  (|CallParentFunction DeltaSeconds) ; This node is disabled and will not be called.\nDrag off pins to build functionality.
)

(event EventUseItem
  (bind _ready (CallFunction|IsReadytoUse))
  (if _ready
    (bind _asfirst_person_character (Utilities|Casting|CastToFirstPersonCharacter (Game|GetPlayerCharacter 0)))
    (switch int 0
      (:0
        (if (Variables|/Game/FirstPersonBP/Blueprints/FirstPersonCharacter.FirstPersonCharacter_C|GetSlowTime _asfirst_person_character)
          (CallFunction|StolenVeg)
          (else
            (CallFunction|FuckOffGreenGroccer)))))))

(event EventCalltoEndQuest
  (if (not (Variables|Default|GetPauseEndQuest))
    (switch Utilities|FlowControl|Switch|SwitchonStateGreengrocer (Default|GetActualStateGreengrocer (Variables|Default|GetBP_GreengrocerState))
      (:NewEnumerator1
        (CallFunction|EndGreenGrocerQuest))
      (:NewEnumerator2
        (CallFunction|EndFishingQuest)))))

(event EventCAlltoStartQuest
  (params (QuestType :type Ingredients%20Enum :default "NewEnumerator9"))
  (bind _bp_greengrocerstate (Variables|Default|GetBP_GreengrocerState))
  (switch Utilities|FlowControl|Switch|SwitchonIngredients QuestType
    (:NewEnumerator2
      (Default|NextStateGreengrocer _bp_greengrocerstate "NewEnumerator2")
      (CallFunction|StartGreenGrocerQuest))
    (:NewEnumerator3
      (Default|NextStateGreengrocer _bp_greengrocerstate "NewEnumerator4")
      (CallFunction|StartFishermanQuest))
    (:NewEnumerator10
      (Default|NextStateGreengrocer _bp_greengrocerstate "NewEnumerator3")
      (CallFunction|StartDogWalkerQuest))))

(event EventStartTask
  (params (TaskID :type Name :default "None"))
  (switch name TaskID
    (:Fishing
      (CallFunction|StartFishing))
    (:Feed
      (CallFunction|StartFeeding))
    (:BuyFeed
      (CallFunction|StartInteraction))
    (:PickUpShit
      (CallFunction|PickUpShit))
    (:DropShit
      (CallFunction|DropShit))
    (:CallDog
      (CallFunction|CallDog))
    (:HelpDog
      (CallFunction|HelpDog)))
  (CallFunction|SetTaskinList TaskID "NewEnumerator0"))

(event EventLoadedData
  (params (Data :type Save%20Object%20Data%20Structure))
  (Default|SetState (Variables|Default|GetBP_GreengrocerState) (.State (Utilities|Struct|BreakSaveObjectData Data))))

(event Custom|Offering
  (bind _animator (Variables|Default|GetAnimator))
  ;[1 1 1] GreenGrocer
  (Variables|Default|SetPauseUse false)
  (Utilities|GetandCheckAnimator
    (:Is%20Valid
      (Rendering|SetVisibility (Variables|Default|GetVegetable) true false)
      (Variables|Default|SetOfferingRunning true)
      (Variables|/Game/FFBlueprints/NPC/Greengrocer/Babushka_AnimBlueprint.Babushka_AnimBlueprint_C|SetUseBabushkaCustom _animator 1.0)
      (Variables|/Game/FFBlueprints/NPC/Greengrocer/Babushka_AnimBlueprint.Babushka_AnimBlueprint_C|SetOffering _animator true)
      (Utilities|FlowControl|Delay 1e+01)
      (Variables|/Game/FFBlueprints/NPC/Greengrocer/Babushka_AnimBlueprint.Babushka_AnimBlueprint_C|SetOffering (Variables|Default|GetAnimator) false)
      (Variables|Default|SetPauseUse true))))

(event Custom|HideVeg
  ;[1 1 1] GreenGrocer
  (Rendering|SetVisibility (Variables|Default|GetVegetable) false false)
  (Variables|/Game/FFBlueprints/NPC/Greengrocer/Babushka_AnimBlueprint.Babushka_AnimBlueprint_C|SetUseBabushkaCustom (Variables|Default|GetAnimator) 0.0)
  (Variables|Default|SetOfferingRunning false))

(event Custom|EndGreenGrocerQuest
  (bind _animator (Variables|Default|GetAnimator))
  ;[1 1 1] GreenGrocer
  (Variables|Default|SetOfferingRunning false)
  (Rendering|SetVisibility (Variables|Default|GetVegetable) false false)
  (Utilities|IsValid _animator
    (:Is%20Valid
      (Variables|/Game/FFBlueprints/NPC/Greengrocer/Babushka_AnimBlueprint.Babushka_AnimBlueprint_C|SetUseBabushkaCustom _animator 0.0))
    (:Is%20Not%20Valid
      _))
  (bind _asbp_npcbase_aicontroller (Utilities|Casting|CastToBP_NPCBaseAIController (Pawn|GetController)))
  (bind _point (Default|GetSpecificPoi _asbp_npcbase_aicontroller "Chill"))
  (AI|Components|Blackboard|SetValueasObject (AI|GetBlackboard 0) (Utilities|Name|MakeLiteralName "ActualObject") _point)
  (Default|SetCurrentBT _asbp_npcbase_aicontroller (Variables|Default|GetBT_IdleAfterGG))
  (CallFunction|EndQuest 1))

(event Custom|FuckOffGreenGroccer
  (bind _quote (Variables|Default|GetQuote))
  ;[1 1 1] GreenGrocer
  (Rendering|SetVisibility _quote true false)
  (Rendering|Components|TextRender|SetText _quote (Utilities|Text|MakeLiteralText "Pay or die."))
  (Variables|/Game/FFBlueprints/NPC/Greengrocer/Babushka_AnimBlueprint.Babushka_AnimBlueprint_C|SetFuckOff (Variables|Default|GetAnimator) true)
  (Variables|Default|SetPauseUse true))

(event Custom|FuckOffEnd
  ;[1 1 1] GreenGrocer
  (Variables|/Game/FFBlueprints/NPC/Greengrocer/Babushka_AnimBlueprint.Babushka_AnimBlueprint_C|SetFuckOff (Variables|Default|GetAnimator) false)
  (if (Utilities|Enum|NotEqual(Enum) (Default|GetActualStateGreengrocer (Variables|Default|GetBP_GreengrocerState)) "NewEnumerator1")
    (CallFunction|FuckOffEndFisherman)
    (else
      (Rendering|SetVisibility (Variables|Default|GetQuote) false false)
      (Variables|Default|SetPauseUse false))))

(event Custom|StolenEnd
  (bind _animator (Variables|Default|GetAnimator))
  ;[1 1 1] GreenGrocer
  (if (Utilities|Enum|NotEqual(Enum) (Default|GetActualStateGreengrocer (Variables|Default|GetBP_GreengrocerState)) "NewEnumerator1")
    (CallFunction|EndFear)
    (else
      (Variables|/Game/FFBlueprints/NPC/Greengrocer/Babushka_AnimBlueprint.Babushka_AnimBlueprint_C|SetOffering _animator false)
      (Variables|/Game/FFBlueprints/NPC/Greengrocer/Babushka_AnimBlueprint.Babushka_AnimBlueprint_C|SetStolen _animator false)
      (CallFunction|EndGreenGrocerQuest))))

(event Custom|StolenVeg
  ;[1 1 1] GreenGrocer
  (Variables|Default|SetPauseEndQuest true)
  (CallFunction|SpawnRealVegetable)
  (Variables|/Game/FFBlueprints/NPC/Greengrocer/Babushka_AnimBlueprint.Babushka_AnimBlueprint_C|SetStolen (Variables|Default|GetAnimator) true))

(event Custom|BoughtVeg
  ;[1 1 1] GreenGrocer
  (Variables|Default|SetPauseEndQuest true)
  (CallFunction|SpawnRealVegetable)
  (Variables|/Game/FFBlueprints/NPC/Greengrocer/Babushka_AnimBlueprint.Babushka_AnimBlueprint_C|SetSold (Variables|Default|GetAnimator) true))

(event Custom|BoughtVegEnd
  (bind _animator (Variables|Default|GetAnimator))
  ;[1 1 1] GreenGrocer
  (Variables|/Game/FFBlueprints/NPC/Greengrocer/Babushka_AnimBlueprint.Babushka_AnimBlueprint_C|SetOffering _animator false)
  (Variables|/Game/FFBlueprints/NPC/Greengrocer/Babushka_AnimBlueprint.Babushka_AnimBlueprint_C|SetSold _animator false)
  (CallFunction|EndGreenGrocerQuest))

(event Custom|StartGreenGrocerQuest
  ;[1 1 1] GreenGrocer
  (bind _asbp_npcbase_aicontroller (Utilities|Casting|CastToBP_NPCBaseAIController (Pawn|GetController)))
  (Default|Initialize _asbp_npcbase_aicontroller (Variables|Default|GetGreenGrocerQuest) "/Game/FFBlueprints/NPC/Greengrocer/BB_GreenGrocer.BB_GreenGrocer" true false))

(event Custom|StartFishermanQuest
  ;[1 1 1] Satart/End Quest
  (bind _asbp_npcbase_aicontroller (Utilities|Casting|CastToBP_NPCBaseAIController (Pawn|GetController)))
  (Default|Initialize _asbp_npcbase_aicontroller (Variables|Fisherman|GetFishermanBT) "/Game/FFBlueprints/NPC/Greengrocer/BB_GreenGrocer.BB_GreenGrocer" true false))

(event Custom|StartFishing
  ;[1 1 1] Animation Start/End
  (bind _animator (Utilities|GetandCheckAnimator)
    (:Is%20Valid
      (Variables|/Game/FFBlueprints/NPC/Greengrocer/Babushka_AnimBlueprint.Babushka_AnimBlueprint_C|SetUseBabushkaCustom _animator 1.0)
      (CallFunction|ShowRodandMagnet true)
      (Variables|/Game/FFBlueprints/NPC/Greengrocer/Babushka_AnimBlueprint.Babushka_AnimBlueprint_C|SetFishing _animator true)
      (Variables|/Game/FFBlueprints/NPC/Greengrocer/Babushka_AnimBlueprint.Babushka_AnimBlueprint_C|SetThrow _animator true)
      (Variables|Default|SetlastUpdate 0.0)
      (Utilities|FlowControl|Delay 1e+01)
      (Variables|/Game/FFBlueprints/NPC/Greengrocer/Babushka_AnimBlueprint.Babushka_AnimBlueprint_C|SetFishing (Variables|Default|GetAnimator) false)
      (CallFunction|Catch))))

(event Custom|SetMagnet
  (params (position :type Integer))
  (bind _magnetroot (Variables|Default|GetMagnetRoot))
  (bind _magnetroot_2 (Variables|Default|GetMagnetRoot))
  ;[1 1 1] VisualHelp
  (switch int position
    (:0
      (Transformation|AttachComponentToComponent _magnetroot (Variables|Character|GetMesh) "spine1" "KeepRelative" "KeepRelative" "KeepRelative" false)
      (Transformation|SetRelativeLocationAndRotation _magnetroot "-5.300000,-23.200001,-26.540001" "77.699997,-156.000000,59.799999" false true))
    (:1
      (Transformation|AttachComponentToComponent (Variables|Default|GetCapsuleComponent) _magnetroot_2 "" "KeepRelative" "KeepRelative" "KeepRelative" false))
    (:2
      (Transformation|AttachComponentToComponent _magnetroot_2 (Variables|Character|GetMesh) "LH_socket" "KeepRelative" "KeepRelative" "KeepRelative" false)
      (Transformation|SetRelativeLocationAndRotation _magnetroot_2 "-11.800000,9.600000,-2.600000" "77.699997,-156.600006,-94.839996" false true))))

(event Custom|ThrowUpdate
  (params (ThrowData :type Float%20%28single-precision%29))
  (bind _spline (Variables|Default|GetSpline))
  (bind _magnetroot (Variables|Default|GetMagnetRoot))
  (Variables|Default|SetlastUpdate (Math|Float|Lerp (Variables|Default|GetlastUpdate) ThrowData 0.1))
  (if (> ThrowData (Spline|GetSplineLength _spline))
    (Transformation|SetWorldLocation _magnetroot (Math|Vector|Lerp(Vector) (Transformation|GetWorldLocation (Variables|Default|GetCable)) (Transformation|GetWorldLocation _magnetroot) 0.01) false true)
    (else
      (Transformation|SetWorldTransform _magnetroot (Math|Transform|MakeTransform (Spline|GetLocationatDistanceAlongSpline _spline (Variables|Default|GetlastUpdate) "World") (Spline|GetRotationatDistanceAlongSpline _spline (Variables|Default|GetlastUpdate) "World")) false false))))

(event Custom|SwitchHook
  ;[1 1 1] VisualHelp
  (Rendering|SetVisibility (Variables|Default|GetMagnet) false false)
  (Rendering|SetVisibility (Variables|Default|GetHook) true false)
  (Variables|Fisherman|SetIsMagnet false))

(event Custom|Catch
  ;[1 1 1] Action
  (if (Variables|Fisherman|GetIsMagnet)
    (if (Variables|Fisherman|GetMangenticFishes)
      (Rendering|SetVisibility (Variables|Default|GetFish) true true)
      (else
        (Rendering|SetVisibility (Variables|Default|GetCoin) true true)))
    (else
      (Rendering|SetVisibility (Variables|Default|GetFishHook) true true))))

(event Custom|UseVendingMachine
  ;[1 1 1] Action
  (Utilities|IsValid (Variables|Fisherman|GetVendingmachine)
    (:Is%20Valid
      (Variables|Fisherman|SetMangenticFishes (Variables|/Game/FFBlueprints/FastFoodOutDoor/FishFoodVendingMachine.FishFoodVendingMachine_C|GetIsMetal (Variables|Fisherman|GetVendingmachine)) :!label _label))
    (:Is%20Not%20Valid
      (bind _asfast_food_game_state (Utilities|Casting|CastToFastFoodGameState (Game|GetGameState)))
      (bind (_value _found) (Default|GetActorReference (Variables|/Game/FFBlueprints/GameMode/FastFoodGameState.FastFoodGameState_C|GetQuestManager _asfast_food_game_state) "VendingMachine"))
      (if _found
        (bind _asfish_food_vending_machine (Utilities|Casting|CastToFishFoodVendingMachine _value))
        (Variables|Fisherman|SetVendingmachine _asfish_food_vending_machine)
        (goto _label)))))

(event Custom|EndFishingQuest
  ;[1 1 1] Satart/End Quest
  (bind _asbp_npcbase_aicontroller (Utilities|Casting|CastToBP_NPCBaseAIController (Pawn|GetController)))
  (bind _point (Default|GetSpecificPoi _asbp_npcbase_aicontroller "Chill"))
  (AI|Components|Blackboard|SetValueasObject (AI|GetBlackboard 0) (Utilities|Name|MakeLiteralName "ActualObject") _point)
  (Default|SetCurrentBT _asbp_npcbase_aicontroller (Variables|Default|GetBT_IdleAfterGG))
  (Variables|/Game/FFBlueprints/NPC/Greengrocer/Babushka_AnimBlueprint.Babushka_AnimBlueprint_C|SetUseBabushkaCustom (Variables|Default|GetAnimator) 0.0)
  (CallFunction|ShowRodandMagnet false)
  (CallFunction|EndQuest 3))

(event Custom|ShowRodAndMagnet
  (params (Show :type Boolean))
  ;[1 1 1] VisualHelp
  (if Show
    (CallFunction|SetRod true)
    (CallFunction|SetMagnet 1)
    (if (not (Variables|Fisherman|GetFishingQuest))
      (Rendering|SetVisibility (Variables|Default|GetMagnet) true false)
      (Rendering|SetVisibility (Variables|Default|GetRot) true false)
      (Rendering|SetVisibility (Variables|Default|GetMagnetRoot) true false)
      (Variables|Fisherman|SetFishingQuest true))
    (else
      (Rendering|SetVisibility (Variables|Default|GetRot) false true)
      (Rendering|SetVisibility (Variables|Default|GetMagnetRoot) false true)
      (Variables|Fisherman|SetFishingQuest false))))

(event Custom|EndFear
  ;[1 1 1] Animation Start/End
  (Variables|/Game/FFBlueprints/NPC/Greengrocer/Babushka_AnimBlueprint.Babushka_AnimBlueprint_C|SetFear (Variables|Default|GetAnimator) false)
  (if (Utilities|Enum|Equal(Enum) (CallFunction|GetTaskState (Variables|DogWalker|GetHelpDogName)) "NewEnumerator0")
    (CallFunction|HelpDogEnd)
    (else
      (CallFunction|SetTaskinList "Fishing" "NewEnumerator2")
      (Game|SpawnActorfromClass "/Game/FFBlueprints/Ingredients/Fish.Fish_C" (Math|Transform|MakeTransform (Transformation|GetWorldLocation (Variables|Default|GetMagnetRoot))) "Undefined" 0 0)
      (CallFunction|EndFishingQuest))))

(event Custom|EndFishing
  (bind _animator (Variables|Default|GetAnimator))
  ;[1 1 1] Animation Start/End
  (bind _animator_2 (Utilities|GetandCheckAnimator)
    (:Is%20Valid
      (Variables|/Game/FFBlueprints/NPC/Greengrocer/Babushka_AnimBlueprint.Babushka_AnimBlueprint_C|SetThrow _animator_2 false)
      (CallFunction|SetRod false)
      (CallFunction|SetMagnet 2)
      (if (and (Variables|Fisherman|GetIsMagnet) (not (Variables|Fisherman|GetMangenticFishes)))
        (Variables|/Game/FFBlueprints/NPC/Greengrocer/Babushka_AnimBlueprint.Babushka_AnimBlueprint_C|SetFuckOff _animator true)
        (else
          (Variables|/Game/FFBlueprints/NPC/Greengrocer/Babushka_AnimBlueprint.Babushka_AnimBlueprint_C|SetFear _animator true))))))

(event Custom|StartFeeding
  ;[1 1 1] Animation Start/End
  (bind _animator (Utilities|GetandCheckAnimator)
    (:Is%20Valid
      (Variables|/Game/FFBlueprints/NPC/Greengrocer/Babushka_AnimBlueprint.Babushka_AnimBlueprint_C|SetUseBabushkaCustom _animator 1.0)
      (Variables|/Game/FFBlueprints/NPC/Greengrocer/Babushka_AnimBlueprint.Babushka_AnimBlueprint_C|SetFeed _animator true))))

(event Custom|EndFeeding
  ;[1 1 1] Animation Start/End
  (bind _animator (Utilities|GetandCheckAnimator)
    (:Is%20Valid
      (Variables|/Game/FFBlueprints/NPC/Greengrocer/Babushka_AnimBlueprint.Babushka_AnimBlueprint_C|SetFeed _animator false)
      (Variables|/Game/FFBlueprints/NPC/Greengrocer/Babushka_AnimBlueprint.Babushka_AnimBlueprint_C|SetUseBabushkaCustom _animator 0.0)
      (CallFunction|SetTaskinList "Feed" "NewEnumerator1"))))

(event Custom|StartInteraction
  ;[1 1 1] Animation Start/End
  (bind _animator (Utilities|GetandCheckAnimator)
    (:Is%20Valid
      (Variables|/Game/FFBlueprints/NPC/Greengrocer/Babushka_AnimBlueprint.Babushka_AnimBlueprint_C|SetUseBabushkaCustom _animator 1.0)
      (Variables|/Game/FFBlueprints/NPC/Greengrocer/Babushka_AnimBlueprint.Babushka_AnimBlueprint_C|SetInteract _animator true)
      (CallFunction|UseVendingMachine))))

(event Custom|EndInteraction
  ;[1 1 1] Animation Start/End
  (bind _animator (Utilities|GetandCheckAnimator)
    (:Is%20Valid
      (Variables|/Game/FFBlueprints/NPC/Greengrocer/Babushka_AnimBlueprint.Babushka_AnimBlueprint_C|SetInteract _animator false)
      (Variables|/Game/FFBlueprints/NPC/Greengrocer/Babushka_AnimBlueprint.Babushka_AnimBlueprint_C|SetUseBabushkaCustom _animator 0.0)
      (CallFunction|SetTaskinList "BuyFeed" "NewEnumerator1"))))

(event Custom|FeedParticle
  (bind _mesh (Variables|Character|GetMesh))
  ;[1 1 1] VisualHelp
  (if (Variables|Fisherman|GetMangenticFishes)
    (Effects|SpawnEmitterAttached "/Game/assets/particles/PS_bolds.PS_bolds" _mesh "RH_socket")
    (else
      (Effects|SpawnEmitterAttached "/Game/assets/particles/PS_feed.PS_feed" _mesh "RH_socket"))))

(event Custom|FuckOffEndFisherman
  ;[1 1 1] Animation Start/End
  (Variables|/Game/FFBlueprints/NPC/Greengrocer/Babushka_AnimBlueprint.Babushka_AnimBlueprint_C|SetUseBabushkaCustom (Variables|Default|GetAnimator) 0.0)
  (CallFunction|SetTaskinList "Fishing" "NewEnumerator1")
  (Rendering|SetVisibility (Variables|Default|GetCoin) false false)
  (CallFunction|SetMagnet))

(event Custom|SetRod
  (params (ToHand :type Boolean))
  (bind _rot (Variables|Default|GetRot))
  (bind _rot_2 (Variables|Default|GetRot))
  ;[1 1 1] VisualHelp
  (if ToHand
    (Transformation|AttachComponentToComponent _rot (Variables|Character|GetMesh) "hand_left_3" "KeepRelative" "KeepRelative" "KeepRelative" true)
    (Transformation|SetRelativeLocationAndRotation _rot "12.000000,1.900000,20.100000" "0,284.000000,34.000000" false true)
    (else
      (Transformation|AttachComponentToComponent _rot_2 (Variables|Character|GetMesh) "spine1" "KeepRelative" "KeepRelative" "KeepRelative" true)
      (Transformation|SetRelativeLocationAndRotation _rot_2 "78.500000,-28.000000,-32.000000" "-16.000000,62.000000,89.000000" false true))))

(event Custom|StartDogWalkerQuest
  (bind _asbp_npcbase_aicontroller (Utilities|Casting|CastToBP_NPCBaseAIController (Pawn|GetController)))
  (Default|Initialize _asbp_npcbase_aicontroller (Variables|DogWalker|GetDogWalkerBT) "/Game/FFBlueprints/NPC/Greengrocer/BB_GreenGrocer.BB_GreenGrocer" true false))

(event Custom|ShitHappens
  (params (Shit :type Shit%20Object%20Reference))
  (bind _shitstopickup (Variables|DogWalker|GetShitsToPickUp))
  (Utilities|FlowControl|Sequence
    (:then_0
      (if (== (Utilities|Array|Length _shitstopickup) 0)
        (AI|Components|Blackboard|SetValueasObject (AI|GetBlackboard 0) (Utilities|Name|MakeLiteralName "ShitTrouble") (Variables|/Game/FFBlueprints/PickableItem.PickableItem_C|GetCube Shit))))
    (:then_1
      (Utilities|Array|Add _shitstopickup Shit))))

(event Custom|HelpDogEnd
  (AI|Components|Blackboard|SetValueasObject (AI|GetBlackboard 0) (Variables|DogWalker|GetDogTrouble) 0)
  (Variables|/Game/FFBlueprints/NPC/Greengrocer/Babushka_AnimBlueprint.Babushka_AnimBlueprint_C|SetUseBabushkaCustom (Variables|Default|GetAnimator) 0.0)
  (CallFunction|SetTaskinList (Variables|DogWalker|GetHelpDogName) "NewEnumerator1"))

(event Custom|PickUpShit
  (bind _animator (Utilities|GetandCheckAnimator)
    (:Is%20Valid
      (Variables|/Game/FFBlueprints/NPC/Greengrocer/Babushka_AnimBlueprint.Babushka_AnimBlueprint_C|SetUseBabushkaCustom _animator 1.0)
      (Variables|/Game/FFBlueprints/NPC/Greengrocer/Babushka_AnimBlueprint.Babushka_AnimBlueprint_C|SetPickUpShit (Variables|Default|GetAnimator) true))))

(event Custom|DropShit
  (bind _animator (Utilities|GetandCheckAnimator)
    (:Is%20Valid
      (Variables|/Game/FFBlueprints/NPC/Greengrocer/Babushka_AnimBlueprint.Babushka_AnimBlueprint_C|SetUseBabushkaCustom _animator 1.0)
      (Variables|/Game/FFBlueprints/NPC/Greengrocer/Babushka_AnimBlueprint.Babushka_AnimBlueprint_C|SetThrowShit (Variables|Default|GetAnimator) true))))

(event Custom|PickUP
  (bind _shitstopickup (Variables|DogWalker|GetShitsToPickUp))
  (Rendering|SetVisibility (Variables|Default|GetShitBag) true false)
  (bind _asstatic_mesh_component (Utilities|Casting|CastToStaticMeshComponent (AI|Components|Blackboard|GetValueasObject (AI|GetBlackboard 0) (Utilities|Name|MakeLiteralName "ShitTrouble"))))
  (bind _asshit (Utilities|Casting|CastToShit (Components|GetOwner _asstatic_mesh_component)))
  (Utilities|Array|RemoveItem _shitstopickup _asshit)
  (if (> (Utilities|Array|Length _shitstopickup) 0)
    (AI|Components|Blackboard|SetValueasObject (AI|GetBlackboard 0) (Utilities|Name|MakeLiteralName "ShitTrouble") (Variables|/Game/FFBlueprints/PickableItem.PickableItem_C|GetCube (Utilities|Array|Get(acopy) (Variables|DogWalker|GetShitsToPickUp))))
    (else
      (AI|Components|Blackboard|SetValueasObject (AI|GetBlackboard 0) (Utilities|Name|MakeLiteralName "ShitTrouble") 0)))
  (Actor|DestroyActor _asshit))

(event Custom|EndPickUpShit
  (bind _animator (Utilities|GetandCheckAnimator)
    (:Is%20Valid
      (Variables|/Game/FFBlueprints/NPC/Greengrocer/Babushka_AnimBlueprint.Babushka_AnimBlueprint_C|SetUseBabushkaCustom _animator 0.0)
      (Variables|/Game/FFBlueprints/NPC/Greengrocer/Babushka_AnimBlueprint.Babushka_AnimBlueprint_C|SetPickUpShit (Variables|Default|GetAnimator) false)
      (CallFunction|SetTaskinList "PickUpShit" "NewEnumerator1"))))

(event Custom|ThrowAwayShit
  (Rendering|SetVisibility (Variables|Default|GetShitBag) false false))

(event Custom|ThrowEnd
  (bind _animator (Utilities|GetandCheckAnimator)
    (:Is%20Valid
      (Variables|/Game/FFBlueprints/NPC/Greengrocer/Babushka_AnimBlueprint.Babushka_AnimBlueprint_C|SetUseBabushkaCustom _animator 0.0)
      (Variables|/Game/FFBlueprints/NPC/Greengrocer/Babushka_AnimBlueprint.Babushka_AnimBlueprint_C|SetThrowShit (Variables|Default|GetAnimator) false)
      (if (Utilities|Enum|Equal(Enum) (CallFunction|GetTaskState "CallDog") "NewEnumerator0")
        (CallFunction|SetTaskinList "CallDog" "NewEnumerator1")
        (else
          (CallFunction|SetTaskinList "DropShit" "NewEnumerator1"))))))

(event Custom|CallDog
  (bind _animator (Utilities|GetandCheckAnimator)
    (:Is%20Valid
      (Variables|/Game/FFBlueprints/NPC/Greengrocer/Babushka_AnimBlueprint.Babushka_AnimBlueprint_C|SetUseBabushkaCustom _animator 1.0)
      (Variables|/Game/FFBlueprints/NPC/Greengrocer/Babushka_AnimBlueprint.Babushka_AnimBlueprint_C|SetThrowShit (Variables|Default|GetAnimator) true)
      (Utilities|FlowControl|Delay 1.0)
      (bind _asbp_npcpoi (Utilities|Casting|CastToBP_NPCPOI (AI|Components|Blackboard|GetValueasObject (AI|GetBlackboard 0) (Utilities|Name|MakeLiteralName "ActualObject"))))
      (bind _asbp_kennel (Utilities|Casting|CastToBP_Kennel (Variables|/Game/FFBlueprints/NPC/BP_NPCPOI.BP_NPCPOI_C|GetActionObject _asbp_npcpoi)))
      (Default|CallDog _asbp_kennel)
      (AI|Components|Blackboard|SetValueasBool (AI|GetBlackboard 0) (Utilities|Name|MakeLiteralName "HaveDog") true))))

(event Custom|HelpDog
  (bind _asbp_dog (Utilities|Casting|CastToBP_Dog (AI|Components|Blackboard|GetValueasObject (AI|GetBlackboard 0) (Variables|DogWalker|GetDogTrouble)))
    (:then
      (Default|DogExplosion _asbp_dog)
      (Game|SpawnActorfromClass "/Game/FFBlueprints/Ingredients/Chocolate.Chocolate_C" (Transformation|GetWorldTransform (Variables|Default|GetShitBag)) "Undefined" 0 0)
      (Variables|/Game/FFBlueprints/NPC/Greengrocer/Babushka_AnimBlueprint.Babushka_AnimBlueprint_C|SetUseBabushkaCustom (Variables|Default|GetAnimator) 1.0)
      (bind _animator (Utilities|GetandCheckAnimator)
        (:Is%20Valid
          (Variables|/Game/FFBlueprints/NPC/Greengrocer/Babushka_AnimBlueprint.Babushka_AnimBlueprint_C|SetFear _animator true))))
    (:CastFailed
      (CallFunction|SetTaskinList (Variables|DogWalker|GetHelpDogName) "NewEnumerator1"))))

(fn ConstructionScript
  (|CallParentFunction)
  (Utilities|IsValid (Variables|Default|GetNPCmanager)
    (:Is%20Not%20Valid
      (bind _asfast_food_game_state (Utilities|Casting|CastToFastFoodGameState (Game|GetGameState)))
      (Variables|Default|SetNPCmanager (Variables|/Game/FFBlueprints/GameMode/FastFoodGameState.FastFoodGameState_C|GetNPCPOIManager _asfast_food_game_state)))))

(fn SpawnRealVegetable
  (bind _vegetable (Variables|Default|GetVegetable))
  (Rendering|SetVisibility _vegetable false true)
  (bind _returnvalue (Game|SpawnActorfromClass "/Game/FFBlueprints/Ingredients/Vegetable.Vegetable_C" (Math|Transform|MakeTransform (Transformation|GetWorldLocation _vegetable)) "Undefined" 0 0))
  (Default|UseItem _returnvalue))

(fn EndQuest
  (params (NextState :type Integer))
  (Default|NextStateGreengrocer (Variables|Default|GetBP_GreengrocerState) "NewEnumerator1")
  (AI|Components|Blackboard|SetValueasBool (AI|GetBlackboard 0) (Utilities|Name|MakeLiteralName "InQuest") false))

(fn DogCallforHelp
  (params (Dog :type BP%20Dog%20Object%20Reference))
  (if (or (not (Utilities|IsValid Dog)) (Utilities|IsValid (AI|Components|Blackboard|GetValueasObject (AI|GetBlackboard self) (Variables|DogWalker|GetDogTrouble))))
    (return false)
    (else
      (AI|Components|Blackboard|SetValueasObject (AI|GetBlackboard 0) (Variables|DogWalker|GetDogTrouble) Dog)
      (return true))))

(fn UpdateState)

(fn CombinewithItem
  (params (ItemToCombine :type Actor%20Object%20Reference))
  (switch Utilities|FlowControl|Switch|SwitchonStateGreengrocer (Default|GetActualStateGreengrocer (Variables|Default|GetBP_GreengrocerState))
    (:NewEnumerator5
      _)
    (:NewEnumerator0
      _)
    (:NewEnumerator1
      (Utilities|Casting|CastToRottenVegetable ItemToCombine)
      (CallFunction|BoughtVeg)
      (return true false false false))
    (:NewEnumerator2
      (Utilities|Casting|CastToHook ItemToCombine)
      (CallFunction|SwitchHook)
      (return true false false false))
    (:NewEnumerator3
      _)
    (:NewEnumerator4
      _))
  (return false false false false))

(fn GetSaveData
  (bind _state (Default|GetActualState (Variables|Default|GetBP_GreengrocerState)))
  (return (Utilities|Struct|MakeSaveObjectData (Utilities|GetClass self) (Transformation|GetWorldTransform (Variables|Default|GetCapsuleComponent)) "0.000000,0.000000,0.000000|0.000000,0.000000,0.000000|1.000000,1.000000,1.000000" _state)))

(fn IsReadytoUse
  (return (or (and (Variables|Default|GetOfferingRunning) (not (Variables|Default|GetPauseUse))) (and (Variables|Fisherman|GetFishingQuest) (not (Utilities|Enum|Equal(Enum) (CallFunction|GetTaskState "Fishing") "NewEnumerator0"))))))