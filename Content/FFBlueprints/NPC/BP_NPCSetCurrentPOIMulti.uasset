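; Behavior tree task that sets an NPC's current point of interest, picked semi-randomly from a weighted map of POI names.
; On execute it picks a name, passes it to SetupPOI with the owner, and finishes successfully.
; Each entry rolls independently at its share of total weight and the last success wins, so odds are not strictly proportional.
; When no roll succeeds, it falls back to the highest-weight entry.
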(event EventReceiveExecute
  (params (OwnerActor :type Actor%20Object%20Reference))
  (bind _pname (CallFunction|GetWeightedRandomPOI))
  (CallFunction|SetupPOI _pname OwnerActor)
  (AI|BehaviorTree|FinishExecute true))

(fn GetWeightedRandomPOI
  (bind _weightsum (CallFunction|ComputeWeightSum))
  (bind _keys (Utilities|Map|Keys (Variables|Default|GetNames)))
  (for _array_element _keys
    (if (.ReturnValue (Utilities|Map|Find (Variables|Default|GetNames) _array_element))
      (if (Math|Random|RandomBoolwithWeight (/ (Math|Conversions|ToFloat(Integer) (.Value (Utilities|Map|Find (Variables|Default|GetNames) _array_element))) (Math|Conversions|ToFloat(Integer) _weightsum)))
        (LocalVariables|SetFound true)
        (LocalVariables|SetPOIName _array_element))))
  (if (LocalVariables|GetFound)
    (return (LocalVariables|GetPOIName))
    (else
      (bind _values (Utilities|Map|Values (Variables|Default|GetNames)))
      (bind _keys_2 (Utilities|Map|Keys (Variables|Default|GetNames)))
      (for (_array_element_2 _array_index) _keys_2
        (if (== _array_index (.IndexOfMaxValue (Math|Integer|MaxOfIntArray _values)))
          (return _array_element_2)))
      (CallFunction|DebugLog "Item with weight cannot be found" "NewEnumerator0"))))

(fn ComputeWeightSum
  (bind _values (Utilities|Map|Values (Variables|Default|GetNames)))
  (for _array_element _values
    (LocalVariables|SetSum (+ _array_element (LocalVariables|GetSum))))
  (return (LocalVariables|GetSum)))