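; Behavior tree task for NPCs that swaps or copies object values between two blackboard keys.
; On execute it caches the ToObject value in Temp, then writes the FromObject value into ToObject.
; Unless OneWay is set, it writes the cached value back into FromObject to complete the swap, then finishes successfully.
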(event EventReceiveExecute
  (params (OwnerActor :type Actor%20Object%20Reference))
  (bind _returnvalue (AI|GetBlackboard OwnerActor))
  (Variables|Default|SetTemp (AI|Components|Blackboard|GetValueasObject _returnvalue (Variables|Default|GetToObject)))
  (AI|Components|Blackboard|SetValueasObject _returnvalue (Variables|Default|GetToObject) (AI|Components|Blackboard|GetValueasObject _returnvalue (Variables|Default|GetFromObject)))
  (if (Variables|Default|GetOneWay)
    _
    (else
      (AI|Components|Blackboard|SetValueasObject _returnvalue (Variables|Default|GetFromObject) (Variables|Default|GetTemp))))
  (AI|BehaviorTree|FinishExecute true))