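; NPC door that extends a crowd-spawning parent, opening and closing as NPCs spawn and leave.
; Spawning a crowd calls the parent logic then opens the door, as does ActorToDestroy overlapping the Leave component.
; LeaveArea closes it for ActorToDestroy or SpawnedActor, then runs the parent logic.
; A single timeline drives the mesh's relative rotation through a shortest-path lerp, reversing to close.
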(event OnComponentBeginOverlap(Leave)
  (params (OverlappedComponent :type Primitive%20Component%20Object%20Reference) (OtherActor :type Actor%20Object%20Reference) (OtherComp :type Primitive%20Component%20Object%20Reference) (OtherBodyIndex :type Integer) (bFromSweep :type Boolean) (SweepResult :type Hit%20Result%20Structure%20%28by%20ref%29))
  (if (== OtherActor (Variables|Default|GetActorToDestroy))
    (CallFunction|OpenDoor)))

(event Custom|OpenDoor
  (bind _openprogress (Timeline|OpenDoors Play)
    (:Update
      (Transformation|SetRelativeRotation (Variables|Default|GetStaticMesh) (Math|Rotator|Lerp(Rotator) "0,-90.000000, 0" "0, 0, 0" _openprogress true) false false))))

(event Custom|CloseDoor
  (bind _openprogress (Timeline|OpenDoors Reverse)
    (:Update
      (Transformation|SetRelativeRotation (Variables|Default|GetStaticMesh) (Math|Rotator|Lerp(Rotator) "0,-90.000000, 0" "0, 0, 0" _openprogress true) false false))))

(event EventBeginPlay)

(event Collision|EventActorBeginOverlap
  (params (OtherActor :type Actor%20Object%20Reference)))

(event EventTick
  (params (DeltaSeconds :type Float%20%28single-precision%29)))

(event EventSpawnCrowd
  (params (CrowdClass :type Crowd%20Character%20Class%20Reference))
  (|CallParentFunction CrowdClass)
  (CallFunction|OpenDoor))

(event EventLeaveArea
  (params (OtherActor :type Actor%20Object%20Reference))
  (Utilities|FlowControl|Sequence
    (:then_0
      (if (or (== OtherActor (Variables|Default|GetActorToDestroy)) (== (Variables|Default|GetSpawnedActor) OtherActor))
        (CallFunction|CloseDoor)))
    (:then_1
      (|CallParentFunction OtherActor))))

(fn ConstructionScript)