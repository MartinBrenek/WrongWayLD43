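; Main menu GameState Blueprint that handles the New Game, Continue and Exit actions.
; New Game and Continue write a fresh TransitionSaveData object to the "TransData" slot, then open the Persistent level.
; The save object carries intent across the level load, with Continue flagging a load of slot index zero.
; A helper reports whether the "SaveGame0" continue save exists, and Exit quits the game.
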(event Custom|NewGame
  (CallFunction|CreateTransData false)
  (Game|OpenLevel(byName) "Persistent"))

(event Custom|ContinueGame
  (CallFunction|CreateTransData true)
  (Game|OpenLevel(byName) "Persistent"))

(event Custom|Exit
  (Game|QuitGame 0 "Quit" false))

(event EventBeginPlay)

(event EventTick
  (params (DeltaSeconds :type Float%20%28single-precision%29)))

(fn ConstructionScript)

(fn CreateTransData
  (params (Continue :type Boolean))
  (bind _returnvalue (SaveGame|CreateSaveGameObject "/Game/FFBlueprints/SaveLoad/TransitionSaveData.TransitionSaveData_C"))
  (LocalVariables|SetData _returnvalue)
  (if Continue
    (Variables|/Game/FFBlueprints/SaveLoad/TransitionSaveData.TransitionSaveData_C|SetLoadGame (LocalVariables|GetData) true)
    (Variables|/Game/FFBlueprints/SaveLoad/TransitionSaveData.TransitionSaveData_C|SetSlotIndex (LocalVariables|GetData) 0))
  (SaveGame|SaveGametoSlot (LocalVariables|GetData) "TransData"))

(fn ExistContinueSave
  (bind _returnvalue (SaveGame|DoesSaveGameExist "SaveGame0"))
  (return _returnvalue))