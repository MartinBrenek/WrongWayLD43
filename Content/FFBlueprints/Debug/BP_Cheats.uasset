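; Debug cheat actor that, when enabled, lets a fast-food level start from a chosen order.
; On BeginPlay it counts ingredient actors in the scene by type and compares them with what the remaining order states need.
; It spawns missing ingredients and destroys surplus ones, with optional color-coded debug logging.
; After a short delay it tells the game state's fast food manager to set up the preceding order as the last one.
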(event EventBeginPlay
  (if (Variables|Default|GetUseCheat)
    (if (== (Utilities|Array|Length (Variables|Default|GetStates)) (Utilities|Array|Length (Variables|Default|GetOriginalOrders)))
      (if (Math|Integer|InRange(Integer) (Variables|Default|GetStartFromOrder) 0 (Utilities|Array|Length (Variables|Default|GetStates)) true false)
        (bind _outactors (Actor|GetAllActorsOfClass "/Game/FFBlueprints/FastFoodIndoor/IngredientsBP.IngredientsBP_C"))
        (CallFunction|CheckIngredients _outactors)
        (Utilities|FlowControl|Delay 0.2)
        (CallFunction|SetupOrders)))))

(event EventTick
  (params (DeltaSeconds :type Float%20%28single-precision%29)))

(fn ConstructionScript)

(fn CheckIngredients
  (params (IngredientsInScene :type Array%20of%20Ingredients%20BP%20Object%20References))
  (bind _output_get (LocalVariables|SetObjects IngredientsInScene))
  (bind _references1 (CallFunction|CountinScene _output_get))
  (LocalVariables|SetReferencesHaveSorted _references1)
  (bind _count (CallFunction|CountNeed))
  (LocalVariables|SetIngredientsCountNeed _count)
  (bind _keys (Utilities|Map|Keys (LocalVariables|GetIngredientsCountNeed)))
  (for _array_element _keys
    (Utilities|Set|Add (LocalVariables|GetIngredientsChecked) _array_element)
    (if (.ReturnValue (Utilities|Map|Find (LocalVariables|GetReferencesHaveSorted) _array_element))
      (CallFunction|CorrectCount (- (.Value (Utilities|Map|Find (LocalVariables|GetIngredientsCountNeed) _array_element)) (CallFunction|GetCountIngredientsinSortedMap (LocalVariables|GetReferencesHaveSorted) _array_element)) _array_element (LocalVariables|GetObjects) (LocalVariables|GetReferencesHaveSorted))
      (else
        (CallFunction|CorrectCount (.Value (Utilities|Map|Find (LocalVariables|GetIngredientsCountNeed) _array_element)) _array_element (LocalVariables|GetObjects) (LocalVariables|GetReferencesHaveSorted)))))
  (bind _keys_2 (Utilities|Map|Keys (LocalVariables|GetReferencesHaveSorted)))
  (for _array_element_2 _keys_2
    (if (not (Utilities|Set|Contains (LocalVariables|GetIngredientsChecked) _array_element_2))
      (CallFunction|CorrectCount (* (CallFunction|GetCountIngredientsinSortedMap (LocalVariables|GetReferencesHaveSorted) _array_element_2) -1) _array_element_2 (LocalVariables|GetObjects) (LocalVariables|GetReferencesHaveSorted)))))

(fn CountinScene
  (params (Array :type Array%20of%20Ingredients%20BP%20Object%20References))
  (bind _references (LocalVariables|GetReferences))
  (for (_array_element _array_index) Array
    (if (.ReturnValue (Utilities|Map|Find _references (Variables|/Game/FFBlueprints/FastFoodIndoor/IngredientsBP.IngredientsBP_C|GetType _array_element)))
      (bind _output_get (LocalVariables|SetTemp (Utilities|Struct|BreakStructArray (.Value (Utilities|Map|Find _references (Variables|/Game/FFBlueprints/FastFoodIndoor/IngredientsBP.IngredientsBP_C|GetType _array_element))))))
      (Utilities|Array|Add _output_get _array_index)
      (Utilities|Map|Add _references (Variables|/Game/FFBlueprints/FastFoodIndoor/IngredientsBP.IngredientsBP_C|GetType _array_element) (Utilities|Struct|MakeStructArray (LocalVariables|GetTemp)))
      (else
        (Utilities|Map|Add (LocalVariables|GetReferences) (Variables|/Game/FFBlueprints/FastFoodIndoor/IngredientsBP.IngredientsBP_C|GetType _array_element) (Utilities|Struct|MakeStructArray (Utilities|Array|MakeArray _array_index))))))
  (Utilities|PrintIngredientsSort (LocalVariables|GetReferences) "(R=1.000000,G=0.000000,B=0.057804,A=1.000000)" "Have")
  (return (LocalVariables|GetReferences)))

(fn CountNeed
  (bind _states (Variables|Default|GetStates))
  (bind _returnvalue (Utilities|Array|Length _states))
  (bind _returnvalue_2 (- _returnvalue 1))
  (for _index (range (Math|Integer|Min(Integer) (Variables|Default|GetStartFromOrder) _returnvalue_2) _returnvalue_2)
    (bind _array_element (Utilities|Array|ForEachLoopwithBreak (Utilities|Struct|BreakGameStatesNeeds (Utilities|Array|Get(acopy) _states _index)))
      (:LoopBody
        (Utilities|AddtoCount (LocalVariables|GetIngredientsCoutNeed) _array_element))))
  (Utilities|PrintIngredients (LocalVariables|GetIngredientsCoutNeed) "(R=0.000000,G=1.000000,B=0.153453,A=1.000000)" "Need")
  (return (LocalVariables|GetIngredientsCoutNeed)))

(fn CorrectCount
  (params (Count :type Integer) (Ingredients :type Ingredients%20Enum :default "NewEnumerator9") (Objects :type Array%20of%20Ingredients%20BP%20Object%20References) (Sorted :type Map%20of%20Ingredients%20Enums%20to%20Structs :default "NewEnumerator9"))
  (bind (_value _returnvalue) (Utilities|Map|Find Sorted Ingredients))
  (bind _array (Utilities|Struct|BreakStructArray _value))
  (Utilities|PrintDebug (Utilities|String|Append (Utilities|String|EnumtoString Ingredients) " Correct: " (Utilities|String|ToString(Integer) Count)) "(R=0.000000,G=1.000000,B=0.829819,A=1.000000)")
  (if (!= Count 0)
    (if (> Count 0)
      (for _index (range 0 (Math|Integer|Max(Integer) 0 (- Count 1)))
        (bind _returnvalue_2 (Game|SpawnActorfromClass (CallFunction|GetIngredientsClass Ingredients) (|GetTransformInMap) "AlwaysSpawn" 0 0))
        (Math|Integer|IncrementInt (Variables|Default|GetNumSpawned)
          (:%20%20
            (bind _returnvalue_3 (Utilities|Array|Add Objects _returnvalue_2))
            (if (.ReturnValue (Utilities|Map|Find Sorted (Variables|/Game/FFBlueprints/FastFoodIndoor/IngredientsBP.IngredientsBP_C|GetType _returnvalue_2)))
              (Utilities|Array|Add (Utilities|Struct|BreakStructArray (.Value (Utilities|Map|Find Sorted (Variables|/Game/FFBlueprints/FastFoodIndoor/IngredientsBP.IngredientsBP_C|GetType _returnvalue_2)))) _returnvalue_3)
              (Utilities|Map|Add Sorted (Variables|/Game/FFBlueprints/FastFoodIndoor/IngredientsBP.IngredientsBP_C|GetType _returnvalue_2) (Utilities|Struct|MakeStructArray (Utilities|Struct|BreakStructArray (.Value (Utilities|Map|Find Sorted (Variables|/Game/FFBlueprints/FastFoodIndoor/IngredientsBP.IngredientsBP_C|GetType _returnvalue_2))))))
              (else
                (Utilities|Map|Add Sorted (Variables|/Game/FFBlueprints/FastFoodIndoor/IngredientsBP.IngredientsBP_C|GetType _returnvalue_2) (Utilities|Struct|MakeStructArray (Utilities|Array|MakeArray _returnvalue_3))))))))
      (elif _returnvalue
        (for _index_2 (range 0 (- (* Count -1) 1))
          (bind (_array_element _array_index) (Utilities|Array|ForEachLoopwithBreak _array :!label _label)
            (:LoopBody
              (if (!= _array_element -1)
                (if (Utilities|IsValid (Utilities|Array|Get(acopy) Objects _array_element))
                  (Actor|DestroyActor (Utilities|Array|Get(acopy) Objects _array_element))
                  (Utilities|Array|SetArrayElem Objects _array_element 0)
                  (Utilities|Array|SetArrayElem _array _array_index -1)
                  (Utilities|PrintDebug (Utilities|String|Append "Dlete: " (Utilities|String|EnumtoString Ingredients)) "(R=0.000000,G=0.665387,B=1.000000,A=1.000000)")
                  (goto _label Break))))))))))

(fn GetIngredientsClass
  (params (Selection :type Ingredients%20Enum :default "NewEnumerator9"))
  (Utilities|FlowControl|Sequence
    (:then_0
      (switch Utilities|FlowControl|Switch|SwitchonIngredients Selection
        (:NewEnumerator0
          (LocalVariables|SetSelectedClass "/Game/FFBlueprints/Ingredients/Bun.Bun_C"))
        (:NewEnumerator1
          (LocalVariables|SetSelectedClass "/Game/FFBlueprints/Ingredients/BeefMeat.BeefMeat_C"))
        (:NewEnumerator2
          (LocalVariables|SetSelectedClass "/Game/FFBlueprints/Ingredients/Vegetable.Vegetable_C"))
        (:NewEnumerator3
          (LocalVariables|SetSelectedClass "/Game/FFBlueprints/Ingredients/FishMeat.FishMeat_C"))
        (:NewEnumerator4
          (LocalVariables|SetSelectedClass "/Game/FFBlueprints/Ingredients/Rice.Rice_C"))
        (:NewEnumerator5
          (LocalVariables|SetSelectedClass "/Game/FFBlueprints/Ingredients/Sausage.Sausage_C"))
        (:NewEnumerator6
          (LocalVariables|SetSelectedClass "/Game/FFBlueprints/Ingredients/Roll.Roll_C"))
        (:NewEnumerator7
          (LocalVariables|SetSelectedClass "/Game/FFBlueprints/Ingredients/PizzaDough.PizzaDough_C"))
        (:NewEnumerator8
          (LocalVariables|SetSelectedClass "/Game/FFBlueprints/Ingredients/PizzaSugo.PizzaSugo_C"))
        (:NewEnumerator10
          (LocalVariables|SetSelectedClass "/Game/FFBlueprints/Ingredients/Topping.Topping_C"))))
    (:then_1
      (if (Utilities|IsValidClass (LocalVariables|GetSelectedClass))
        _
        (else
          (Development|PrintString (Utilities|String|Append "NOT SET CLASS FOR INGREDIENTS: " (Utilities|String|EnumtoString Selection)) true true "(R=1.000000,G=0.000000,B=0.000000,A=1.000000)" 3e+01)))
      (return (LocalVariables|GetSelectedClass)))))

(fn GetCountIngredientsinSortedMap
  (params (Sorted :type Map%20of%20Ingredients%20Enums%20to%20Structs :default "NewEnumerator9") (Ingredient :type Ingredients%20Enum :default "NewEnumerator9"))
  (bind (_value _returnvalue) (Utilities|Map|Find Sorted Ingredient))
  (if _returnvalue
    (for _array_element (Utilities|Struct|BreakStructArray _value)
      (if (>= _array_element 0)
        (Math|Integer|IncrementInt (LocalVariables|GetNum))))
    (return (LocalVariables|GetNum))
    (else
      (return 0))))

(fn SetupOrders
  (bind _asfast_food_game_state (Utilities|Casting|CastToFastFoodGameState (Game|GetGameState)))
  (Default|CheatSetupLastOrder (Variables|/Game/FFBlueprints/GameMode/FastFoodGameState.FastFoodGameState_C|GetFastFoodManger _asfast_food_game_state) (- (Variables|Default|GetStartFromOrder) 1)))

(fn FinishQuests)