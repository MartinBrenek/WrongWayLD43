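; Debug manager actor for the fast food game that registers with the game state and, outside packaged distribution builds, applies test overrides after a short BeginPlay delay.
; It can replace the order queue, change game speed and enforce per-type ingredient counts by destroying extra actors or spawning missing ones in a grid.
; It also resolves a debug save-slot index from a none, checkpoint or slot setting.
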(event EventBeginPlay
  (Utilities|FlowControl|Sequence
    (:then_0
      (Variables|/Game/FFBlueprints/GameMode/FastFoodGameState.FastFoodGameState_C|SetDebugManager (CallFunction|GetFastFoodGameState) self))
    (:then_1
      (if (not (Class|KismetSystemLibrary|IsPackagedforDistribution))
        (Utilities|FlowControl|Delay 0.2)
        (Utilities|FlowControl|Sequence
          (:then_0
            (|UseDebugOrderQue))
          (:then_1
            (CallFunction|SetLimitOfIngredients))
          (:then_2
            (CallFunction|SetDebugSpeedGame)))))))

(event Collision|EventActorBeginOverlap
  (params (OtherActor :type Actor%20Object%20Reference)))

(event EventTick
  (params (DeltaSeconds :type Float%20%28single-precision%29)))

(fn ConstructionScript)

(fn SetLimitOfIngredients
  (if (and (Variables|Ingredients|GetUseDebugLimitIngredients) (!= (Utilities|Map|Length (Variables|Ingredients|GetLimitIngredients)) 0))
    (CallFunction|DebugLog "Using debug ingrediets limits" "NewEnumerator2")
    (bind _outactors (Actor|GetAllActorsOfClass "/Game/FFBlueprints/FastFoodIndoor/IngredientsBP.IngredientsBP_C"))
    (bind _output_get (LocalVariables|SetAllIngredients _outactors))
    (for _array_element _output_get
      (LocalVariables|Setitem _array_element)
      (if (.ReturnValue (Utilities|Map|Find (LocalVariables|GetSortByIngredients) (Variables|/Game/FFBlueprints/FastFoodIndoor/IngredientsBP.IngredientsBP_C|GetType _array_element)))
        (bind _output_get_2 (LocalVariables|SetActors (Utilities|Struct|BreakArrayBPIngredients (.Value (Utilities|Map|Find (LocalVariables|GetSortByIngredients) (Variables|/Game/FFBlueprints/FastFoodIndoor/IngredientsBP.IngredientsBP_C|GetType _array_element))))))
        (Utilities|Array|Add _output_get_2 (LocalVariables|Getitem))
        (Utilities|Map|Add (LocalVariables|GetSortByIngredients) (Variables|/Game/FFBlueprints/FastFoodIndoor/IngredientsBP.IngredientsBP_C|GetType (LocalVariables|Getitem)) (Utilities|Struct|MakeArrayBPIngredients (LocalVariables|GetActors)))
        (else
          (Utilities|Map|Add (LocalVariables|GetSortByIngredients) (Variables|/Game/FFBlueprints/FastFoodIndoor/IngredientsBP.IngredientsBP_C|GetType (LocalVariables|Getitem)) (Utilities|Struct|MakeArrayBPIngredients (Utilities|Array|MakeArray (LocalVariables|Getitem)))))))
    (Utilities|Array|Clear (LocalVariables|GetActors))
    (bind _keys (Utilities|Map|Keys (Variables|Ingredients|GetLimitIngredients)))
    (for _array_element_2 _keys
      (LocalVariables|SetCount (.Value (Utilities|Map|Find (Variables|Ingredients|GetLimitIngredients) _array_element_2)))
      (if (.ReturnValue (Utilities|Map|Find (LocalVariables|GetSortByIngredients) _array_element_2))
        (bind _output_get_3 (LocalVariables|SetActors (Utilities|Struct|BreakArrayBPIngredients (.Value (Utilities|Map|Find (LocalVariables|GetSortByIngredients) _array_element_2)))))
        (LocalVariables|SetLenght (Utilities|Array|Length _output_get_3))
        (else
          (LocalVariables|SetLenght 0)))
      (if (> (LocalVariables|GetLenght) (Math|Conversions|ToInteger(Byte) (LocalVariables|GetCount)))
        (for _index (range 0 (Utilities|GetLastIndex (- (LocalVariables|GetLenght) (Math|Conversions|ToInteger(Byte) (LocalVariables|GetCount)))))
          (Actor|DestroyActor (Utilities|Array|Get(acopy) (LocalVariables|GetActors) _index)))
        (elif (< (LocalVariables|GetLenght) (Math|Conversions|ToInteger(Byte) (LocalVariables|GetCount)))
          (for _index_2 (range (Utilities|GetLastIndex (LocalVariables|GetLenght)) (Utilities|GetLastIndex (Math|Conversions|ToInteger(Byte) (LocalVariables|GetCount))))
            (if (.ReturnValue (Utilities|Map|Find (Variables|Default|GetIngredientsList) _array_element_2))
              (Game|SpawnActorfromClass (.Value (Utilities|Map|Find (Variables|Default|GetIngredientsList) _array_element_2)) (Utilities|GetActualTransform _index_2 (LocalVariables|GetNumOfSpawns)) "AdjustIfPossibleButAlwaysSpawn" 0 0)
              (else
                (CallFunction|DebugLog (Utilities|String|Append "Not set BP form ingredients: " (Utilities|String|EnumtoString _array_element_2) "in BP_DebugFastFood") "NewEnumerator2"))))
          (Math|Integer|IncrementInt (LocalVariables|GetNumOfSpawns)))))))

(fn GetDebugUseSaveSlot
  (if (not (Class|KismetSystemLibrary|IsPackagedforDistribution))
    (switch Utilities|FlowControl|Switch|SwitchonSaveSlot (Variables|Save|GetUseSaveSlot)
      (:NewEnumerator0
        (return -1))
      (:NewEnumerator1
        (return 0))
      (:NewEnumerator2
        (bind _asfast_food_game_state (Utilities|Casting|CastToFastFoodGameState (Game|GetGameState)))
        (bind _exist (Default|IsSaveonIndex _asfast_food_game_state))
        (if _exist
          (return (+ (Math|Integer|Clamp(Integer) (Variables|Save|GetUseSaveSlotIndex) 0 10) 5))
          (else
            (CallFunction|DebugLog "Try load debug data from empty slot." "NewEnumerator2")
            (return -1)))))
    (else
      (return -1))))

(fn SetDebugSpeedGame
  (bind _gamespeed (Variables|GameSpeed|GetGameSpeed))
  (if (!= _gamespeed 1.0)
    (CallFunction|DebugLog (Utilities|String|Append "Use debug modify speed game to: " (Utilities|String|ToString(Float) _gamespeed)) "NewEnumerator1")
    (CallFunction|ChangeGameSpeed (Variables|GameSpeed|GetGameSpeed))))

(fn ChangeGameSpeed
  (params (Speed :type Float%20%28single-precision%29))
  (bind _fastfoodmanager (CallFunction|GetFastFoodManager))
  (Variables|GameSpeed|SetGameSpeed Speed)
  (Variables|/Game/FFBlueprints/FastFoodIndoor/FastFoodManager.FastFoodManager_C|SetNormalTimeSpeed _fastfoodmanager (Variables|GameSpeed|GetGameSpeed))
  (Default|SpeedTime _fastfoodmanager 1.0))