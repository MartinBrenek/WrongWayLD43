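; Worm companion actor that delivers dialogue with audio and animation, using an in-body UI mesh and the player's out-of-body worm mesh.
; ActivateWorm attaches the out-of-body mesh to the requested player worm position and triggers the in-body disappear state, or plays immediately without one.
; Camera position selects which anim instance receives the dialogue sequence.
; Setup binds both instances' callbacks; events relay subtitle advances and dialogue completion.
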(event Custom|SetAnimation
  (params (Anim :type Anim%20Sequence%20Object%20Reference) (Loop :type Boolean))
  (bind _mesh (CallFunction|SetAnimbyCameraPosition (Variables|Default|GetActivedPos) Anim)))

(event Custom|PlaySound
  (params (soundClue :type Sound%20Base%20Object%20Reference))
  (bind _audio (Variables|Default|GetAudio))
  (Audio|Components|Audio|SetSound _audio soundClue)
  (Audio|Components|Audio|Play _audio 0.0)
  (EventDispatchers|BindEventtoOnAudioFinished _audio (delegate Custom|OnAudioFinished)))

(event Custom|OnAudioFinished
  (Audio|Components|Audio|SetSound (Variables|Default|GetAudio) 0))

(event Custom|ShowSubtitle
  (Default|CallNextSubtittle))

(event Custom|WormDissappear
  (CallFunction|PlayDialog))

(event Custom|PlayDialog
  (bind _dialogdata (Variables|Default|GetDialogData))
  (bind (_text _animation _activecamera _audioclip _autoplayaudio _audiodelay _textdelay _nexttext _textend) (Utilities|Struct|BreakWormDialogStruct _dialogdata))
  (Utilities|FlowControl|Sequence
    (:then_0
      (CallFunction|PlaySound _audioclip))
    (:then_1
      (Utilities|IsValid _animation
        (:Is%20Valid
          (CallFunction|SetAnimation _animation false))))))

(event Custom|AnimEnd
  (Default|CallDialogFinished))

(event Custom|AnimEndOutBody
  (Variables|/Game/assets/characters/worm/BPA_worm_UI.BPA_worm_UI_C|SetDissappear (Variables|Default|GetInBodyAnimInstance) false))

(event Custom|WormAppear
  (CallFunction|AnimEnd))

(event EventBeginPlay)

(event Collision|EventActorBeginOverlap
  (params (OtherActor :type Actor%20Object%20Reference)))

(event EventTick
  (params (DeltaSeconds :type Float%20%28single-precision%29)))

(fn ConstructionScript)

(fn ActivateWorm
  (params (DialogData :type Worm%20Dialog%20Struct%20Structure) (FinishedCallback :type Delegate%20%28by%20ref%29))
  (Variables|Default|SetDialogData DialogData)
  (EventDispatchers|BindEventtoDialogFinished FinishedCallback)
  (Variables|Default|SetActivedPos (.ActiveCamera (Utilities|Struct|BreakWormDialogStruct (Variables|Default|GetDialogData))))
  (if (.ReturnValue (Utilities|Map|Find (Variables|/Game/FirstPersonBP/Blueprints/FirstPersonCharacter.FirstPersonCharacter_C|GetWormPositions (CallFunction|GetPlayer)) (Variables|Default|GetActivedPos)))
    (Transformation|AttachComponentToComponent (Variables|Default|GetOutBodvMesh) (.Value (Utilities|Map|Find (Variables|/Game/FirstPersonBP/Blueprints/FirstPersonCharacter.FirstPersonCharacter_C|GetWormPositions (CallFunction|GetPlayer)) (Variables|Default|GetActivedPos))) "None" "KeepRelative" "KeepRelative" "KeepRelative" true)
    (Variables|/Game/assets/characters/worm/BPA_worm_UI.BPA_worm_UI_C|SetDissappear (Variables|Default|GetInBodyAnimInstance) true)
    (else
      (Variables|Default|SetActivedPos (.ActiveCamera (Utilities|Struct|BreakWormDialogStruct (Variables|Default|GetDialogData))))
      (CallFunction|PlayDialog))))

(fn SetAnimbyCameraPosition
  (params (CameraPosition :type WormCameraPosition%20Enum :default "NewEnumerator0") (Anim :type Anim%20Sequence%20Object%20Reference))
  (switch Utilities|FlowControl|Switch|SwitchonWormCameraPosition CameraPosition
    (:NewEnumerator0
      (Variables|/Game/assets/characters/worm/BPA_worm_UI.BPA_worm_UI_C|SetSequence (Variables|Default|GetInBodyAnimInstance) Anim)
      (return (Variables|Default|GetInBodyMesh)))
    (:NewEnumerator1
      _)
    (:NewEnumerator2
      _)
    (:NewEnumerator3
      _)
    (:NewEnumerator4
      _))
  (Variables|/Game/assets/characters/worm/BPA_Worm.BPA_Worm_C|SetSequence (Variables|Default|GetOutBodyAnimIstance) Anim)
  (return (Variables|Default|GetOutBodvMesh)))

(fn Setup
  (Variables|Default|SetPlayer (CallFunction|GetPlayer))
  (bind _player (Variables|Default|GetPlayer)
    (:then
      (Utilities|FlowControl|Sequence
        (:then_0
          (bind _output_get (Variables|Default|SetOutBodvMesh (Variables|/Game/FirstPersonBP/Blueprints/FirstPersonCharacter.FirstPersonCharacter_C|GetWormMesh _player)))
          (bind _asbpa_worm (Utilities|Casting|CastToBPA_Worm (Components|SkeletalMesh|GetAnimInstance _output_get)))
          (Variables|Default|SetOutBodyAnimIstance _asbpa_worm))
        (:then_1
          (bind _asbpa_worm_ui (Utilities|Casting|CastToBPA_worm_UI (Components|SkeletalMesh|GetAnimInstance (Variables|Default|GetInBodyMesh))))
          (Variables|Default|SetInBodyAnimInstance _asbpa_worm_ui))
        (:then_2
          (EventDispatchers|BindEventtoNextSubtitle (Variables|Default|GetInBodyAnimInstance) (EventDispatchers|CreateEvent :!event Custom|ShowSubtitle))
          (EventDispatchers|BindEventtoEndAnim (Variables|Default|GetInBodyAnimInstance) (EventDispatchers|CreateEvent :!event Custom|AnimEnd))
          (EventDispatchers|BindEventtoNextSubtitle (Variables|Default|GetOutBodyAnimIstance) (EventDispatchers|CreateEvent :!event Custom|ShowSubtitle))
          (EventDispatchers|BindEventtoCallEndAnim (Variables|Default|GetOutBodyAnimIstance) (EventDispatchers|CreateEvent :!event Custom|AnimEndOutBody)))))
    (:else)))