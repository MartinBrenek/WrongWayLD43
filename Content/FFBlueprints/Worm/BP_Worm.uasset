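; BP_Worm is a worm actor that exposes simple animation and sound controls for other code to drive.
; SetAnimation plays a given animation on the skeletal mesh, with optional looping.
; PlaySound assigns and plays a sound on the audio component, then binds to its finished event.
; When playback ends, it clears the sound and calls AudioFinished to signal completion.
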(event Custom|SetAnimation
  (params (Anim :type Anim%20Sequence%20Object%20Reference) (Loop :type Boolean))
  (Components|Animation|PlayAnimation (Variables|Default|GetSkeletalMesh) Anim Loop))

(event Custom|PlaySound
  (params (soundClue :type Sound%20Base%20Object%20Reference))
  (bind _audio (Variables|Default|GetAudio))
  (Audio|Components|Audio|SetSound _audio soundClue)
  (Audio|Components|Audio|Play _audio 0.0)
  (EventDispatchers|BindEventtoOnAudioFinished _audio (delegate Custom|OnAudioFinished)))

(event Custom|OnAudioFinished
  (Audio|Components|Audio|SetSound (Variables|Default|GetAudio) 0)
  (Default|CallAudioFinished))

(event EventBeginPlay)

(event Collision|EventActorBeginOverlap
  (params (OtherActor :type Actor%20Object%20Reference)))

(event EventTick
  (params (DeltaSeconds :type Float%20%28single-precision%29)))

(fn ConstructionScript)