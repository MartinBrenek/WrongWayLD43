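; Configurable house building actor, assembled entirely in the construction script with no active runtime logic.
; HouseType and BuildingType pick a wooden or brick mesh, then dynamic material instances tint walls, roof, doors, windows, wood and drainpipe.
; Building types 4 and above skip roof coloring and take detail colors on material slot 1 instead of 2.
; An optional chimney smoke static mesh attaches to the house's Chimney socket.
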(event EventBeginPlay)

(event Collision|EventActorBeginOverlap
  (params (OtherActor :type Actor%20Object%20Reference)))

(event EventTick
  (params (DeltaSeconds :type Float%20%28single-precision%29)))

(fn ConstructionScript
  (bind _house_mesh (Variables|Default|Gethouse_mesh))
  (bind _house_mesh_2 (Variables|Default|Gethouse_mesh))
  ;[1 1 1] chimney smoke
  (if (Variables|Default|GetChimneySmoke)
    (bind _returnvalue (AddComponent|AddStaticMeshComponent false))
    (Transformation|AttachComponentToComponent _returnvalue (Variables|Default|Gethouse_mesh) "Chimney" "KeepRelative" "KeepRelative" "KeepRelative" true))
  (switch Utilities|FlowControl|Switch|SwitchonHouseType (Variables|Default|GetHouseType)
    (:NewEnumerator0
      ;[1 1 1] mesh select
      (Components|StaticMesh|SetStaticMesh _house_mesh (Utilities|Array|Get(acopy) (Variables|Default|GetWoodenHouses) (Variables|Default|GetBuildingType)))
      ;[1 1 1] set house color
      (bind _returnvalue_2 (Rendering|Material|CreateDynamicMaterialInstance (Variables|Default|Gethouse_mesh) 0 0 "None" :!class /Script/Engine.PrimitiveComponent))
      (Rendering|Material|SetVectorParameterValue _returnvalue_2 "color" (Variables|Default|GetHouseWoodColor) :!class /Script/Engine.MaterialInstanceDynamic)
      (Rendering|Material|SetVectorParameterValue _returnvalue_2 "color_fresnel" (Variables|Default|GetFresnelColor) :!class /Script/Engine.MaterialInstanceDynamic))
    (:NewEnumerator1
      (Components|StaticMesh|SetStaticMesh _house_mesh (Utilities|Array|Get(acopy) (Variables|Default|GetBrickHouses) (Variables|Default|GetBuildingType)))
      (bind _returnvalue_3 (Rendering|Material|CreateDynamicMaterialInstance (Variables|Default|Gethouse_mesh) 0 0 "None" :!class /Script/Engine.PrimitiveComponent))
      (Rendering|Material|SetVectorParameterValue _returnvalue_3 "BrickColor" (Variables|Default|GetBrickColor) :!class /Script/Engine.MaterialInstanceDynamic)
      (Rendering|Material|SetVectorParameterValue _returnvalue_3 "CementColor" (Variables|Default|GetCementColor) :!class /Script/Engine.MaterialInstanceDynamic)
      (Rendering|Material|SetVectorParameterValue _returnvalue_3 "PlasterColor" (Variables|Default|GetPlasterColor) :!class /Script/Engine.MaterialInstanceDynamic)
      (Rendering|Material|SetVectorParameterValue _returnvalue_3 "color_fresnel" (Variables|Default|GetFresnelColor) :!class /Script/Engine.MaterialInstanceDynamic)))
  ;[1 1 1] set Roof Color
  (if (>= (Variables|Default|GetBuildingType) 4)
    ;[1 1 1] Set Detail Colors
    (bind _returnvalue_4 (Rendering|Material|CreateDynamicMaterialInstance _house_mesh_2 1 0 "None" :!class /Script/Engine.PrimitiveComponent))
    (LocalVariables|SetMaterialInstaince _returnvalue_4)
    (else
      ;[1 1 1] set roof color
      (bind _returnvalue_5 (Rendering|Material|CreateDynamicMaterialInstance (Variables|Default|Gethouse_mesh) 1 0 "None" :!class /Script/Engine.PrimitiveComponent))
      (Rendering|Material|SetVectorParameterValue _returnvalue_5 "color" (Variables|Default|GetRoofColor) :!class /Script/Engine.MaterialInstanceDynamic)
      (bind _returnvalue_6 (Rendering|Material|CreateDynamicMaterialInstance _house_mesh_2 2 0 "None" :!class /Script/Engine.PrimitiveComponent))
      (LocalVariables|SetMaterialInstaince _returnvalue_6)))
  (Rendering|Material|SetVectorParameterValue (LocalVariables|GetMaterialInstaince) "DoorColor" (Variables|Default|GetDoorColor) :!class /Script/Engine.MaterialInstanceDynamic)
  (Rendering|Material|SetVectorParameterValue (LocalVariables|GetMaterialInstaince) "WoodColor" (Variables|Default|GetWoodColor) :!class /Script/Engine.MaterialInstanceDynamic)
  (Rendering|Material|SetVectorParameterValue (LocalVariables|GetMaterialInstaince) "WindowColor1" (Variables|Default|GetWindowColor1) :!class /Script/Engine.MaterialInstanceDynamic)
  (Rendering|Material|SetVectorParameterValue (LocalVariables|GetMaterialInstaince) "WindowColor2" (Variables|Default|GetWindowColor2) :!class /Script/Engine.MaterialInstanceDynamic)
  (Rendering|Material|SetScalarParameterValue (LocalVariables|GetMaterialInstaince) "drainpipeColor" (Variables|Default|GetDrainPipeColor) :!class /Script/Engine.MaterialInstanceDynamic))