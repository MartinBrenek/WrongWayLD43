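; BP_LightControl is a control actor that syncs a referenced sun or moon light with the water materials and sky.
; On construction it rotates the light to match its Arrow, updates the material collections and refreshes BP_Sky_Sphere's sun direction.
; UpdateSunAndMoon writes sun or moon direction vectors to MPC_Ocean, chosen by SunOrMoon, and the light color to the ocean, river and lake collections.
; It repeats every Tick, which UpdateEnable toggles.
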(event Custom|UpdateSunAndMoon
  (bind _light (Variables|Default|GetLight))
  (bind _lightcomponent (Variables|/Script/Engine.Light|GetLightComponent _light))
  (bind _returnvalue (Rendering|Components|Light|GetLightColor _lightcomponent))
  (bind _returnvalue_2 (Transformation|GetWorldRotation _lightcomponent))
  (bind _returnvalue_3 (Math|Rotator|GetRotationXVector _returnvalue_2))
  (bind _returnvalue_4 (Math|Vector|GetForwardVector _returnvalue_2))
  (bind _returnvalue_5 (Math|Vector|GetForwardVector _returnvalue_2))
  (bind _returnvalue_6 (Math|Vector|GetForwardVector _returnvalue_2))
  (Utilities|FlowControl|Sequence
    (:then_0
      (Utilities|IsValid _light
        (:Is%20Valid
          (if (Variables|Default|GetSun%20Or%20Moon)
            (Rendering|Material|SetVectorParameterValue "/Game/assets/stall/base_mats/MaterialCollections/MPC_Ocean.MPC_Ocean" "SSS Vector" (Utilities|Struct|MakeLinearColor (.x _returnvalue_6) (.y _returnvalue_6) (.z _returnvalue_6) 0.0) :!class /Script/Engine.KismetMaterialLibrary)
            (Rendering|Material|SetVectorParameterValue "/Game/assets/stall/base_mats/MaterialCollections/MPC_Ocean.MPC_Ocean" "Sun Vector" (Utilities|Struct|MakeLinearColor (.x _returnvalue_5) (.y _returnvalue_5) (.z _returnvalue_5) 0.0) :!class /Script/Engine.KismetMaterialLibrary)
            (else
              (Rendering|Material|SetVectorParameterValue "/Game/assets/stall/base_mats/MaterialCollections/MPC_Ocean.MPC_Ocean" "SSS Moon Vector" (Utilities|Struct|MakeLinearColor (.x _returnvalue_4) (.y _returnvalue_4) (.z _returnvalue_4) 0.0) :!class /Script/Engine.KismetMaterialLibrary)
              (Rendering|Material|SetVectorParameterValue "/Game/assets/stall/base_mats/MaterialCollections/MPC_Ocean.MPC_Ocean" "Moon Vector" (Utilities|Struct|MakeLinearColor (.x _returnvalue_3) (.y _returnvalue_3) (.z _returnvalue_3) 0.0) :!class /Script/Engine.KismetMaterialLibrary))))))
    (:then_1
      (Rendering|Material|SetVectorParameterValue "/Game/assets/stall/base_mats/MaterialCollections/MPC_River.MPC_River" "Sun Reflection Color" _returnvalue :!class /Script/Engine.KismetMaterialLibrary)
      (Rendering|Material|SetVectorParameterValue "/Game/assets/stall/base_mats/MaterialCollections/MPC_Ocean.MPC_Ocean" "Sun Reflection Color" _returnvalue :!class /Script/Engine.KismetMaterialLibrary)
      (Rendering|Material|SetVectorParameterValue "/Game/assets/stall/base_mats/MaterialCollections/MPC_Lake.MPC_Lake" "Sun Reflection Color" _returnvalue :!class /Script/Engine.KismetMaterialLibrary))))

(event EventTick
  (params (DeltaSeconds :type Float%20%28single-precision%29))
  (CallFunction|UpdateSunandMoon))

(fn ConstructionScript
  (bind _arrow (Variables|Default|GetArrow))
  (bind _light (Variables|Default|GetLight))
  (bind _returnvalue (Transformation|GetWorldRotation _arrow))
  (Actor|Tick|SetActorTickEnabled (Variables|Default|GetUpdate%20Enable))
  ;[1 1 1] Rotate The Sun and Moon
  (Utilities|IsValid _light
    (:Is%20Valid
      (Transformation|SetActorRotation _light (Math|Rotator|MakeRotator (.roll _returnvalue) (.pitch _returnvalue) (.yaw _returnvalue)))
      ;[1 1 1] Update The sky
      (CallFunction|UpdateSunandMoon)
      (bind _outactors (Actor|GetAllActorsOfClass "/Engine/EngineSky/BP_Sky_Sphere.BP_Sky_Sphere_C"))
      (Default|UpdateSunDirection _outactors))))