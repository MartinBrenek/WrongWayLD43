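; Cartoon waterfall actor that supports its own colors through dynamic material instances on the water and extra foam slots.
; The Construction Script creates both instances, then runs WaterfallParameters, which BeginPlay also calls.
; That function writes foam, flow, reflection, SSS and normal scalars to the shared MPC_Waterfall collection, so only colors are per actor.
; Texture overrides for cubemap, normal map and detail pattern exist but are not wired.
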(event EventBeginPlay
  (CallFunction|WaterfallParameters))

(fn ConstructionScript
  (bind _waterfall (Variables|Default|GetWaterfall))
  (Utilities|FlowControl|Sequence
    (:then_0
      (bind _returnvalue (Rendering|Material|CreateDynamicMaterialInstance (Variables|Default|GetWaterfall) 0 "/Game/assets/stall/base_mats/Water/Waterfall/MI_Waterfall_01_ChangeableColor.MI_Waterfall_01_ChangeableColor" "None" :!class /Script/Engine.PrimitiveComponent))
      (bind _output_get (Variables|Default|SetInstance%20Mat _returnvalue))
      (Rendering|Material|SetMaterial _waterfall 0 _output_get))
    (:then_1
      (bind _returnvalue_2 (Rendering|Material|CreateDynamicMaterialInstance (Variables|Default|GetWaterfall) 1 "/Game/assets/stall/base_mats/Water/Waterfall/MI_Waterfall_Extra_Foam_ChangeableColor.MI_Waterfall_Extra_Foam_ChangeableColor" "None" :!class /Script/Engine.PrimitiveComponent))
      (bind _output_get_2 (Variables|Default|SetExtra%20Instance%20Mat _returnvalue_2))
      (Rendering|Material|SetMaterial _waterfall 1 _output_get_2))
    (:then_2
      (CallFunction|WaterfallParameters))))

(fn WaterfallParameters
  (bind _instance_mat (Variables|Default|GetInstance%20Mat))
  (bind _foam_color (Variables|Color|GetFoam%20Color))
  (Utilities|FlowControl|Sequence
    (:then_0
      ;[1 1 1] Foam
      (Rendering|Material|SetScalarParameterValue "/Game/assets/stall/base_mats/MaterialCollections/MPC_Waterfall.MPC_Waterfall" "Foam Speed" (Variables|Foam|GetFoam%20Speed) :!class /Script/Engine.KismetMaterialLibrary)
      (Rendering|Material|SetScalarParameterValue "/Game/assets/stall/base_mats/MaterialCollections/MPC_Waterfall.MPC_Waterfall" "Foam X Tile" (Variables|Foam|GetFoam%20X%20Tile) :!class /Script/Engine.KismetMaterialLibrary)
      (Rendering|Material|SetScalarParameterValue "/Game/assets/stall/base_mats/MaterialCollections/MPC_Waterfall.MPC_Waterfall" "Foam Y Tile" (Variables|Foam|GetFoam%20Y%20Tile) :!class /Script/Engine.KismetMaterialLibrary)
      (Rendering|Material|SetScalarParameterValue "/Game/assets/stall/base_mats/MaterialCollections/MPC_Waterfall.MPC_Waterfall" "Foam Width" (Variables|Foam|GetFoam%20Width) :!class /Script/Engine.KismetMaterialLibrary)
      (Rendering|Material|SetScalarParameterValue "/Game/assets/stall/base_mats/MaterialCollections/MPC_Waterfall.MPC_Waterfall" "Vertex Offset" (Variables|Foam|GetVertex%20Offset) :!class /Script/Engine.KismetMaterialLibrary)
      (Rendering|Material|SetScalarParameterValue "/Game/assets/stall/base_mats/MaterialCollections/MPC_Waterfall.MPC_Waterfall" "Waterfall Flow Speed" (Variables|GlobalParameters|GetWaterfall%20Flow%20Speed) :!class /Script/Engine.KismetMaterialLibrary)
      (Rendering|Material|SetScalarParameterValue "/Game/assets/stall/base_mats/MaterialCollections/MPC_Waterfall.MPC_Waterfall" "Day Intensity" (Variables|GlobalParameters|GetDay%20Intensity) :!class /Script/Engine.KismetMaterialLibrary))
    (:then_1
      ;[1 1 1] Reflection
      (Rendering|Material|SetScalarParameterValue "/Game/assets/stall/base_mats/MaterialCollections/MPC_Waterfall.MPC_Waterfall" "CubeMap Intensity" (Variables|Reflection|GetCubemap%20Intensity) :!class /Script/Engine.KismetMaterialLibrary)
      (Rendering|Material|SetScalarParameterValue "/Game/assets/stall/base_mats/MaterialCollections/MPC_Waterfall.MPC_Waterfall" "Specular Intensity" (Variables|Reflection|GetSpecular%20Intensity) :!class /Script/Engine.KismetMaterialLibrary)
      (Rendering|Material|SetScalarParameterValue "/Game/assets/stall/base_mats/MaterialCollections/MPC_Waterfall.MPC_Waterfall" "Reflection Angle" (Variables|Reflection|GetReflection%20Angle) :!class /Script/Engine.KismetMaterialLibrary))
    (:then_2
      ;[1 1 1] SSS
      (Rendering|Material|SetScalarParameterValue "/Game/assets/stall/base_mats/MaterialCollections/MPC_Waterfall.MPC_Waterfall" "SSS Intensity" (Variables|SSS|GetSSS%20Intensity) :!class /Script/Engine.KismetMaterialLibrary)
      (Rendering|Material|SetScalarParameterValue "/Game/assets/stall/base_mats/MaterialCollections/MPC_Waterfall.MPC_Waterfall" "SSS Power" (Variables|SSS|GetSSS%20Power) :!class /Script/Engine.KismetMaterialLibrary))
    (:then_3
      ;[1 1 1] Normal
      (Rendering|Material|SetScalarParameterValue "/Game/assets/stall/base_mats/MaterialCollections/MPC_Waterfall.MPC_Waterfall" "Normal Intensity" (Variables|Normal|GetNormal%20Intensity) :!class /Script/Engine.KismetMaterialLibrary)
      (Rendering|Material|SetScalarParameterValue "/Game/assets/stall/base_mats/MaterialCollections/MPC_Waterfall.MPC_Waterfall" "Normal X Tile" (Variables|Normal|GetNormal%20X%20Tile) :!class /Script/Engine.KismetMaterialLibrary)
      (Rendering|Material|SetScalarParameterValue "/Game/assets/stall/base_mats/MaterialCollections/MPC_Waterfall.MPC_Waterfall" "Normal Y Tile" (Variables|Normal|GetNormal%20Y%20Tile) :!class /Script/Engine.KismetMaterialLibrary)
      (Rendering|Material|SetScalarParameterValue "/Game/assets/stall/base_mats/MaterialCollections/MPC_Waterfall.MPC_Waterfall" "Distorsion" (Variables|Normal|GetDistorsion) :!class /Script/Engine.KismetMaterialLibrary))
    (:then_4
      ;[1 1 1] Color
      (Rendering|Material|SetVectorParameterValue _instance_mat "Base Color" (Variables|Color|GetBase%20Color%20) :!class /Script/Engine.MaterialInstanceDynamic)
      (Rendering|Material|SetVectorParameterValue _instance_mat "Far Color" (Variables|Color|GetSpecular%20Color) :!class /Script/Engine.MaterialInstanceDynamic)
      (Rendering|Material|SetVectorParameterValue _instance_mat "Foam Color" _foam_color :!class /Script/Engine.MaterialInstanceDynamic)
      (Rendering|Material|SetVectorParameterValue _instance_mat "SSS Color" (Variables|Color|GetSSS%20Color) :!class /Script/Engine.MaterialInstanceDynamic))
    (:then_5
      (Rendering|Material|SetVectorParameterValue (Variables|Default|GetExtra%20Instance%20Mat) "Foam Color" _foam_color :!class /Script/Engine.MaterialInstanceDynamic))))