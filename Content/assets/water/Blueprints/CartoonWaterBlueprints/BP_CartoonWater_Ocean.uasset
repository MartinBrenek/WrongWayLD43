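; Cartoon ocean actor that configures the look and Gerstner waves of a stylized water surface.
; Its construction script picks the surface material by OceanType (unlit, PBR or mobile), then assigns a matching depth material or hides the depth mesh for opaque types.
; WaterParameters writes all tuning values to the shared MPC_Ocean on construction and BeginPlay; Tick optionally refreshes Ocean Level from mesh height.
; Texture overrides exist but are unconnected.
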(event EventBeginPlay
  (CallFunction|WaterParameters))

(event EventTick
  (params (DeltaSeconds :type Float%20%28single-precision%29))
  (if (Variables|GlobalParameters|GetUpdate%20WaterMesh%20Transform%20Runtime)
    (Rendering|Material|SetScalarParameterValue "/Game/assets/stall/base_mats/MaterialCollections/MPC_Ocean.MPC_Ocean" "Ocean Level" (.z (Transformation|GetWorldLocation (Variables|Default|GetCartoonWater))) :!class /Script/Engine.KismetMaterialLibrary)))

(fn ConstructionScript
  (bind _cartoonwaterdepth (Variables|Default|GetCartoonWaterDepth))
  (bind _ocean_type (Variables|GlobalParameters|GetOcean%20Type))
  (Utilities|FlowControl|Sequence
    (:then_0
      (bind _returnvalue (Rendering|Material|CreateDynamicMaterialInstance (Variables|Default|GetCartoonWater) 0 (Utilities|Select :Index _ocean_type :NewEnumerator53 "/Game/assets/stall/base_mats/Water/Ocean/MI_Ocean_UNLIT_Transparent_Tesselated.MI_Ocean_UNLIT_Transparent_Tesselated" :NewEnumerator55 "/Game/assets/stall/base_mats/Water/Ocean/MI_Ocean_UNLIT_Transparent_NonTessellated.MI_Ocean_UNLIT_Transparent_NonTessellated" :NewEnumerator54 "/Game/assets/stall/base_mats/Water/Ocean/MI_Ocean_UNLIT_NonTransparent_Tessellated.MI_Ocean_UNLIT_NonTransparent_Tessellated" :NewEnumerator56 "/Game/assets/stall/base_mats/Water/Ocean/MI_Ocean_UNLIT_NonTransparent_NonTessellated.MI_Ocean_UNLIT_NonTransparent_NonTessellated" :NewEnumerator57 0 :NewEnumerator58 "/Game/assets/stall/base_mats/Water/Ocean/MI_Ocean_PBR_Transparent_Tessellated.MI_Ocean_PBR_Transparent_Tessellated" :NewEnumerator60 "/Game/assets/stall/base_mats/Water/Ocean/MI_Ocean_PBR_Transparent_NonTessellated.MI_Ocean_PBR_Transparent_NonTessellated" :NewEnumerator59 "/Game/assets/stall/base_mats/Water/Ocean/MI_Ocean_PBR_NonTransparent_Tessellated.MI_Ocean_PBR_NonTransparent_Tessellated" :NewEnumerator61 "/Game/assets/stall/base_mats/Water/Ocean/MI_Ocean_PBR_NonTransparent_NonTessellated.MI_Ocean_PBR_NonTransparent_NonTessellated" :NewEnumerator62 0 :NewEnumerator63 "/Game/assets/stall/base_mats/Water/Ocean/MI_Ocean_Mobile.MI_Ocean_Mobile" :NewEnumerator64 "/Game/assets/stall/base_mats/Water/Ocean/MI_Ocean_Mobile_NonTransparent.MI_Ocean_Mobile_NonTransparent") "None" :!class /Script/Engine.PrimitiveComponent))
      (bind _output_get (Variables|Default|SetCurrent%20Material%20 _returnvalue))
      (Rendering|Material|SetMaterial (Variables|Default|GetCartoonWater) 0 _output_get)
      (switch Utilities|FlowControl|Switch|SwitchonOceanType _ocean_type
        (:NewEnumerator53
          (bind _returnvalue_2 (Rendering|Material|CreateDynamicMaterialInstance _cartoonwaterdepth 0 "/Game/assets/stall/base_mats/Water/Ocean/MI_Ocean_Tesselated_Depth.MI_Ocean_Tesselated_Depth" "None" :!class /Script/Engine.PrimitiveComponent :!label _label))
          (bind _output_get_2 (Variables|Default|SetCurrent%20Depth%20Material%20 _returnvalue_2))
          (Rendering|Material|SetMaterial (Variables|Default|GetCartoonWaterDepth) 0 _output_get_2))
        (:NewEnumerator55
          (bind _returnvalue_3 (Rendering|Material|CreateDynamicMaterialInstance _cartoonwaterdepth 0 "/Game/assets/stall/base_mats/Water/Ocean/MI_Ocean_NoTessellation_Depth.MI_Ocean_NoTessellation_Depth" "None" :!class /Script/Engine.PrimitiveComponent :!label _label_2))
          (bind _output_get_3 (Variables|Default|SetCurrent%20Depth%20Material%20 _returnvalue_3))
          (Rendering|Material|SetMaterial (Variables|Default|GetCartoonWaterDepth) 0 _output_get_3))
        (:NewEnumerator54
          (Rendering|SetVisibility _cartoonwaterdepth false false :!label _label_3))
        (:NewEnumerator56
          (goto _label_3))
        (:NewEnumerator58
          (goto _label))
        (:NewEnumerator60
          (goto _label_2))
        (:NewEnumerator59
          (goto _label_3))
        (:NewEnumerator61
          (goto _label_3))
        (:NewEnumerator63
          (goto _label_2))
        (:NewEnumerator64
          (goto _label_3))))
    (:then_1
      (CallFunction|WaterParameters))))

(fn WaterParameters
  (Utilities|FlowControl|Sequence
    (:then_0
      ;[1 1 1] Global Parameters
      (Rendering|Material|SetScalarParameterValue "/Game/assets/stall/base_mats/MaterialCollections/MPC_Ocean.MPC_Ocean" "Wave Speed Global" (Variables|GlobalParameters|GetWave%20Speed) :!class /Script/Engine.KismetMaterialLibrary)
      (Rendering|Material|SetScalarParameterValue "/Game/assets/stall/base_mats/MaterialCollections/MPC_Ocean.MPC_Ocean" "Global Opacity" (Variables|GlobalParameters|GetGlobal%20Opacity) :!class /Script/Engine.KismetMaterialLibrary)
      (Rendering|Material|SetScalarParameterValue "/Game/assets/stall/base_mats/MaterialCollections/MPC_Ocean.MPC_Ocean" "Day Intensity" (Variables|GlobalParameters|GetDay%20Intensity) :!class /Script/Engine.KismetMaterialLibrary)
      (Rendering|Material|SetScalarParameterValue "/Game/assets/stall/base_mats/MaterialCollections/MPC_Ocean.MPC_Ocean" "Water Depth" (Variables|GlobalParameters|GetWater%20Depth) :!class /Script/Engine.KismetMaterialLibrary)
      (Rendering|Material|SetScalarParameterValue "/Game/assets/stall/base_mats/MaterialCollections/MPC_Ocean.MPC_Ocean" "Sun Reflection Intensity" (Variables|GlobalParameters|GetSun%20Reflection%20Intensity) :!class /Script/Engine.KismetMaterialLibrary)
      (Rendering|Material|SetScalarParameterValue "/Game/assets/stall/base_mats/MaterialCollections/MPC_Ocean.MPC_Ocean" "Sun Reflection Tightness" (Variables|GlobalParameters|GetSun%20Reflection%20Tightness) :!class /Script/Engine.KismetMaterialLibrary)
      (Rendering|Material|SetScalarParameterValue "/Game/assets/stall/base_mats/MaterialCollections/MPC_Ocean.MPC_Ocean" "Shore Distance" (Variables|GlobalParameters|GetShore%20Distance) :!class /Script/Engine.KismetMaterialLibrary)
      (Rendering|Material|SetScalarParameterValue "/Game/assets/stall/base_mats/MaterialCollections/MPC_Ocean.MPC_Ocean" "Tesselation Factor" (Variables|GlobalParameters|GetTessellation%20Factor) :!class /Script/Engine.KismetMaterialLibrary))
    (:then_1
      ;[1 1 1] Gerstner Waves
      (Rendering|Material|SetScalarParameterValue "/Game/assets/stall/base_mats/MaterialCollections/MPC_Ocean.MPC_Ocean" "Wave Length" (Variables|GerstnerWave|GetWave%20Length) :!class /Script/Engine.KismetMaterialLibrary)
      (Rendering|Material|SetScalarParameterValue "/Game/assets/stall/base_mats/MaterialCollections/MPC_Ocean.MPC_Ocean" "Amplitude" (Variables|GerstnerWave|GetAmplitude) :!class /Script/Engine.KismetMaterialLibrary)
      (Rendering|Material|SetScalarParameterValue "/Game/assets/stall/base_mats/MaterialCollections/MPC_Ocean.MPC_Ocean" "Steepness" (Variables|GerstnerWave|GetSteepness) :!class /Script/Engine.KismetMaterialLibrary)
      (Rendering|Material|SetScalarParameterValue "/Game/assets/stall/base_mats/MaterialCollections/MPC_Ocean.MPC_Ocean" "Gerstner Wave Speed " (Variables|GerstnerWave|GetGerstner%20Wave%20Speed%20) :!class /Script/Engine.KismetMaterialLibrary)
      (Rendering|Material|SetScalarParameterValue "/Game/assets/stall/base_mats/MaterialCollections/MPC_Ocean.MPC_Ocean" "Wind Direction" (Variables|GerstnerWave|GetWind%20Direction) :!class /Script/Engine.KismetMaterialLibrary)
      (Rendering|Material|SetScalarParameterValue "/Game/assets/stall/base_mats/MaterialCollections/MPC_Ocean.MPC_Ocean" "Number of Summed Waves" (Variables|GerstnerWave|GetNumber%20of%20Summed%20Waves) :!class /Script/Engine.KismetMaterialLibrary))
    (:then_2
      ;[1 1 1] Distances
      (Rendering|Material|SetScalarParameterValue "/Game/assets/stall/base_mats/MaterialCollections/MPC_Ocean.MPC_Ocean" "Color Distance Fade" (Variables|Distances|GetColor%20Distance%20Fade) :!class /Script/Engine.KismetMaterialLibrary)
      (Rendering|Material|SetScalarParameterValue "/Game/assets/stall/base_mats/MaterialCollections/MPC_Ocean.MPC_Ocean" "Color Distance Falloff" (Variables|Distances|GetColor%20Distance%20Falloff) :!class /Script/Engine.KismetMaterialLibrary)
      (Rendering|Material|SetScalarParameterValue "/Game/assets/stall/base_mats/MaterialCollections/MPC_Ocean.MPC_Ocean" "Water Depth Distance Fade" (Variables|Distances|GetWater%20Depth%20Distance%20Fade) :!class /Script/Engine.KismetMaterialLibrary)
      (Rendering|Material|SetScalarParameterValue "/Game/assets/stall/base_mats/MaterialCollections/MPC_Ocean.MPC_Ocean" "Water Depth Distance Falloff" (Variables|Distances|GetWater%20Depth%20Distance%20Falloff) :!class /Script/Engine.KismetMaterialLibrary)
      (Rendering|Material|SetScalarParameterValue "/Game/assets/stall/base_mats/MaterialCollections/MPC_Ocean.MPC_Ocean" "Foam Distance Fade" (Variables|Distances|GetFoam%20Distance%20Fade) :!class /Script/Engine.KismetMaterialLibrary)
      (Rendering|Material|SetScalarParameterValue "/Game/assets/stall/base_mats/MaterialCollections/MPC_Ocean.MPC_Ocean" "Foam Distance Falloff" (Variables|Distances|GetFoam%20Distance%20Falloff) :!class /Script/Engine.KismetMaterialLibrary)
      (Rendering|Material|SetScalarParameterValue "/Game/assets/stall/base_mats/MaterialCollections/MPC_Ocean.MPC_Ocean" "Normal Distance Fade" (Variables|Distances|GetNormal%20Distance%20Fade) :!class /Script/Engine.KismetMaterialLibrary)
      (Rendering|Material|SetScalarParameterValue "/Game/assets/stall/base_mats/MaterialCollections/MPC_Ocean.MPC_Ocean" "Normal Distance Falloff" (Variables|Distances|GetNormal%20Distance%20Falloff) :!class /Script/Engine.KismetMaterialLibrary)
      (Rendering|Material|SetScalarParameterValue "/Game/assets/stall/base_mats/MaterialCollections/MPC_Ocean.MPC_Ocean" "Refraction Distance Fade" (Variables|Distances|GetRefraction%20Distance%20Fade) :!class /Script/Engine.KismetMaterialLibrary)
      (Rendering|Material|SetScalarParameterValue "/Game/assets/stall/base_mats/MaterialCollections/MPC_Ocean.MPC_Ocean" "Refraction Distance Falloff" (Variables|Distances|GetRefraction%20Distance%20Falloff) :!class /Script/Engine.KismetMaterialLibrary)
      (Rendering|Material|SetScalarParameterValue "/Game/assets/stall/base_mats/MaterialCollections/MPC_Ocean.MPC_Ocean" "SSS Distance Fade" (Variables|Distances|GetSSS%20Distance%20Fade) :!class /Script/Engine.KismetMaterialLibrary)
      (Rendering|Material|SetScalarParameterValue "/Game/assets/stall/base_mats/MaterialCollections/MPC_Ocean.MPC_Ocean" "SSS Distance Falloff" (Variables|Distances|GetSSS%20Distance%20Falloff) :!class /Script/Engine.KismetMaterialLibrary))
    (:then_3
      ;[1 1 1] Normals
      (Rendering|Material|SetScalarParameterValue "/Game/assets/stall/base_mats/MaterialCollections/MPC_Ocean.MPC_Ocean" "Small Normal Speed" (Variables|Normals|GetSmall%20Normal%20Speed) :!class /Script/Engine.KismetMaterialLibrary)
      (Rendering|Material|SetScalarParameterValue "/Game/assets/stall/base_mats/MaterialCollections/MPC_Ocean.MPC_Ocean" "Small Normal Intensity" (Variables|Normals|GetSmall%20Normal%20Intensity) :!class /Script/Engine.KismetMaterialLibrary)
      (Rendering|Material|SetScalarParameterValue "/Game/assets/stall/base_mats/MaterialCollections/MPC_Ocean.MPC_Ocean" "Small Normal Tiling" (Variables|Normals|GetSmall%20Normal%20Tiling) :!class /Script/Engine.KismetMaterialLibrary)
      (Rendering|Material|SetScalarParameterValue "/Game/assets/stall/base_mats/MaterialCollections/MPC_Ocean.MPC_Ocean" "Large Normal Speed" (Variables|Normals|GetLarge%20Normal%20Speed) :!class /Script/Engine.KismetMaterialLibrary)
      (Rendering|Material|SetScalarParameterValue "/Game/assets/stall/base_mats/MaterialCollections/MPC_Ocean.MPC_Ocean" "Large Normal Intensity" (Variables|Normals|GetLarge%20Normal%20Intensity) :!class /Script/Engine.KismetMaterialLibrary)
      (Rendering|Material|SetScalarParameterValue "/Game/assets/stall/base_mats/MaterialCollections/MPC_Ocean.MPC_Ocean" "Large Normal Tiling" (Variables|Normals|GetLarge%20Normal%20Tiling) :!class /Script/Engine.KismetMaterialLibrary))
    (:then_4
      ;[1 1 1] Seafoam
      (Rendering|Material|SetScalarParameterValue "/Game/assets/stall/base_mats/MaterialCollections/MPC_Ocean.MPC_Ocean" "Seafoam Intensity" (Variables|Seafoam|GetSeafoam%20Intensity) :!class /Script/Engine.KismetMaterialLibrary)
      (Rendering|Material|SetScalarParameterValue "/Game/assets/stall/base_mats/MaterialCollections/MPC_Ocean.MPC_Ocean" "Seafoam Base Height" (Variables|Seafoam|GetSeafoam%20Base%20Height) :!class /Script/Engine.KismetMaterialLibrary)
      (Rendering|Material|SetScalarParameterValue "/Game/assets/stall/base_mats/MaterialCollections/MPC_Ocean.MPC_Ocean" "Seafoam Softness" (Variables|Seafoam|GetSeafoam%20Softness) :!class /Script/Engine.KismetMaterialLibrary)
      (Rendering|Material|SetScalarParameterValue "/Game/assets/stall/base_mats/MaterialCollections/MPC_Ocean.MPC_Ocean" "Seafoam Distorsion" (Variables|Seafoam|GetSeafoam%20Distorsion) :!class /Script/Engine.KismetMaterialLibrary)
      (Rendering|Material|SetScalarParameterValue "/Game/assets/stall/base_mats/MaterialCollections/MPC_Ocean.MPC_Ocean" "Seafoam Tiling" (Variables|Seafoam|GetSeafoam%20Tiling) :!class /Script/Engine.KismetMaterialLibrary))
    (:then_5
      ;[1 1 1] Foam
      (Rendering|Material|SetScalarParameterValue "/Game/assets/stall/base_mats/MaterialCollections/MPC_Ocean.MPC_Ocean" "Foam Intensity" (Variables|Foam|GetFoam%20Intensity) :!class /Script/Engine.KismetMaterialLibrary)
      (Rendering|Material|SetScalarParameterValue "/Game/assets/stall/base_mats/MaterialCollections/MPC_Ocean.MPC_Ocean" "Foam Speed" (Variables|Foam|GetFoam%20Speed) :!class /Script/Engine.KismetMaterialLibrary)
      (Rendering|Material|SetScalarParameterValue "/Game/assets/stall/base_mats/MaterialCollections/MPC_Ocean.MPC_Ocean" "Foam X Tile" (Variables|Foam|GetFoam%20X%20Tile) :!class /Script/Engine.KismetMaterialLibrary)
      (Rendering|Material|SetScalarParameterValue "/Game/assets/stall/base_mats/MaterialCollections/MPC_Ocean.MPC_Ocean" "Foam Y Tile" (Variables|Foam|GetFoam%20Y%20Tile) :!class /Script/Engine.KismetMaterialLibrary)
      (Rendering|Material|SetScalarParameterValue "/Game/assets/stall/base_mats/MaterialCollections/MPC_Ocean.MPC_Ocean" "Intersection Size" (Variables|Foam|GetIntersection%20Size) :!class /Script/Engine.KismetMaterialLibrary)
      (Rendering|Material|SetScalarParameterValue "/Game/assets/stall/base_mats/MaterialCollections/MPC_Ocean.MPC_Ocean" "Intersection Softness" (Variables|Foam|GetIntersection%20Softness) :!class /Script/Engine.KismetMaterialLibrary))
    (:then_6
      ;[1 1 1] Cubemap
      (Rendering|Material|SetScalarParameterValue "/Game/assets/stall/base_mats/MaterialCollections/MPC_Ocean.MPC_Ocean" "CubeMap Intensity" (Variables|Reflection|GetCubeMap%20Intensity) :!class /Script/Engine.KismetMaterialLibrary)
      (Rendering|Material|SetScalarParameterValue "/Game/assets/stall/base_mats/MaterialCollections/MPC_Ocean.MPC_Ocean" "Reflection Angle" (Variables|Reflection|GetReflection%20Angle) :!class /Script/Engine.KismetMaterialLibrary)
      (Rendering|Material|SetScalarParameterValue "/Game/assets/stall/base_mats/MaterialCollections/MPC_Ocean.MPC_Ocean" "Specular Intensity" (Variables|Reflection|GetSpecular%20Intensity) :!class /Script/Engine.KismetMaterialLibrary))
    (:then_7
      ;[1 1 1] Refraction
      (Rendering|Material|SetScalarParameterValue "/Game/assets/stall/base_mats/MaterialCollections/MPC_Ocean.MPC_Ocean" "Refraction Amount" (Variables|Refraction|GetRefraction%20Amount) :!class /Script/Engine.KismetMaterialLibrary)
      (Rendering|Material|SetScalarParameterValue "/Game/assets/stall/base_mats/MaterialCollections/MPC_Ocean.MPC_Ocean" "Refraction View Angle" (Variables|Refraction|GetRefraction%20View%20Angle) :!class /Script/Engine.KismetMaterialLibrary))
    (:then_8
      ;[1 1 1] Highlight
      (Rendering|Material|SetScalarParameterValue "/Game/assets/stall/base_mats/MaterialCollections/MPC_Ocean.MPC_Ocean" "Highlight Intensity" (Variables|Highlight|GetHighlight%20Intensity) :!class /Script/Engine.KismetMaterialLibrary)
      (Rendering|Material|SetScalarParameterValue "/Game/assets/stall/base_mats/MaterialCollections/MPC_Ocean.MPC_Ocean" "Highlight Base Height" (Variables|Highlight|GetHighlight%20Base%20Height) :!class /Script/Engine.KismetMaterialLibrary)
      (Rendering|Material|SetScalarParameterValue "/Game/assets/stall/base_mats/MaterialCollections/MPC_Ocean.MPC_Ocean" "Highlight Softness" (Variables|Highlight|GetHighlight%20Softness) :!class /Script/Engine.KismetMaterialLibrary)
      (Rendering|Material|SetScalarParameterValue "/Game/assets/stall/base_mats/MaterialCollections/MPC_Ocean.MPC_Ocean" "Highlight Density" (Variables|Highlight|GetHighlight%20Density) :!class /Script/Engine.KismetMaterialLibrary))
    (:then_9
      ;[1 1 1] Trough
      (Rendering|Material|SetScalarParameterValue "/Game/assets/stall/base_mats/MaterialCollections/MPC_Ocean.MPC_Ocean" "Trough Intensity" (Variables|Trough|GetTrough%20Intensity) :!class /Script/Engine.KismetMaterialLibrary)
      (Rendering|Material|SetScalarParameterValue "/Game/assets/stall/base_mats/MaterialCollections/MPC_Ocean.MPC_Ocean" "Trough Base Height" (Variables|Trough|GetTrough%20Base%20Height) :!class /Script/Engine.KismetMaterialLibrary)
      (Rendering|Material|SetScalarParameterValue "/Game/assets/stall/base_mats/MaterialCollections/MPC_Ocean.MPC_Ocean" "Trough Softnes" (Variables|Trough|GetTrough%20Softnes) :!class /Script/Engine.KismetMaterialLibrary))
    (:then_10
      ;[1 1 1] SSS
      (Rendering|Material|SetScalarParameterValue "/Game/assets/stall/base_mats/MaterialCollections/MPC_Ocean.MPC_Ocean" "SSS Intensity" (Variables|SubsurfaceScattering|GetSSS%20Intensity) :!class /Script/Engine.KismetMaterialLibrary)
      (Rendering|Material|SetScalarParameterValue "/Game/assets/stall/base_mats/MaterialCollections/MPC_Ocean.MPC_Ocean" "SSS Base Height" (Variables|SubsurfaceScattering|GetSSS%20Base%20Height) :!class /Script/Engine.KismetMaterialLibrary)
      (Rendering|Material|SetScalarParameterValue "/Game/assets/stall/base_mats/MaterialCollections/MPC_Ocean.MPC_Ocean" "SSS Softness" (Variables|SubsurfaceScattering|GetSSS%20Softness) :!class /Script/Engine.KismetMaterialLibrary))
    (:then_11
      ;[1 1 1] Colors
      (Rendering|Material|SetVectorParameterValue "/Game/assets/stall/base_mats/MaterialCollections/MPC_Ocean.MPC_Ocean" "Base Color" (Variables|Colors|GetBase%20Color) :!class /Script/Engine.KismetMaterialLibrary)
      (Rendering|Material|SetVectorParameterValue "/Game/assets/stall/base_mats/MaterialCollections/MPC_Ocean.MPC_Ocean" "Far Color" (Variables|Colors|GetFar%20Color) :!class /Script/Engine.KismetMaterialLibrary)
      (Rendering|Material|SetVectorParameterValue "/Game/assets/stall/base_mats/MaterialCollections/MPC_Ocean.MPC_Ocean" "Shallow Water Color" (Variables|Colors|GetShallow%20Water%20Color) :!class /Script/Engine.KismetMaterialLibrary)
      (Rendering|Material|SetVectorParameterValue "/Game/assets/stall/base_mats/MaterialCollections/MPC_Ocean.MPC_Ocean" "Trough Color" (Variables|Colors|GetTrough%20Color) :!class /Script/Engine.KismetMaterialLibrary)
      (Rendering|Material|SetVectorParameterValue "/Game/assets/stall/base_mats/MaterialCollections/MPC_Ocean.MPC_Ocean" "SSS Color" (Variables|Colors|GetSSS%20Color) :!class /Script/Engine.KismetMaterialLibrary)
      (Rendering|Material|SetVectorParameterValue "/Game/assets/stall/base_mats/MaterialCollections/MPC_Ocean.MPC_Ocean" "Foam Color" (Variables|Colors|GetFoam%20Color) :!class /Script/Engine.KismetMaterialLibrary)
      (Rendering|Material|SetVectorParameterValue "/Game/assets/stall/base_mats/MaterialCollections/MPC_Ocean.MPC_Ocean" "Seafoam Color" (Variables|Colors|GetSeafoam%20Color) :!class /Script/Engine.KismetMaterialLibrary))
    (:then_12
      ;[1 1 1] Location Z
      (Rendering|Material|SetScalarParameterValue "/Game/assets/stall/base_mats/MaterialCollections/MPC_Ocean.MPC_Ocean" "Ocean Level" (.z (Transformation|GetWorldLocation (Variables|Default|GetCartoonWater))) :!class /Script/Engine.KismetMaterialLibrary))))