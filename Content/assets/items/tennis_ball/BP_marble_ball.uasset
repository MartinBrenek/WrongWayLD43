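; Marble ball item that, on activation, enables physics on Sphere1 and, after a delay, launches it with a fixed, mass-independent force.
; When Sphere begins an overlap, a check on the actor's speed toggles KillPP and passes the other actor to Overlapstartbegin only if the ball is moving.
; Ending an overlap always calls Overlapend, while the other lifecycle events only defer to the parent or are disabled.
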(event OnComponentBeginOverlap(Sphere)
  (params (OverlappedComponent :type Primitive%20Component%20Object%20Reference) (OtherActor :type Actor%20Object%20Reference) (OtherComp :type Primitive%20Component%20Object%20Reference) (OtherBodyIndex :type Integer) (bFromSweep :type Boolean) (SweepResult :type Hit%20Result%20Structure%20%28by%20ref%29))
  (bind _returnvalue (Transformation|GetVelocity))
  (bind _returnvalue_2 (Math|Vector|VectorLength _returnvalue))
  (bind _returnvalue_3 (> _returnvalue_2 2.0))
  (Variables|/Script/Engine.PostProcessComponent|SetbEnabled (Variables|Default|GetkillPP) _returnvalue_3)
  (if _returnvalue_3
    (CallFunction|Overlapstartbegin OtherActor)))

(event OnComponentEndOverlap(Sphere)
  (params (OverlappedComponent :type Primitive%20Component%20Object%20Reference) (OtherActor :type Actor%20Object%20Reference) (OtherComp :type Primitive%20Component%20Object%20Reference) (OtherBodyIndex :type Integer))
  (CallFunction|Overlapend))

(event Custom|activate
  (Physics|SetSimulatePhysics (Variables|Default|GetSphere1) true)
  (Utilities|FlowControl|Delay (Variables|Default|Getdelay))
  (Physics|AddForce (Variables|Default|GetSphere1) "-80000.000000,200000.000000, 0" "None" true))

(event EventBeginPlay
  (|CallParentFunction))

(event Collision|EventActorBeginOverlap
  (params (OtherActor :type Actor%20Object%20Reference))
  (|CallParentFunction OtherActor) ; This node is disabled and will not be called.\nDrag off pins to build functionality.
)

(event EventTick
  (params (DeltaSeconds :type Float%20%28single-precision%29))
  (|CallParentFunction DeltaSeconds))

(fn ConstructionScript
  (|CallParentFunction))