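; A rock barrier obstacle that falls over, apparently to close off a path, when the first-person character enters its trigger box.
; The first overlap fires once, notifying an optional linked InteractionObject through the Interaction interface and starting a timeline.
; The timeline's Fall track pitches RotationPivot to tip the rock over.
; A debug message prints if the linked object lacks the interface.
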(event OnComponentBeginOverlap(Box)
  (params (OverlappedComponent :type Primitive%20Component%20Object%20Reference) (OtherActor :type Actor%20Object%20Reference) (OtherComp :type Primitive%20Component%20Object%20Reference) (OtherBodyIndex :type Integer) (bFromSweep :type Boolean) (SweepResult :type Hit%20Result%20Structure%20%28by%20ref%29))
  (Utilities|Casting|CastToFirstPersonCharacter OtherActor)
  (Utilities|FlowControl|DoOnce false
    (:Completed
      (CallFunction|Interaction)
      (bind _fall (Timeline|Timeline_0 PlayFromStart)
        (:Update
          (Transformation|SetRelativeRotation (Variables|Default|Getrotation_pivot) (Math|Rotator|MakeRotator 0.0 (* _fall 94.0) 0.0) false false))))))

(event EventBeginPlay)

(event Collision|EventActorBeginOverlap
  (params (OtherActor :type Actor%20Object%20Reference)))

(event EventTick
  (params (DeltaSeconds :type Float%20%28single-precision%29)))

(fn ConstructionScript)

(fn Interaction
  (bind _interactionobject (Variables|Default|GetInteractionObject))
  (Utilities|IsValid _interactionobject
    (:Is%20Valid
      (if (Utilities|DoesObjectImplementInterface _interactionobject "/Game/FFBlueprints/Interaction.Interaction_C")
        (Class|Interaction|Interaction(Message) (Variables|Default|GetInteractionObject) self)
        (else
          (Development|PrintString "Object not implemet intercation interface" true true "(R=1.000000,G=0.000000,B=0.000000,A=1.000000)"))))))