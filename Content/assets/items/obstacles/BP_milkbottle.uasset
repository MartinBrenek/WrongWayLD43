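; Milk bottle obstacle for the LSD world that tips over by rolling its pivot, with the tipped state tracked in save data.
; The Interaction event plays a timeline that drives the roll.
; The first sphere overlap sends "Continue" to the Snake and sets the saved rotated flag, but does not itself rotate the bottle.
; On BeginPlay a set flag replays the rotation animation rather than snapping to the end pose.
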(event OnComponentBeginOverlap(Sphere)
  (params (OverlappedComponent :type Primitive%20Component%20Object%20Reference) (OtherActor :type Actor%20Object%20Reference) (OtherComp :type Primitive%20Component%20Object%20Reference) (OtherBodyIndex :type Integer) (bFromSweep :type Boolean) (SweepResult :type Hit%20Result%20Structure%20%28by%20ref%29))
  (Utilities|FlowControl|DoOnce false
    (:Completed
      (Default|TriggeredbyPlayer (Variables|Default|GetSnake) "Continue")
      (Variables|/Game/FFBlueprints/SaveLoad/SaveGameLSDWorld.SaveGameLSDWorld_C|SetIsBottleRotated (Variables|/Game/FFBlueprints/GameMode/FastFoodGameState.FastFoodGameState_C|GetSaveDataLSDWorld (CallFunction|GetFastFoodGameState)) true))))

(event EventBeginPlay
  (if (Variables|/Game/FFBlueprints/SaveLoad/SaveGameLSDWorld.SaveGameLSDWorld_C|GetIsBottleRotated (Variables|/Game/FFBlueprints/GameMode/FastFoodGameState.FastFoodGameState_C|GetSaveDataLSDWorld (CallFunction|GetFastFoodGameState)))
    (CallFunction|Interaction)))

(event Collision|EventActorBeginOverlap
  (params (OtherActor :type Actor%20Object%20Reference)))

(event EventTick
  (params (DeltaSeconds :type Float%20%28single-precision%29)))

(event EventInteraction
  (params (Caller :type Actor%20Object%20Reference))
  (bind _rotation (Timeline|rotation Play)
    (:Update
      (Transformation|SetRelativeRotation (Variables|Default|Getpivot) (Math|Rotator|MakeRotator (* _rotation -8e+01) 0.0 0.0) false false))))

(fn ConstructionScript)