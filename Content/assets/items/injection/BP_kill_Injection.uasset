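; BP_kill_Injection is an injection item that flies to a target point and releases a liquid splash with an overlap zone.
; On BeginPlay, a timeline lerps the mesh between two marker components, then triggers a camera shake.
; After a short pause it plays the hit animation while a second timeline scales the decal and sphere.
; Sphere overlaps forward to Overlapstartbegin and Overlapend, which are not defined here.
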(event OnComponentBeginOverlap(Sphere)
  (params (OverlappedComponent :type Primitive%20Component%20Object%20Reference) (OtherActor :type Actor%20Object%20Reference) (OtherComp :type Primitive%20Component%20Object%20Reference) (OtherBodyIndex :type Integer) (bFromSweep :type Boolean) (SweepResult :type Hit%20Result%20Structure%20%28by%20ref%29))
  (CallFunction|Overlapstartbegin OtherActor))

(event OnComponentEndOverlap(Sphere)
  (params (OverlappedComponent :type Primitive%20Component%20Object%20Reference) (OtherActor :type Actor%20Object%20Reference) (OtherComp :type Primitive%20Component%20Object%20Reference) (OtherBodyIndex :type Integer))
  (CallFunction|Overlapend))

(event EventBeginPlay
  (bind _final_position (Variables|Default|Getfinal%20position))
  (bind _returnvalue (Transformation|GetWorldLocation _final_position))
  (|CallParentFunction)
  (bind _alpha (Timeline|Timeline_0 PlayFromStart)
    (:Update
      (Transformation|SetWorldLocation (Variables|Default|Getinjection) (Math|Vector|Lerp(Vector) (Transformation|GetWorldLocation (Variables|Default|Getinitial%20position)) _returnvalue _alpha) false false))
    (:Finished
      (Camera|PlayWorldCameraShake "/Game/assets/items/injection/Injection_camshake.Injection_camshake_C" _returnvalue 0.0 3e+03)
      (Utilities|FlowControl|Delay 0.5)
      (Components|Animation|PlayAnimation (Variables|Default|Getinjection) "/Game/assets/items/injection_hit.injection_hit" false)
      (bind (_direction _liquid _sphere) (Timeline|Timeline_1 PlayFromStart)
        (:Update
          (Transformation|SetRelativeScale3D (Variables|Default|GetDecal) (Math|Conversions|ToVector(Float) (* _liquid 1.5)))
          (Transformation|SetRelativeScale3D (Variables|Default|GetSphere) (Math|Conversions|ToVector(Float) (* _sphere 1.5))))))))

(event Collision|EventActorBeginOverlap
  (params (OtherActor :type Actor%20Object%20Reference)))

(event EventTick
  (params (DeltaSeconds :type Float%20%28single-precision%29)))

(fn ConstructionScript
  (|CallParentFunction))