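; BP_WaterKill is a trigger volume that sinks the first-person player and teleports them back to the sandbox.
; On box overlap it stores the character and plays the SinlToSand timeline, whose curves drive the player's speed and camera height.
; When the timeline finishes, the player is teleported.
; Leaving the box early restores speed and camera height, clears the reference and resets the timeline time.
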(event OnComponentBeginOverlap(Box)
  (params (OverlappedComponent :type Primitive%20Component%20Object%20Reference) (OtherActor :type Actor%20Object%20Reference) (OtherComp :type Primitive%20Component%20Object%20Reference) (OtherBodyIndex :type Integer) (bFromSweep :type Boolean) (SweepResult :type Hit%20Result%20Structure%20%28by%20ref%29))
  (bind _asfirst_person_character (Utilities|Casting|CastToFirstPersonCharacter OtherActor))
  (Utilities|IsValid (Variables|Default|GetActor)
    (:Is%20Valid
      (bind (_direction _speed _deepth) (Timeline|SinlToSand Play)
        (:Update
          (Utilities|IsValid (Variables|Default|GetActor)
            (:Is%20Valid
              (Default|SetSpeedPercentage (Variables|Default|GetActor) _speed)
              (Default|SetHeightOfCamera (Variables|Default|GetActor) _deepth))
            (:Is%20Not%20Valid
              (Timeline|SinlToSand Stop))))
        (:Finished
          (Utilities|IsValid (Variables|Default|GetActor)
            (:Is%20Valid
              (Default|TeleporttoSandBox (Variables|Default|GetActor)))))))
    (:Is%20Not%20Valid
      (Variables|Default|SetActor _asfirst_person_character)
      (Timeline|SinlToSand Play))))

(event OnComponentEndOverlap(Box)
  (params (OverlappedComponent :type Primitive%20Component%20Object%20Reference) (OtherActor :type Actor%20Object%20Reference) (OtherComp :type Primitive%20Component%20Object%20Reference) (OtherBodyIndex :type Integer))
  (Utilities|IsValid (Variables|Default|GetActor)
    (:Is%20Valid
      (Default|SetSpeedPercentage (Variables|Default|GetActor) 1.0)
      (Default|SetHeightOfCamera (Variables|Default|GetActor) 1.0)
      (Variables|Default|SetActor 0)
      (bind (_direction _speed _deepth) (Timeline|SinlToSand SetNewTime)
        (:Update
          (Utilities|IsValid (Variables|Default|GetActor)
            (:Is%20Valid
              (Default|SetSpeedPercentage (Variables|Default|GetActor) _speed)
              (Default|SetHeightOfCamera (Variables|Default|GetActor) _deepth))
            (:Is%20Not%20Valid
              (Timeline|SinlToSand Stop))))
        (:Finished
          (Utilities|IsValid (Variables|Default|GetActor)
            (:Is%20Valid
              (Default|TeleporttoSandBox (Variables|Default|GetActor)))))))))

(event EventBeginPlay)

(event Collision|EventActorBeginOverlap
  (params (OtherActor :type Actor%20Object%20Reference)))

(event EventTick
  (params (DeltaSeconds :type Float%20%28single-precision%29)))

(fn ConstructionScript)