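; Storm cloud effect Blueprint that bobs four cloud puff components up and down.
; Each Tick, it adds a sine of game time, shaped by shared Speed and Scale variables, to each puff's relative Z.
; Small per-puff phase offsets stagger the motion.
; The offset accumulates on the current position rather than a stored base, so the bob depends on frame rate.
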(event EventBeginPlay)

(event Collision|EventActorBeginOverlap
  (params (OtherActor :type Actor%20Object%20Reference)))

(event EventTick
  (params (DeltaSeconds :type Float%20%28single-precision%29))
  (bind _returnvalue (Utilities|Time|GetTimeSeconds))
  (bind _cloudpuff2 (Variables|Default|GetCloudPuff2))
  (bind _cloudpuff3 (Variables|Default|GetCloudPuff3))
  (bind _speed (Variables|Bounce|GetSpeed))
  (bind _scale (Variables|Bounce|GetScale))
  (bind _cloudpuff (Variables|Default|GetCloudPuff))
  (bind _cloudpuff4 (Variables|Default|GetCloudPuff4))
  (bind _returnvalue_2 (* _returnvalue _speed))
  (bind _relativelocation (Variables|/Script/Engine.SceneComponent|GetRelativeLocation _cloudpuff3))
  (bind _relativelocation_2 (Variables|/Script/Engine.SceneComponent|GetRelativeLocation _cloudpuff2))
  (bind _relativelocation_3 (Variables|/Script/Engine.SceneComponent|GetRelativeLocation _cloudpuff))
  (bind _relativelocation_4 (Variables|/Script/Engine.SceneComponent|GetRelativeLocation _cloudpuff4))
  (Transformation|SetRelativeLocation _cloudpuff (Math|Vector|MakeVector (.x _relativelocation_3) (.y _relativelocation_3) (+ (.z _relativelocation_3) (* (Math|Trig|Sin(Radians) (+ _returnvalue_2 0.3)) _scale) 0.0)) false false)
  (Transformation|SetRelativeLocation _cloudpuff4 (Math|Vector|MakeVector (.x _relativelocation_4) (.y _relativelocation_4) (+ (.z _relativelocation_4) (* (Math|Trig|Sin(Radians) (+ _returnvalue_2 0.0)) _scale) 0.0)) false false)
  (Transformation|SetRelativeLocation _cloudpuff2 (Math|Vector|MakeVector (.x _relativelocation_2) (.y _relativelocation_2) (+ (.z _relativelocation_2) (* (Math|Trig|Sin(Radians) (+ _returnvalue_2 0.1)) _scale) 0.0)) false false)
  (Transformation|SetRelativeLocation _cloudpuff3 (Math|Vector|MakeVector (.x _relativelocation) (.y _relativelocation) (+ (.z _relativelocation) (* (Math|Trig|Sin(Radians) (+ _returnvalue_2 0.2)) _scale) 0.0)) false false))

(fn ConstructionScript)