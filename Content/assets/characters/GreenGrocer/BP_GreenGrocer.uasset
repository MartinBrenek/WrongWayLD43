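; Green grocer NPC that offers a vegetable during a quest, which the player can steal or buy.
; Using it while offering steals the vegetable if the player has SlowTime active, otherwise shows a "Pay or die." refusal; combining with a RottenVegetable buys it.
; Babushka anim blueprint flags drive the reactions, and a real vegetable replaces the prop.
; Ending the quest clears the InQuest blackboard key and switches to an idle behavior tree.
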(event EventBeginPlay
  (|CallParentFunction) ; This node is disabled and will not be called.\nDrag off pins to build functionality.
)

(event Collision|EventActorBeginOverlap
  (params (OtherActor :type Actor%20Object%20Reference))
  (|CallParentFunction OtherActor) ; This node is disabled and will not be called.\nDrag off pins to build functionality.
)

(event EventTick
  (params (DeltaSeconds :type Float%20%28single-precision%29))
  (|CallParentFunction DeltaSeconds) ; This node is disabled and will not be called.\nDrag off pins to build functionality.
)

(event EventUseItem
  (bind _ready (CallFunction|IsReadytoUse))
  (if _ready
    (bind _asfirst_person_character (Utilities|Casting|CastToFirstPersonCharacter (Game|GetPlayerCharacter 0)))
    (switch int 0
      (:0
        (if (Variables|/Game/FirstPersonBP/Blueprints/FirstPersonCharacter.FirstPersonCharacter_C|GetSlowTime _asfirst_person_character)
          (CallFunction|StolenVeg)
          (else
            (CallFunction|FuckOffGreenGroccer)))))))

(event EventCalltoEndQuest
  (if (not (Variables|Default|GetPauseEndQuest))
    (switch int (Variables|Default|GetState)
      (:0
        (CallFunction|EndGreenGrocerQuest)
        (Variables|Default|SetState 1)
        (AI|Components|Blackboard|SetValueasBool (AI|GetBlackboard 0) (Utilities|Name|MakeLiteralName "InQuest") false)))))

(event EventCAlltoStartQuest
  (AI|Components|Blackboard|SetValueasBool (AI|GetBlackboard 0) (Utilities|Name|MakeLiteralName "InQuest") true))

(event Custom|Offering
  ;[1 1 1] GreenGrocer
  (Variables|Default|SetPauseUse false)
  (Utilities|IsValid (Variables|Default|GetAnimator)
    (:Is%20Valid
      _)
    (:Is%20Not%20Valid
      (bind _asbabushka_anim_blueprint (Utilities|Casting|CastToBabushka_AnimBlueprint (Components|SkeletalMesh|GetAnimInstance (Variables|Character|GetMesh))))
      (Variables|Default|SetAnimator _asbabushka_anim_blueprint)))
  (Rendering|SetVisibility (Variables|Default|GetVegetable) true false)
  (Variables|Default|SetOfferingRunning true)
  (Variables|/Game/assets/characters/Babushka/Babushka_AnimBlueprint.Babushka_AnimBlueprint_C|SetUseBabushkaCustom (Variables|Default|GetAnimator) 1.0)
  (Variables|/Game/assets/characters/Babushka/Babushka_AnimBlueprint.Babushka_AnimBlueprint_C|SetOffering (Variables|Default|GetAnimator) true)
  (Utilities|FlowControl|Delay 1e+01)
  (Variables|/Game/assets/characters/Babushka/Babushka_AnimBlueprint.Babushka_AnimBlueprint_C|SetOffering (Variables|Default|GetAnimator) false)
  (Variables|Default|SetPauseUse true))

(event Custom|HideVeg
  ;[1 1 1] GreenGrocer
  (Rendering|SetVisibility (Variables|Default|GetVegetable) false false)
  (Variables|/Game/assets/characters/Babushka/Babushka_AnimBlueprint.Babushka_AnimBlueprint_C|SetUseBabushkaCustom (Variables|Default|GetAnimator) 0.0)
  (Variables|Default|SetOfferingRunning false))

(event Custom|EndGreenGrocerQuest
  ;[1 1 1] GreenGrocer
  (Variables|Default|SetOfferingRunning false)
  (Rendering|SetVisibility (Variables|Default|GetVegetable) false false)
  (Variables|/Game/assets/characters/Babushka/Babushka_AnimBlueprint.Babushka_AnimBlueprint_C|SetUseBabushkaCustom (Variables|Default|GetAnimator) 0.0)
  (bind _asbp_npcbase_aicontroller (Utilities|Casting|CastToBP_NPCBaseAIController (Pawn|GetController)))
  (bind _point (Default|GetSpecificPoi _asbp_npcbase_aicontroller "Chill"))
  (AI|Components|Blackboard|SetValueasObject (AI|GetBlackboard 0) (Utilities|Name|MakeLiteralName "ActualObject") _point)
  (Default|SetCurrentBT _asbp_npcbase_aicontroller (Variables|Default|GetBT_IdleAfterGG)))

(event Custom|FuckOffGreenGroccer
  (bind _quote (Variables|Default|GetQuote))
  ;[1 1 1] GreenGrocer
  (Rendering|SetVisibility _quote true false)
  (Rendering|Components|TextRender|SetText _quote (Utilities|Text|MakeLiteralText "Pay or die."))
  (Variables|/Game/assets/characters/Babushka/Babushka_AnimBlueprint.Babushka_AnimBlueprint_C|SetFuckOff (Variables|Default|GetAnimator) true)
  (Variables|Default|SetPauseUse true))

(event Custom|FuckOffEnd
  ;[1 1 1] GreenGrocer
  (Variables|/Game/assets/characters/Babushka/Babushka_AnimBlueprint.Babushka_AnimBlueprint_C|SetFuckOff (Variables|Default|GetAnimator) false)
  (Rendering|SetVisibility (Variables|Default|GetQuote) false false)
  (Variables|Default|SetPauseUse false))

(event Custom|StolenEnd
  (bind _animator (Variables|Default|GetAnimator))
  ;[1 1 1] GreenGrocer
  (Variables|/Game/assets/characters/Babushka/Babushka_AnimBlueprint.Babushka_AnimBlueprint_C|SetOffering _animator false)
  (Variables|/Game/assets/characters/Babushka/Babushka_AnimBlueprint.Babushka_AnimBlueprint_C|SetStolen _animator false)
  (CallFunction|EndGreenGrocerQuest)
  (CallFunction|EndQuest 1))

(event Custom|StolenVeg
  ;[1 1 1] GreenGrocer
  (Variables|Default|SetPauseEndQuest true)
  (CallFunction|SpawnRealVegetable)
  (Variables|/Game/assets/characters/Babushka/Babushka_AnimBlueprint.Babushka_AnimBlueprint_C|SetStolen (Variables|Default|GetAnimator) true))

(event Custom|BoughtVeg
  ;[1 1 1] GreenGrocer
  (Variables|Default|SetPauseEndQuest true)
  (CallFunction|SpawnRealVegetable)
  (Variables|/Game/assets/characters/Babushka/Babushka_AnimBlueprint.Babushka_AnimBlueprint_C|SetSold (Variables|Default|GetAnimator) true))

(event Custom|BoughtVegEnd
  (bind _animator (Variables|Default|GetAnimator))
  ;[1 1 1] GreenGrocer
  (Variables|/Game/assets/characters/Babushka/Babushka_AnimBlueprint.Babushka_AnimBlueprint_C|SetOffering _animator false)
  (Variables|/Game/assets/characters/Babushka/Babushka_AnimBlueprint.Babushka_AnimBlueprint_C|SetSold _animator false)
  (CallFunction|EndGreenGrocerQuest)
  (CallFunction|EndQuest 1))

(fn ConstructionScript
  (|CallParentFunction))

(fn SpawnRealVegetable
  (bind _vegetable (Variables|Default|GetVegetable))
  (Rendering|SetVisibility _vegetable false true)
  (bind _returnvalue (Game|SpawnActorfromClass "/Game/FFBlueprints/Ingredients/Vegetable.Vegetable_C" (Math|Transform|MakeTransform (Transformation|GetWorldLocation _vegetable)) "Undefined" 0 0))
  (Default|UseItem _returnvalue))

(fn EndQuest
  (params (NexState :type Integer))
  (Variables|Default|SetState NexState)
  (AI|Components|Blackboard|SetValueasBool (AI|GetBlackboard 0) (Utilities|Name|MakeLiteralName "InQuest") false))

(fn CombinewithItem
  (params (ItemToCombine :type Actor%20Object%20Reference))
  (switch int (Variables|Default|GetState)
    (:Default
      (return false))
    (:0
      (Utilities|Casting|CastToRottenVegetable ItemToCombine)
      (CallFunction|BoughtVeg)
      (return true))))

(fn IsReadytoUse
  (return (and (Variables|Default|GetOfferingRunning) (not (Variables|Default|GetPauseUse)))))