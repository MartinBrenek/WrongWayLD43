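; BP_shitmonster is a monster actor that drives a post-process effect based on the player's proximity.
; Each Tick it measures the distance from player 0's capsule to its own root, then clamps and inverts it into the PostProcess blend weight.
; The effect peaks when the player is on top of the actor and fades linearly to zero at 3000 units.
; The weight is also printed every frame.
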(event Collision|EventActorBeginOverlap
  (params (OtherActor :type Actor%20Object%20Reference)))

(event EventTick
  (params (DeltaSeconds :type Float%20%28single-precision%29))
  (bind _output_get (Variables|/Script/Engine.PostProcessComponent|SetBlendWeight (Variables|Default|GetPostProcess) (/ (Math|Float|Absolute(Float) (- (Math|Float|Clamp(Float) (Math|Vector|Distance(Vector) (Transformation|GetWorldLocation (Variables|/Script/Engine.Character|GetCapsuleComponent (Game|GetPlayerCharacter 0))) (Transformation|GetWorldLocation (Variables|Default|GetDefaultSceneRoot))) 0.0 3e+03) 3e+03)) 3e+03)))
  (Development|PrintString (Utilities|String|ToString(Float) _output_get)))

(fn ConstructionScript)