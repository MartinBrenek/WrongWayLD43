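; Shitmonster boss that, on a one-time interaction, digs up from underground via a timeline driving position, animation blend and smoke particles.
; A Tick-timed state machine alternates idle turning toward the player with attacks, advanced by Grounded and ReturnedFromAttack events, with the anim Blueprint holding an owner reference.
; Touching the mesh during the attack's lethal window kills the player.
; Post-process weight rises as the player nears.
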(event OnComponentBeginOverlap(MinAttackRange)
  (params (OverlappedComponent :type Primitive%20Component%20Object%20Reference) (OtherActor :type Actor%20Object%20Reference) (OtherComp :type Primitive%20Component%20Object%20Reference) (OtherBodyIndex :type Integer) (bFromSweep :type Boolean) (SweepResult :type Hit%20Result%20Structure%20%28by%20ref%29)))

(event OnComponentEndOverlap(MaxAttackRange)
  (params (OverlappedComponent :type Primitive%20Component%20Object%20Reference) (OtherActor :type Actor%20Object%20Reference) (OtherComp :type Primitive%20Component%20Object%20Reference) (OtherBodyIndex :type Integer))
  (Utilities|Casting|CastToFirstPersonCharacter OtherActor)
  (Utilities|IsValid (Variables|Default|GetTartget)
    (:Is%20Valid
      (Variables|Default|SetTartget 0))))

(event OnComponentBeginOverlap(shitmonster)
  (params (OverlappedComponent :type Primitive%20Component%20Object%20Reference) (OtherActor :type Actor%20Object%20Reference) (OtherComp :type Primitive%20Component%20Object%20Reference) (OtherBodyIndex :type Integer) (bFromSweep :type Boolean) (SweepResult :type Hit%20Result%20Structure%20%28by%20ref%29))
  (if (Variables|Default|GetHurt)
    (bind _asfirst_person_character (Utilities|Casting|CastToFirstPersonCharacter OtherActor))
    (Default|Die _asfirst_person_character "SandBox")))

(event Custom|Triggered
  (for _array_element (Variables|Default|GetParticles)
    (Components|Activation|Activate _array_element true))
  (bind (_direction _digout _animationtransition) (Timeline|Timeline_0 PlayFromStart)
    (:Update
      (Transformation|SetRelativeLocation (Variables|Default|Getshitmonster) (Math|Vector|Lerp(Vector) (Variables|Default|GetDownPosition) "0, 0, 0" _digout) false false)
      (Variables|/Game/assets/characters/shitmonster/shitmonster_Skeleton_AnimBlueprint.shitmonster_Skeleton_AnimBlueprint_C|SetBlendWeight (Variables|Default|GetAnimator) _animationtransition))
    (:Finished
      (for _array_element_2 (Variables|Default|GetParticles)
        (Components|Activation|Deactivate _array_element_2)
        (Variables|Default|SetState "NewEnumerator1")
        (Variables|Default|SetTimer (Variables|Default|GetIdleTime))))))

(event Custom|ReturnedFromAttack
  (Variables|Default|SetState "NewEnumerator1")
  (Variables|Default|SetTimer (Variables|Default|GetIdleTime)))

(event Custom|Grounded
  (Variables|Default|SetHurt false)
  (Variables|Default|SetState "NewEnumerator2")
  (Variables|Default|SetTimer (Variables|Default|GetGroundedTime)))

(event Custom|DealDamage
  (params (Damage :type Float%20%28single-precision%29)))

(event EventBeginPlay
  (Transformation|SetRelativeLocation (Variables|Default|Getshitmonster) (Variables|Default|GetDownPosition) false false)
  (bind _asshitmonster_skeleton_anim_blueprint (Utilities|Casting|CastToshitmonster_Skeleton_AnimBlueprint (Components|SkeletalMesh|GetAnimInstance (Variables|Default|Getshitmonster)))
    (:then
      (bind _output_get (Variables|Default|SetAnimator _asshitmonster_skeleton_anim_blueprint))
      (Variables|/Game/assets/characters/shitmonster/shitmonster_Skeleton_AnimBlueprint.shitmonster_Skeleton_AnimBlueprint_C|SetOwner _output_get self))
    (:CastFailed
      _))
  (Variables|Default|SetParticles (Utilities|Array|MakeArray (Variables|Default|GetP_shitmonster_smoke2) (Variables|Default|GetP_shitmonster_smoke) (Variables|Default|GetP_shitmonster_smoke1)))
  (bind _asfirst_person_character (Utilities|Casting|CastToFirstPersonCharacter (Game|GetPlayerCharacter 0)))
  (Variables|Default|SetTartget _asfirst_person_character))

(event EventInteraction
  (params (Caller :type Actor%20Object%20Reference))
  (Utilities|FlowControl|DoOnce false
    (:Completed
      (CallFunction|Triggered))))

(event EventTick
  (params (DeltaSeconds :type Float%20%28single-precision%29))
  (Utilities|FlowControl|Sequence
    (:then_0
      (switch Utilities|FlowControl|Switch|SwitchonEnemyStates (Variables|Default|GetState)
        (:NewEnumerator1
          (CallFunction|RotateonPlayer DeltaSeconds))))
    (:then_1
      (bind _output_get (Variables|Default|SetTimer (- (Variables|Default|GetTimer) DeltaSeconds)))
      (if (<= _output_get 0.0)
        (switch Utilities|FlowControl|Switch|SwitchonEnemyStates (Variables|Default|GetState)
          (:NewEnumerator1
            (Variables|Default|SetState "NewEnumerator0")
            (Variables|Default|SetHurt true)
            (Variables|/Game/assets/characters/shitmonster/shitmonster_Skeleton_AnimBlueprint.shitmonster_Skeleton_AnimBlueprint_C|SetAttack (Variables|Default|GetAnimator) true))
          (:NewEnumerator2
            (Variables|Default|SetState "NewEnumerator0")
            (Variables|/Game/assets/characters/shitmonster/shitmonster_Skeleton_AnimBlueprint.shitmonster_Skeleton_AnimBlueprint_C|SetAttack (Variables|Default|GetAnimator) false)))))
    (:then_2
      (bind _output_get_2 (Variables|/Script/Engine.PostProcessComponent|SetBlendWeight (Variables|Default|GetPostProcess) (/ (Math|Float|Absolute(Float) (- (Math|Float|Clamp(Float) (Math|Vector|Distance(Vector) (Transformation|GetWorldLocation (Variables|/Script/Engine.Character|GetCapsuleComponent (Game|GetPlayerCharacter 0))) (Transformation|GetWorldLocation (Variables|Default|GetDefaultSceneRoot))) 0.0 3e+03) 3e+03)) 3e+03))))))

(fn ConstructionScript)

(fn RotateonPlayer
  (params (A :type Float%20%28single-precision%29))
  (bind _shitmonster (Variables|Default|Getshitmonster))
  (bind _returnvalue (Transformation|GetWorldRotation _shitmonster))
  (bind (_roll _pitch) (Math|Rotator|BreakRotator _returnvalue))
  (Transformation|SetWorldRotation (Variables|Default|Getshitmonster) (Math|Rotator|MakeRotator _roll _pitch (.Yaw (Math|Rotator|BreakRotator (Math|Rotator|Lerp(Rotator) _returnvalue (Math|Transform|TransformRotation (Math|Transform|MakeTransform "0, 0, 0" (Variables|Default|GetRotationHelp)) (Math|Rotator|FindLookatRotation (Transformation|GetWorldLocation (Variables|Default|Getshitmonster)) (Transformation|GetActorLocation (Variables|Default|GetTartget)))) (* A 1.0) true)))) false false))