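; BP_chestnut_horse is a chestnut figure horse actor that moves along a path through a PFPathFollower component.
; ButtonPressed starts the follower from distance zero.
; On actor overlap, it scans the follower's event points and binds the point named Breakdoor to a breakdoor event, whose body is still empty.
; Tick and the construction script do nothing.
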(event Custom|breakdoor
  (params (FollowerComp :type PF%20Path%20Follower%20Component%20Object%20Reference) (Distance :type Float%20%28single-precision%29) (ExtraData :type Object%20Object%20Reference)))

(event Collision|EventActorBeginOverlap
  (params (OtherActor :type Actor%20Object%20Reference))
  (bind _returnvalue (Class|PFPathFollowerComponent|GetEventPoints (Variables|Default|GetPFPathFollower)))
  (for _array_element (.points _returnvalue)
    (switch name (.name _array_element)
      (:breakdoor
        (bind _returnvalue_2 (Class|PFPathFollowerComponent|GetEventPointDelegatebyName (Variables|Default|GetPFPathFollower) (.name _array_element)))
        (EventDispatchers|AssignOnEventPointReached _returnvalue_2 (delegate Custom|breakdoor))))))

(event EventTick
  (params (DeltaSeconds :type Float%20%28single-precision%29)))

(event EventButtonPressed
  (params (ButtonActor :type Actor%20Object%20Reference))
  (Class|PFPathFollowerComponent|Start (Variables|Default|GetPFPathFollower) 0.0))

(fn ConstructionScript)