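; BP_RopeBase is a cannon-style actor that automatically launches one harpoon projectile two seconds after play begins.
; It spawns BP_ProjectileHarpoon at the PoseableMesh's Fire socket, passing itself as parent actor and enabling debug tracing.
; The harpoon also receives the root primitive of the actor the mesh is attached to as its parent collision component, then gets this actor's ForceObject assigned.
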(event EventBeginPlay
  (bind _poseablemesh (Variables|Default|GetPoseableMesh))
  (Utilities|FlowControl|Delay 2.0)
  (bind _returnvalue (Game|SpawnActorfromClass "/Game/ShipsAndExamples/Cannonz/BP_ProjectileHarpoon.BP_ProjectileHarpoon_C" (Math|Transform|MakeTransform (Transformation|GetSocketLocation _poseablemesh "Fire") (Transformation|GetSocketRotation _poseablemesh "Fire")) "AlwaysSpawn" 0 self (.AsPrimitive%20Component (Utilities|Casting|CastToPrimitiveComponent (VehicleSound|GetRootComponent (Components|GetOwner (Transformation|GetAttachParent (Variables|Default|GetPoseableMesh)))))) "0.000000,0.000000,10.000000" true 0))
  (Variables|/Game/ShipsAndExamples/Cannonz/BP_ProjectileHarpoon.BP_ProjectileHarpoon_C|Setforceobj _returnvalue (Variables|Default|GetForceObject)))

(event Collision|EventActorBeginOverlap
  (params (OtherActor :type Actor%20Object%20Reference)))

(event EventTick
  (params (DeltaSeconds :type Float%20%28single-precision%29)))

(fn ConstructionScript)